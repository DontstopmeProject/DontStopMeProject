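; Low-signal zone actor that shows a connection-problems widget and plays white noise while the player character is inside its trigger box.
; Overlap begin and end on Box create and clear both effects, but only while the second box, Box1, has collision enabled.
; The construction script sizes both boxes from extent variables.
; A SaveWeapon graph, not called by these events, copies a held weapon's class, ammo and health to the game mode.
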(event `self.ReceiveBeginPlay`
  (bind _asdsm_game_instance (cast `/Game/Blueprints/Dsm_GameInstance` (`GameplayStatics.GetGameInstance`)))
  (set `self.GI` _asdsm_game_instance))

(event `self.Box.OnComponentBeginOverlap`
  (params (OverlappedComponent :type "PrimitiveComponent Object Reference") (OtherActor :type "Actor Object Reference") (OtherComp :type "PrimitiveComponent Object Reference") (OtherBodyIndex :type Integer) (bFromSweep :type Boolean) (SweepResult :type "HitResult Structure (by ref)"))
  (cast `/Game/Blueprints/PlayersCharacter` OtherActor)
  (if (not (`|EnumEquality` (`PrimitiveComponent.GetCollisionEnabled` (`self.Box1`)) "NoCollision"))
    (bind _returnvalue (`|CreateWidget` "/Game/Blueprints/Widgets/BaseWidgets/W_ConnectionProblems.W_ConnectionProblems_C"))
    (bind _output_get (set `self.Widget` _returnvalue))
    (`UserWidget.AddToViewport` _output_get 0)
    (bind _returnvalue_2 (`GameplayStatics.CreateSound2D` "/Game/Assets/Sounds/GUI/White_noise_dont_stop_me.White_noise_dont_stop_me" 1.5 1.0 0.0 null false false))
    (bind _output_get_2 (set `self.Sound` _returnvalue_2))
    (`AudioComponent.Play` _output_get_2 0.0)))

(event `self.Box.OnComponentEndOverlap`
  (params (OverlappedComponent :type "PrimitiveComponent Object Reference") (OtherActor :type "Actor Object Reference") (OtherComp :type "PrimitiveComponent Object Reference") (OtherBodyIndex :type Integer))
  (bind _widget (`self.Widget`))
  (bind _sound (`self.Sound`))
  (cast `/Game/Blueprints/PlayersCharacter` OtherActor)
  (if (not (`|EnumEquality` (`PrimitiveComponent.GetCollisionEnabled` (`self.Box1`)) "NoCollision"))
    (`/Engine/EditorBlueprintResources/StandardMacros.IsValid` _widget
      (:`Is Valid`
        (`Widget.RemoveFromParent` _widget)
        (`/Engine/EditorBlueprintResources/StandardMacros.IsValid` _sound
          (:`Is Valid`
            _)))
      (:`Is Not Valid`
        _))
    (`AudioComponent.Stop` _sound)))

(fn `SaveWaeponFunc`)

(fn `UserConstructionScript`
  (`BoxComponent.SetBoxExtent` (`self.Box`) (`self.BoxExtent`) true)
  (`BoxComponent.SetBoxExtent` (`self.Box1`) (`self.BoxExtent1`) true))