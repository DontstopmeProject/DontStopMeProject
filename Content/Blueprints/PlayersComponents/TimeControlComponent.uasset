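; Player component that smoothly slows or restores global time dilation, pausing the game once a slowdown reaches its target.
; ToggleTD takes a target (zero selects defaults), unpauses when speeding up, and opens a Gate driven by Tick.
; Each tick interpolates dilation at constant speed until the target closes the Gate.
; Unless ForceToggle is set, disabled time-dilation flags on PlayersCharacter abort the transition and unpause the game.
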(event `ToggleTD`
  (params (TargetTD :type "Float (double-precision)") (Slow :type Boolean) (ForceToggle :type Boolean))
  (bind _returnvalue (`KismetMathLibrary.FInterpTo_Constant` (`GameplayStatics.GetGlobalTimeDilation`) (`self.TargetTD`) (`GameplayStatics.GetWorldDeltaSeconds`) (`self.InterpolationSpeed`)))
  ;[1 1 1] Вызывается откуда необходимо
  (set `self.Slow` Slow)
  (if (== TargetTD 0.0)
    (if (`self.Slow`)
      (set `self.TargetTD` 0.2)
      (goto _label :!via `Open`)
      (else
        (set `self.TargetTD` 1.0)
        (`GameplayStatics.SetGamePaused` false)
        (goto _label :!via `Open`)))
    (elif (`self.Slow`)
      (set `self.TargetTD` TargetTD)
      (goto _label :!via `Open`)
      (else
        (set `self.TargetTD` TargetTD)
        (`GameplayStatics.SetGamePaused` false)
        (goto _label :!via `Open`)))))

(event `self.ReceiveTick`
  (params (DeltaSeconds :type "Float (single-precision)"))
  (bind _returnvalue (`KismetMathLibrary.FInterpTo_Constant` (`GameplayStatics.GetGlobalTimeDilation`) (`self.TargetTD`) (`GameplayStatics.GetWorldDeltaSeconds`) (`self.InterpolationSpeed`)))
  (`/Engine/EditorBlueprintResources/StandardMacros.Gate` true :!label _label
    (:`Exit`
      (bind _asplayers_character (cast `/Game/Blueprints/PlayersCharacter` (`GameplayStatics.GetPlayerCharacter` 0)))
      (if (stale `ToggleTD` ForceToggle)
        _
        (elif (or (not (`/Game/Blueprints/PlayersCharacter.MasterEnableTimeDilation` _asplayers_character)) (not (`/Game/Blueprints/PlayersCharacter.ChangeTimeDilationInPlayersClass` _asplayers_character)))
          (`GameplayStatics.SetGamePaused` false)
          (goto _label :!via `Close`)
          (else
            _)))
      (if (`self.Slow`)
        ;[1 1 1] Происходит при замедлении
        (if (== (`GameplayStatics.GetGlobalTimeDilation`) (`self.TargetTD`))
          (`GameplayStatics.SetGamePaused` true)
          (`self.NewFunction_0`)
          (goto _label :!via `Close`)
          (else
            (`GameplayStatics.SetGlobalTimeDilation` _returnvalue)))
        (else
          ;[1 1 1] Происходит при ускорении
          (`GameplayStatics.SetGlobalTimeDilation` _returnvalue)
          (if (== (`GameplayStatics.GetGlobalTimeDilation`) (`self.TargetTD`))
            (goto _label :!via `Close`)))))))

(fn `NewFunction_0`
  (returns (MasterEnableTimeDilation :type Boolean))
  (bind _asplayers_character (cast `/Game/Blueprints/PlayersCharacter` (`GameplayStatics.GetPlayerCharacter` 0)))
  (bind _masterenabletimedilation (`/Game/Blueprints/PlayersCharacter.MasterEnableTimeDilation` _asplayers_character))
  (if (not _masterenabletimedilation)
    (`GameplayStatics.SetGamePaused` false))
  (return _masterenabletimedilation))