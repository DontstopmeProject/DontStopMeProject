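; Actor component that plays a slow-motion death cinematic, orbiting a camera around a sphere while tracking a given actor.
; EventPlay runs once: it randomizes the sphere's yaw, slows global time, blends view to the owner and disables player input, with glitch widgets and sounds.
; Tick keeps rotating the sphere.
; After short delays it returns view and input, re-enables the character's time-dilation control and starts calm music.
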(event `EventPlay`
  (params (Camera :type "CineCameraComponent Object Reference") (parentSphere :type "SphereComponent Object Reference") (`Actor to Track` :type "Actor Object Reference"))
  (bind _camera (`self.Camera`))
  (bind _output_get (set `self.Parent` parentSphere))
  (set `self.Camera` Camera)
  (`/Engine/EditorBlueprintResources/StandardMacros.DoOnce` false
    (:`Completed`
      (bind _returnvalue_location (`KismetMathLibrary.BreakTransform` (`SceneComponent.GetRelativeTransform` _output_get)))
      (set `self.Location` _returnvalue_location)
      (bind _returnvalue (`|CreateWidget` "/Game/Blueprints/Widgets/BaseWidgets/GlitchWidget.GlitchWidget_C"))
      (`UserWidget.AddToViewport` _returnvalue 0)
      (`GameplayStatics.PlaySound2D` "/Game/Assets/Sounds/Effects/1Slow_Motion_Sound_Effect__WAV_.1Slow_Motion_Sound_Effect__WAV_")
      (`self.ToggleActive` _camera)
      (set `CineCameraComponent.FocusSettings` (make `CameraFocusSettings` "Tracking" 100000.0 (make `CameraTrackingFocusSettings` `Actor to Track` (0.0 0.0 0.0) true) true) _camera)
      (bind _output_get_2 (set `self.Int` (`KismetMathLibrary.RandomIntegerInRange` 0 1)))
      (`SceneComponent.K2_SetRelativeRotation` (`self.Parent`) (`KismetMathLibrary.MakeRotator` 0.0 0.0 (select `int` _output_get_2 :`0` (`KismetMathLibrary.RandomFloatInRange` -50.0 -110.0) :`1` (`KismetMathLibrary.RandomFloatInRange` 150.0 68.0))) false false)
      (set `self.Rotation` (`KismetMathLibrary.MakeRotator` 0.0 0.0 (select `int` (`self.Int`) :`0` 0.1 :`1` -0.1 :!type "Float (single-precision)")))
      (bind _asplayers_character (cast `/Game/Blueprints/PlayersCharacter` (`GameplayStatics.GetPlayerCharacter` 0)))
      (set `/Game/Blueprints/PlayersCharacter.MasterEnableTimeDilation` false _asplayers_character)
      (set `/Game/Blueprints/BaseCharacterClass.StopChangingCustomTime` true _asplayers_character)
      (set `Actor.CustomTimeDilation` 1.0 _asplayers_character)
      (`GameplayStatics.SetGlobalTimeDilation` 0.05)
      (`PlayerController.SetViewTargetWithBlend` (`GameplayStatics.GetPlayerController` 0) (`self.GetOwner`) 0.0 "VTBlend_Linear" 0.0 false)
      (set `self.Rotate` true)
      (`Actor.DisableInput` _asplayers_character (`GameplayStatics.GetPlayerController` 0))
      (`KismetSystemLibrary.Delay` 0.02)
      (`Widget.RemoveFromParent` _returnvalue)
      (`KismetSystemLibrary.Delay` 0.35)
      (`GameplayStatics.PlaySound2D` "/Game/Assets/Sounds/Effects/2Slow_Motion_Sound_Effect__WAV_.2Slow_Motion_Sound_Effect__WAV_")
      (bind _returnvalue_2 (`|CreateWidget` "/Game/Blueprints/Widgets/BaseWidgets/GlitchWidget.GlitchWidget_C"))
      (`UserWidget.AddToViewport` _returnvalue_2 0)
      (`PlayerController.SetViewTargetWithBlend` (`GameplayStatics.GetPlayerController` 0) (`GameplayStatics.GetPlayerCharacter` 0) 0.0 "VTBlend_Linear" 0.0 false)
      (`KismetSystemLibrary.Delay` 0.012)
      (bind _asplayers_character_2 (cast `/Game/Blueprints/PlayersCharacter` (`GameplayStatics.GetPlayerCharacter` 0)))
      (set `/Game/Blueprints/PlayersCharacter.MasterEnableTimeDilation` true _asplayers_character_2)
      (set `/Game/Blueprints/BaseCharacterClass.StopChangingCustomTime` false _asplayers_character_2)
      (bind _asdsm_gamemode (cast `/Game/Blueprints/DsmGamemode` (`GameplayStatics.GetGameMode`)))
      (`/Game/Blueprints/DsmGamemode.EventPlayCalmMusic` _asdsm_gamemode)
      (`Actor.EnableInput` _asplayers_character_2 (`GameplayStatics.GetPlayerController` 0))
      (`Widget.RemoveFromParent` _returnvalue_2))))

(event `self.ReceiveTick`
  (params (DeltaSeconds :type "Float (single-precision)"))
  (bind (_rotation_roll _rotation_pitch _rotation_yaw) (`KismetMathLibrary.BreakRotator` (`self.Rotation`)))
  (if (`self.Rotate`)
    (`SceneComponent.K2_AddRelativeRotation` (`self.Parent`) (`KismetMathLibrary.MakeRotator` 0.0 0.0 _rotation_yaw) false false)))