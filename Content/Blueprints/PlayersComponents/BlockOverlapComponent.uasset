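; Weapon component that handles the recoil of the wielding character when EventBlockOverlap fires on a blocked hit.
; The event stops the current montage, disables weapon hit collisions and clears focus on the hit actor's AI controller.
; Tick then pushes the character backward for a counted number of frames at normal global time dilation, suspending player controls or NPC attack and chase flags.
; DoOnce gates restore those states once the recoil ends.
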(event `self.ReceiveTick`
  (params (DeltaSeconds :type "Float (single-precision)"))
  (bind _ownercharacter (`self.OwnerCharacter`))
  (if (`self.MoveWhenBlock`)
    (if (<= (`self.MoveCounter`) (`self.DesiredCounterValue`))
      (bind _asbase_npc (cast `/Game/Blueprints/Ai/BaseNPC` _ownercharacter)
        (:`then`
          (`|ExecutionSequence`
            (:`then_0`
              (`/Engine/EditorBlueprintResources/StandardMacros.DoOnce` false :!label _label
                (:`Completed`
                  (set `/Game/Blueprints/Ai/BaseNPC.NpcAttack` false _asbase_npc)
                  (set `/Game/Blueprints/Ai/BaseNPC.TempSeesEnemy` (`/Game/Blueprints/Ai/BaseNPC.SeesEnemy?` _asbase_npc) _asbase_npc)
                  (set `/Game/Blueprints/Ai/BaseNPC.TempFollowsEnemy` (`/Game/Blueprints/Ai/BaseNPC.FollowsEnemy?` _asbase_npc) _asbase_npc)
                  (set `/Game/Blueprints/Ai/BaseNPC.SeesEnemy?` false _asbase_npc)
                  (set `/Game/Blueprints/Ai/BaseNPC.FollowsEnemy?` false _asbase_npc)
                  (bind _asweapon_base (cast `/Game/Blueprints/Weapons/Weapons/WeaponBase` (`ChildActorComponent.ChildActor` (`/Game/Blueprints/BaseCharacterClass.PickableItem` _asbase_npc))))
                  (set `/Game/Blueprints/Weapons/Weapons/WeaponBase.ResetAttack` false _asweapon_base))))
            (:`then_1`
              (`Pawn.AddMovementInput` (`self.OwnerCharacter`) (`Actor.GetActorForwardVector` _ownercharacter) -1.0 false :!label _label_2)
              (`GameplayStatics.SetGlobalTimeDilation` 1.0)
              (`/Engine/EditorBlueprintResources/StandardMacros.IncrementInt` (`self.MoveCounter`)
                (:`  `
                  (goto _label_3 :!via `Reset`))))))
        (:`CastFailed`
          (bind _asplayers_character (cast `/Game/Blueprints/PlayersCharacter` (`self.OwnerCharacter`)))
          (set `/Game/Blueprints/PlayersCharacter.BlockMovements` true _asplayers_character)
          (set `/Game/Blueprints/PlayersCharacter.BlockLook` true _asplayers_character)
          (set `/Game/Blueprints/PlayersCharacter.BlockAttack` true _asplayers_character)
          (set `/Game/Blueprints/PlayersCharacter.BlockDodging` true _asplayers_character)
          (set `/Game/Blueprints/PlayersCharacter.ChangeTimeDilationInPlayersClass` false _asplayers_character)
          (goto _label_2)))
      (else
        (set `self.MoveWhenBlock` false)))
    (else
      (set `self.MoveCounter` 0)
      (`/Engine/EditorBlueprintResources/StandardMacros.DoOnce` true :!label _label_3
        (:`Completed`
          (set `/Game/Blueprints/BaseCharacterClass.Blocked` false (`self.OwnerCharacter`))
          (bind _asbase_npc_2 (cast `/Game/Blueprints/Ai/BaseNPC` (`self.OwnerCharacter`))
            (:`then`
              (set `/Game/Blueprints/Ai/BaseNPC.NpcAttack` true _asbase_npc_2)
              (set `/Game/Blueprints/Ai/BaseNPC.SeesEnemy?` (`/Game/Blueprints/Ai/BaseNPC.TempSeesEnemy` _asbase_npc_2) _asbase_npc_2)
              (set `/Game/Blueprints/Ai/BaseNPC.FollowsEnemy?` (`/Game/Blueprints/Ai/BaseNPC.TempFollowsEnemy` _asbase_npc_2) _asbase_npc_2)
              (goto _label :!via `Reset`))
            (:`CastFailed`
              (bind _asplayers_character_2 (cast `/Game/Blueprints/PlayersCharacter` (`self.OwnerCharacter`)))
              (set `/Game/Blueprints/PlayersCharacter.BlockMovements` false _asplayers_character_2)
              (set `/Game/Blueprints/PlayersCharacter.BlockLook` false _asplayers_character_2)
              (set `/Game/Blueprints/PlayersCharacter.BlockAttack` false _asplayers_character_2)
              (set `/Game/Blueprints/PlayersCharacter.BlockDodging` false _asplayers_character_2)
              (set `/Game/Blueprints/PlayersCharacter.ChangeTimeDilationInPlayersClass` true _asplayers_character_2)
              (bind _asweapon_base_2 (cast `/Game/Blueprints/Weapons/Weapons/WeaponBase` (`ChildActorComponent.ChildActor` (`/Game/Blueprints/BaseCharacterClass.PickableItem` _asplayers_character_2))))
              (set `/Game/Blueprints/Weapons/Weapons/WeaponBase.Blocked` false _asweapon_base_2)
              (set `/Game/Blueprints/Weapons/Weapons/WeaponBase.ResetAttack` true _asweapon_base_2)
              (set `self.MoveWhenBlock` false)
              (goto _label :!via `Reset`))))))))

(event `self.ReceiveBeginPlay`
  (bind _asweapon_base (cast `/Game/Blueprints/Weapons/Weapons/WeaponBase` (`self.GetOwner`)))
  (bind _output_get (set `self.OwnerWeapon` _asweapon_base))
  (bind _asbase_character_class (cast `/Game/Blueprints/BaseCharacterClass` (`Actor.GetParentActor` _output_get)))
  (set `self.OwnerCharacter` _asbase_character_class))

(event `EventBlockOverlap`
  (bind _returnvalue (`AIBlueprintHelperLibrary.GetAIController` (`/Game/Blueprints/Weapons/Weapons/WeaponBase.HitActor` (`self.OwnerWeapon`))))
  (`self.Macro`)
  (set `self.MoveCounter` 0)
  (set `self.MoveWhenBlock` true)
  (`self.AbortAttack`)
  (`/Engine/EditorBlueprintResources/StandardMacros.IsValid` _returnvalue
    (:`Is Valid`
      (`AIController.K2_ClearFocus` _returnvalue))))

(fn `AbortAttack`
  (bind _asweapon_base (cast `/Game/Blueprints/Weapons/Weapons/WeaponBase` (`ChildActorComponent.ChildActor` (`/Game/Blueprints/BaseCharacterClass.PickableItem` (`self.OwnerCharacter`)))))
  (`/Game/Blueprints/Weapons/Weapons/WeaponBase.EventToggleHitCollisions` _asweapon_base false))