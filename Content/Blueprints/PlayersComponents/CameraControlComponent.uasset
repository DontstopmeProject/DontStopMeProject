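; Player camera control component that pans the character's CameraMove component within limits around its starting position.
; MoveCamera scales input, flips X by the game instance's input type, and limits the offset through GetMoveData using MoveRadius.
; MoveCameraBack eases to the saved location and resets Cursor rotation, also firing once on death if CanMoveCursor is set.
; Both moves briefly lift game pause around MoveComponentTo.
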(event `self.ReceiveTick`
  (params (DeltaSeconds :type "Float (single-precision)"))
  (if (and (`/Game/Blueprints/BaseCharacterClass.Dead` (`self.Player`)) (`self.CanMoveCursor`))
    (`/Engine/EditorBlueprintResources/StandardMacros.DoOnce` true :!label _label
      (:`Completed`
        (`self.MoveCameraBack` (`/Game/Blueprints/PlayersCharacter.CameraMove` (`self.Player`)))))
    (else
      (goto _label :!via `Reset`))))

(event `self.ReceiveBeginPlay`
  (bind _asplayers_character (cast `/Game/Blueprints/PlayersCharacter` (`GameplayStatics.GetPlayerCharacter` 0)))
  (bind _output_get (set `self.Player` _asplayers_character))
  (bind _cameramove (`/Game/Blueprints/PlayersCharacter.CameraMove` _output_get))
  (set `self.CameraPosition` (`KismetMathLibrary.MakeTransform` (`SceneComponent.RelativeLocation` _cameramove) (`SceneComponent.RelativeRotation` _cameramove))))

(event `MoveCamera`
  (params (Component :type "SceneComponent Object Reference") (X :type "Float (double-precision)") (Y :type "Float (double-precision)") (IsGamePaused :type Boolean))
  (if (not (`/Game/Blueprints/BaseCharacterClass.Dead` (`self.Player`)))
    (set `self.IsGamePaused` IsGamePaused)
    (bind _asdsm_game_instance (cast `/Game/Blueprints/Dsm_GameInstance` (`GameplayStatics.GetGameInstance`))
      (:`then`
        _)
      (:`CastFailed`
        _))
    (if (`self.IsGamePaused`)
      (`GameplayStatics.SetGamePaused` false))
    (bind (_xout _yout _zout) (`self.GetMoveData` Component (`KismetMathLibrary.SelectFloat` X (* X -1.0) (`|EnumEquality` (`/Game/Blueprints/Dsm_GameInstance.InputType` _asdsm_game_instance) "NewEnumerator0")) Y))
    (`KismetSystemLibrary.MoveComponentTo` Component (`KismetMathLibrary.MakeVector` _xout _yout _zout) (struct) false true 0.0)
    (`/Engine/EditorBlueprintResources/StandardMacros.DoOnce` false :!label _label_2
      (:`Completed`
        (`GameplayStatics.SetGamePaused` false)))))

(event `MoveCameraBack`
  (params (Component :type "SceneComponent Object Reference"))
  (bind _cameraposition_location (`KismetMathLibrary.BreakTransform` (`self.CameraPosition`)))
  (if (`GameplayStatics.IsGamePaused`)
    (`GameplayStatics.SetGamePaused` false)
    (set `self.IsGamePaused` true)
    (else
      (set `self.IsGamePaused` false)))
  (`KismetSystemLibrary.MoveComponentTo` Component _cameraposition_location (struct) false false 0.007)
  (`|ExecutionSequence`
    (:`then_0`
      (if (`self.IsGamePaused`)
        (`GameplayStatics.SetGamePaused` true)
        (goto _label_2 :!via `Reset`)
        (else
          (goto _label_2 :!via `Reset`))))
    (:`then_1`
      (`SceneComponent.K2_SetRelativeRotation` (`/Game/Blueprints/PlayersCharacter.Cursor` (`self.Player`)) (struct :`Pitch` 90.0) false false))))

(fn `GetMoveData`
  (params (Component :type "SceneComponent Object Reference") (X :type "Float (double-precision)") (Y :type "Float (double-precision)"))
  (returns (Xout :type "Float (double-precision)") (Yout :type "Float (double-precision)") (Zout :type "Float (double-precision)"))
  (bind _cameraposition (`self.CameraPosition`))
  (bind _moveradius (`self.MoveRadius`))
  (bind (_relativelocation_x _relativelocation_y _relativelocation_z) (`KismetMathLibrary.BreakVector` (`SceneComponent.RelativeLocation` Component)))
  (bind _cameraposition_2 (`self.CameraPosition`))
  (bind _returnvalue (- (.y (.location _cameraposition)) _moveradius))
  (bind _returnvalue_2 (- (.x (.location _cameraposition_2)) (`self.MoveRadius`)))
  (bind _returnvalue_3 (+ (* Y 10.0) _relativelocation_y))
  (bind _returnvalue_4 (+ (* X 10.0) _relativelocation_x))
  (bind _returnvalue_5 (+ (.y (.location _cameraposition)) _moveradius))
  (bind _returnvalue_6 (+ (.x (.location _cameraposition_2)) (* (`self.MoveRadius`) 0.7)))
  (return (`KismetMathLibrary.SelectFloat` _returnvalue_4 (`KismetMathLibrary.SelectFloat` _returnvalue_6 _returnvalue_2 (> _returnvalue_4 0.0)) (and (>= _returnvalue_6 _returnvalue_4) (<= _returnvalue_2 _returnvalue_4))) (`KismetMathLibrary.SelectFloat` _returnvalue_3 (`KismetMathLibrary.SelectFloat` _returnvalue_5 _returnvalue (> _returnvalue_3 0.0)) (and (>= _returnvalue_5 _returnvalue_3) (<= _returnvalue _returnvalue_3))) _relativelocation_z))