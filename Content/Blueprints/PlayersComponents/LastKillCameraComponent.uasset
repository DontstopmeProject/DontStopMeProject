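; Last-kill camera component on a BaseActionNPC that plays a slow-motion orbit shot of its owner.
; EventPlay blocks input, hides cursor and outlines, switches view to the owner with glitch and sound effects, then returns control after timed delays.
; SetCameraLocation picks a random side, recursively retries on a distance check, and sets tracking focus.
; Tick rotates the camera parent and applies global dilation, handling player death; the skip dispatcher adjusts dilation.
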(event `EventPlay`
  (params (Camera :type "CineCameraComponent Object Reference") (parentSphere :type "SphereComponent Object Reference") (`Actor to Track` :type "Actor Object Reference"))
  (bind _player (`self.Player`))
  (bind _player_2 (`self.Player`))
  (bind _player_3 (`self.Player`))
  (bind _player_4 (`self.Player`))
  (bind _pickableitemvar (`/Game/Blueprints/BaseCharacterClass.PickableItemVar` _player_4))
  (set `self.Parent` parentSphere)
  (set `self.Camera` Camera)
  (set `self.ActorToTrack` `Actor to Track`)
  (`/Engine/EditorBlueprintResources/StandardMacros.DoOnce` false
    (:`Completed`
      (bind _asdsm_gamemode (cast `/Game/Blueprints/DsmGamemode` (`GameplayStatics.GetGameMode`)))
      (set `/Game/Blueprints/DsmGamemode.CustomMusic` true _asdsm_gamemode)
      (bind _returnvalue (`|CreateWidget` "/Game/Blueprints/Widgets/BaseWidgets/GlitchWidget.GlitchWidget_C"))
      (`UserWidget.AddToViewport` _returnvalue 0)
      (`GameplayStatics.PlaySound2D` "/Game/Assets/Sounds/Effects/1Slow_Motion_Sound_Effect__WAV_.1Slow_Motion_Sound_Effect__WAV_")
      (set `self.Counter` 0)
      (`self.ToggleActive` (`self.Camera`))
      (`self.SetCameraLocation`)
      (`PrimitiveComponent.SetRenderCustomDepth` (`Character.Mesh` _player) false)
      (`SceneComponent.SetVisibility` (`/Game/Blueprints/PlayersCharacter.Cursor` _player) false false)
      (set `/Game/Blueprints/PlayersCharacter.MasterEnableTimeDilation` false _player)
      (set `/Game/Blueprints/BaseCharacterClass.StopChangingCustomTime` true _player)
      (`GameplayStatics.SetGamePaused` false)
      (set `Actor.CustomTimeDilation` 1.0 _player)
      (set `self.Dilation` 0.2)
      (`PlayerController.SetViewTargetWithBlend` (`GameplayStatics.GetPlayerController` 0) (`self.GetOwner`) 0.0 "VTBlend_Linear" 0.0 false)
      (set `self.Rotate` true)
      (set `/Game/Blueprints/BaseCharacterClass.CanAttack` false _player_3)
      (`/Game/Blueprints/PlayersCharacter.EventSetInput` _player_3 true true true true true false true true false)
      (`KismetSystemLibrary.Delay` 0.025)
      (`Widget.RemoveFromParent` _returnvalue)
      (`KismetSystemLibrary.Delay` 0.15)
      (set `self.Dilation` 0.05)
      (`KismetSystemLibrary.Delay` 0.2)
      (if (not (`/Game/Blueprints/BaseCharacterClass.Dead` (`self.Player`)))
        (bind _asdsm_gamemode_2 (cast `/Game/Blueprints/DsmGamemode` (`GameplayStatics.GetGameMode`)))
        (`/Game/Blueprints/DsmGamemode.EventToggleMusic` _asdsm_gamemode_2 false)
        (bind _returnvalue_2 (`|CreateWidget` "/Game/Blueprints/Widgets/BaseWidgets/GlitchWidget.GlitchWidget_C"))
        (`UserWidget.AddToViewport` _returnvalue_2 0)
        (`PlayerController.SetViewTargetWithBlend` (`GameplayStatics.GetPlayerController` 0) (`GameplayStatics.GetPlayerCharacter` 0) 0.0 "VTBlend_Linear" 0.0 false)
        (`KismetSystemLibrary.Delay` 0.012)
        (set `/Game/Blueprints/BaseCharacterClass.StopChangingCustomTime` false (`self.Player`))
        (set `self.Rotate` false)
        (set `/Game/Blueprints/BaseCharacterClass.CanAttack` true _player_2)
        (`/Game/Blueprints/PlayersCharacter.EventSetInput` _player_2 false false false false false false false false false)
        (`SceneComponent.SetVisibility` (`/Game/Blueprints/PlayersCharacter.Cursor` _player_2) true false)
        (`Widget.RemoveFromParent` _returnvalue_2)
        (`/Engine/EditorBlueprintResources/StandardMacros.IsValid` _pickableitemvar
          (:`Is Valid`
            (`/Game/Blueprints/Weapons/Weapons/WeaponBase.EventSetRenderCustomDepth` (`/Game/Blueprints/BaseCharacterClass.WeaponBase` _player_4) _pickableitemvar true))
          (:`Is Not Valid`
            _))
        (`PrimitiveComponent.SetRenderCustomDepth` (`Character.Mesh` (`self.Player`)) true)))))

(event `self.ReceiveBeginPlay`
  (bind _asbase_action_npc (cast `/Game/Blueprints/Ai/Enemies/BaseActionNPC` (`self.GetOwner`)))
  (set `self.OwnerCharacter` _asbase_action_npc)
  (bind _asplayers_character (cast `/Game/Blueprints/PlayersCharacter` (`GameplayStatics.GetPlayerCharacter` 0)))
  (set `self.Player` _asplayers_character)
  (add `/Game/Blueprints/PlayersCharacter.SkipDispatcher` (`self.Player`) (delegate `EventSkip`)))

(event `EventSkip`
  (if (`self.Rotate`)
    (set `self.Dilation` 1.0)
    (else
      (set `self.Dilation` 0.05))))

(event `self.ReceiveTick`
  (params (DeltaSeconds :type "Float (single-precision)"))
  (bind (_rotation_roll _rotation_pitch _rotation_yaw) (`KismetMathLibrary.BreakRotator` (`self.Rotation`)))
  (bind _player (`self.Player`))
  (bind _pickableitemvar (`/Game/Blueprints/BaseCharacterClass.PickableItemVar` _player))
  (if (`self.Rotate`)
    (if (`/Game/Blueprints/BaseCharacterClass.Dead` (`self.Player`))
      (`/Engine/EditorBlueprintResources/StandardMacros.DoOnce` false
        (:`Completed`
          (`PlayerController.SetViewTargetWithBlend` (`GameplayStatics.GetPlayerController` 0) (`self.Player`) 0.0 "VTBlend_Linear" 0.0 false)
          (set `self.Rotate` false)
          (`GameplayStatics.SetGlobalTimeDilation` 1.0)
          (`GameplayStatics.PlaySound2D` "/Game/Assets/Sounds/Effects/2Slow_Motion_Sound_Effect__WAV_.2Slow_Motion_Sound_Effect__WAV_")))
      (else
        (`SceneComponent.K2_AddRelativeRotation` (`self.Parent`) (`KismetMathLibrary.MakeRotator` 0.0 0.0 _rotation_yaw) false false)
        (`GameplayStatics.SetGlobalTimeDilation` (`self.Dilation`))
        (set `Actor.CustomTimeDilation` 1.0 (`self.Player`))
        (`/Engine/EditorBlueprintResources/StandardMacros.IsValid` _pickableitemvar
          (:`Is Valid`
            (`/Game/Blueprints/Weapons/Weapons/WeaponBase.EventSetRenderCustomDepth` (`/Game/Blueprints/BaseCharacterClass.WeaponBase` _player) _pickableitemvar false)))))))

(fn `SetCameraLocation`
  (bind _counter (`self.Counter`))
  (bind _returnvalue_location (`KismetMathLibrary.BreakTransform` (`SceneComponent.GetRelativeTransform` (`self.Camera`))))
  (bind _returnvalue_location_2 (`KismetMathLibrary.BreakTransform` (`SceneComponent.GetRelativeTransform` (`Character.Mesh` (`self.OwnerCharacter`)))))
  (bind _returnvalue (`KismetMathLibrary.GetPointDistanceToLine` (`self.Location`) _returnvalue_location_2 (`SceneComponent.GetForwardVector` (`self.Camera`))))
  (bind _output_get (set `self.Int` (`KismetMathLibrary.RandomIntegerInRange` 0 1)))
  (`SceneComponent.K2_SetRelativeRotation` (`self.Parent`) (`KismetMathLibrary.MakeRotator` 0.0 0.0 (select `int` _output_get :`0` (`KismetMathLibrary.RandomFloatInRange` -50.0 -110.0) :`1` (`KismetMathLibrary.RandomFloatInRange` 150.0 68.0))) false false)
  (set `self.Location` _returnvalue_location)
  (set `self.Rotation` (`KismetMathLibrary.MakeRotator` 0.0 0.0 (select `int` (`self.Int`) :`0` 0.2 :`1` -0.2 :!type "Float (single-precision)")))
  (if (< _returnvalue 1000.0)
    (if (<= _counter 20)
      (`/Engine/EditorBlueprintResources/StandardMacros.IncrementInt` _counter
        (:`  `
          (`self.SetCameraLocation`)))
      (else
        (set `self.Counter` 0 :!label _label)
        (set `CineCameraComponent.FocusSettings` (make `CameraFocusSettings` "Tracking" _returnvalue (make `CameraTrackingFocusSettings` (`self.ActorToTrack`)) true) (`self.Camera`))))
    (else
      (goto _label))))