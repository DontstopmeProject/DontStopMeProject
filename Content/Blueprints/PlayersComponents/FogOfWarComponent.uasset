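; Fog of war component for the player that toggles visibility of NPCs and weapons caught in a cone-shaped trace.
; EventActivateFW approximates the cone with stepped sphere traces of varying radius along the player mesh's right vector, collecting hit actors.
; ToggleVis compares hits against CurrentActor, then flips visibility of living, active action NPCs with their weapons, or of weapons and their NPC owners.
; The hit list is cleared inside its processing loop, and debug drawing is on.
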(event `self.ReceiveBeginPlay`
  (set `self.Radius` (`self.StartRadius`)))

(event `EventActivateFW`
  (bind _conetraceoffset (`self.ConeTraceOffset`))
  (bind _returnvalue (/ 1.0 (`KismetMathLibrary.Conv_IntToDouble` (`self.TraceSteps`))))
  (bind _mesh (`Character.Mesh` (cast `/Game/Blueprints/PlayersCharacter` (`GameplayStatics.GetPlayerCharacter` 0) :!pure true)))
  (bind _returnvalue_2 (`SceneComponent.K2_GetComponentLocation` _mesh))
  (bind _output_get (set `self.ConeTraceOffset` (+ _returnvalue_2 (* (`SceneComponent.GetRightVector` _mesh) (/ 1.0 (`KismetMathLibrary.Conv_IntToDouble` (`self.TraceSteps`)))))))
  (bind _outhit (`KismetSystemLibrary.SphereTraceSingleForObjects` _returnvalue_2 _output_get (`self.Radius`) (`|MakeArray` "ObjectTypeQuery4" "ObjectTypeQuery10" "ObjectTypeQuery13" :!type "EObjectTypeQuery Enum") false (`|MakeArray` (`GameplayStatics.GetPlayerCharacter` 0)) "ForOneFrame"))
  (`KismetArrayLibrary.Array_Add` (`self.HitActors`) (`.HitActor` (`GameplayStatics.BreakHitResult` _outhit)))
  (for _index (range 2 (+ (`self.TraceSteps`) 1))
    (set `self.Index` _index)
    (bind _output_get_2 (set `self.ConeTraceOffset` (+ _conetraceoffset (* (`SceneComponent.GetRightVector` (`Character.Mesh` (cast `/Game/Blueprints/PlayersCharacter` (`GameplayStatics.GetPlayerCharacter` 0) :!pure true))) (* (`self.TraceDistance`) _returnvalue)))))
    (bind _outhit_2 (`KismetSystemLibrary.SphereTraceSingleForObjects` _conetraceoffset _output_get_2 (`KismetMathLibrary.MapRangeClamped` (* (`KismetMathLibrary.Conv_IntToDouble` (`self.Index`)) _returnvalue) 0.0 1.0 (`self.StartRadius`) (`self.EndRadius`)) (`|MakeArray` "ObjectTypeQuery4" "ObjectTypeQuery10" "ObjectTypeQuery13" :!type "EObjectTypeQuery Enum") false (`|MakeArray` (`GameplayStatics.GetPlayerCharacter` 0)) "ForOneFrame"))
    (`KismetArrayLibrary.Array_Add` (`self.HitActors`) (`.HitActor` (`GameplayStatics.BreakHitResult` _outhit_2))))
  (for _array_element (`self.HitActors`)
    (`/Engine/EditorBlueprintResources/StandardMacros.IsValid` _array_element
      (:`Is Valid`
        (`self.ToggleVis` _array_element))
      (:`Is Not Valid`
        _))
    (`KismetArrayLibrary.Array_Clear` (`self.HitActors`))))

(fn `FetchArrayVis`
  (params (Array :type "Array of SceneComponent Object Reference"))
  (for _array_element Array
    (if (`SceneComponent.IsVisible` _array_element)
      (`SceneComponent.SetVisibility` _array_element false true)
      (else
        (`SceneComponent.SetVisibility` _array_element true true)))))

(fn `ToggleVis`
  (params (TracedActor :type "Actor Object Reference"))
  (bind _returnvalue (`Actor.GetOwner` TracedActor))
  (if (!= (select `bool` (`KismetSystemLibrary.IsValid` _returnvalue) :`false` TracedActor :`true` _returnvalue :!type "Object Object Reference") (`self.CurrentActor`))
    (bind _output_get (set `self.CurrentActor` TracedActor))
    (bind _asbase_npc (cast `/Game/Blueprints/Ai/BaseNPC` _output_get)
      (:`then`
        (bind _asbase_action_npc (cast `/Game/Blueprints/Ai/Enemies/BaseActionNPC` _asbase_npc))
        (if (and (`/Game/Blueprints/Ai/Enemies/BaseActionNPC.Active` _asbase_action_npc) (not (`/Game/Blueprints/BaseCharacterClass.Dead` _asbase_action_npc)))
          (for _array_element (`|MakeArray` (`Actor.RootComponent` (`/Game/Blueprints/BaseCharacterClass.EquipedWeaponL` _asbase_action_npc)) (`Character.Mesh` _asbase_action_npc) (`Actor.RootComponent` (`/Game/Blueprints/BaseCharacterClass.EquipedWeapon` _asbase_action_npc)) :!type "SceneComponent Object Reference")
            (if (`SceneComponent.IsVisible` _array_element)
              (`SceneComponent.SetVisibility` _array_element false true)
              (else
                (`SceneComponent.SetVisibility` _array_element true true))))))
      (:`CastFailed`
        (bind _asweapon_base (cast `/Game/Blueprints/Weapons/Weapons/WeaponBase` (`self.CurrentActor`)))
        (if (`/Game/Blueprints/Weapons/Weapons/WeaponBase.PlacedManualy` _asweapon_base)
          (bind _rootcomponent (`Actor.RootComponent` _asweapon_base))
          (`self.FetchArrayVis` (`|MakeArray` _rootcomponent))
          (else
            (bind _returnvalue_2 (`Actor.GetOwner` _asweapon_base))
            (`/Engine/EditorBlueprintResources/StandardMacros.IsValid` _returnvalue_2
              (:`Is Valid`
                (bind _asbase_action_npc_2 (cast `/Game/Blueprints/Ai/Enemies/BaseActionNPC` _returnvalue_2))
                (`self.FetchArrayVis` (`|MakeArray` (`Actor.RootComponent` _asbase_action_npc_2) _rootcomponent))))))))))