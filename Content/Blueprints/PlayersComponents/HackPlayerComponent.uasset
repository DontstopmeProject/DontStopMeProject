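; Player component that lets the player hack NPCs, temporarily turning them against their own side.
; While tracking, Tick capsule-traces from the cursor for a target, manages a dialog window and reports status in a console widget.
; EventHack restores game time, starts a cooldown, highlights the NPC via custom depth stencil and swaps its enemy class and tag.
; If the player is alive, a delay later reverts these and clears matching groupmate enemies.
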(event `self.ReceiveBeginPlay`
  (bind _asplayers_character (cast `/Game/Blueprints/PlayersCharacter` (`self.GetOwner`)))
  (set `self.Player` _asplayers_character))

(event `self.ReceiveTick`
  (params (DeltaSeconds :type "Float (single-precision)"))
  (bind _widget (`self.Widget`))
  (bind _widget_2 (`self.Widget`))
  (bind _dialogwindow (`self.DialogWindow`))
  (bind _widget_3 (`self.Widget`))
  (bind _player (`self.Player`))
  (bind _returnvalue_location (`KismetMathLibrary.BreakTransform` (`SceneComponent.K2_GetComponentToWorld` (`/Game/Blueprints/PlayersCharacter.Cursor` _player))))
  (if (`/Game/Blueprints/PlayersCharacter.GamePaused` (`self.Player`))
    _
    (elif (`self.ReadyToTrack`)
      (`|ExecutionSequence`
        (:`then_0`
          (`|ExecutionSequence`
            (:`then_0`
              (goto _label_5 :!via `Reset`))
            (:`then_1`
              (`/Engine/EditorBlueprintResources/StandardMacros.IsValid` _dialogwindow :!label _label
                (:`Is Valid`
                  (`Actor.K2_DestroyActor` _dialogwindow)
                  (goto _label_4 :!via `Reset`))
                (:`Is Not Valid`
                  (goto _label_4 :!via `Reset`))))))
        (:`then_1`
          (if (`self.StartTracking`)
            (bind _outhit (`KismetSystemLibrary.CapsuleTraceSingleForObjects` :`Start` _returnvalue_location :`End` (+ _returnvalue_location (* (`SceneComponent.GetUpVector` (`Actor.RootComponent` _player)) 1000.0)) :`Radius` 30.0 :`HalfHeight` 1000.0 :`ObjectTypes` (`|MakeArray` "ObjectTypeQuery13" :!type "EObjectTypeQuery Enum") :`DrawDebugType` "ForOneFrame"))
            (`|ExecutionSequence`
              (:`then_0`
                (`/Engine/EditorBlueprintResources/StandardMacros.DoOnce` false :!label _label_2
                  (:`Completed`
                    (`/Engine/EditorBlueprintResources/StandardMacros.IsValid` _widget_2
                      (:`Is Valid`
                        (if (not (`Widget.IsVisible` _widget_2))
                          (bind _returnvalue (`|CreateWidget` "/Game/Blueprints/Widgets/W_TestHackLine.W_TestHackLine_C" :!label _label_3))
                          (bind _output_get (set `self.Widget` _returnvalue))
                          (`UserWidget.AddToViewport` _output_get 10)))
                      (:`Is Not Valid`
                        (goto _label_3)))
                    (`/Game/Blueprints/Widgets/W_TestHackLine.event Console` (`self.Widget`) "hacking mode on"))))
              (:`then_1`
                (`/Engine/EditorBlueprintResources/StandardMacros.IsValid` (`.HitActor` (`GameplayStatics.BreakHitResult` _outhit))
                  (:`Is Valid`
                    (set `self.TrackedActor` (`.HitActor` (`GameplayStatics.BreakHitResult` _outhit)))
                    (`/Engine/EditorBlueprintResources/StandardMacros.DoOnce` false :!label _label_4
                      (:`Completed`
                        (set `self.Actor` (`self.TrackedActor`))
                        (bind _returnvalue_2 (`|SpawnActorFromClass` "/Game/Blueprints/Widgets/BaseWidgets/BP_DialogWindow.BP_DialogWindow_C" (`KismetMathLibrary.Conv_VectorToTransform` (+ (0.0 0.0 0.0) (0.0 0.0 230.0))) "Undefined" "OverrideRootScale" null null))
                        (set `self.DialogWindow` _returnvalue_2))))
                  (:`Is Not Valid`
                    (set `self.TrackedActor` null)
                    (goto _label)))))
            (else
              (`|ExecutionSequence`
                (:`then_0`
                  (goto _label_2 :!via `Reset`))
                (:`then_1`
                  (`/Engine/EditorBlueprintResources/StandardMacros.IsValid` _widget_3
                    (:`Is Valid`
                      (if (`Widget.IsVisible` _widget_3)
                        (`|ExecutionSequence`
                          (:`then_0`
                            (`KismetSystemLibrary.Delay` 1.0)
                            (`Widget.RemoveFromParent` _widget))
                          (:`then_1`
                            (goto _label)))
                        (else
                          (goto _label))))
                    (:`Is Not Valid`
                      (goto _label)))))))))
      (else
        (`|ExecutionSequence`
          (:`then_0`
            (goto _label_2 :!via `Reset`))
          (:`then_1`
            (bind _output_get_2 (set `self.Timer` (+ DeltaSeconds (`self.Timer`))))
            (if (>= _output_get_2 15.0)
              (set `self.ReadyToTrack` true)
              (set `self.Timer` 0.0)
              (`/Game/Blueprints/Widgets/W_TestHackLine.event Console` _widget "Ready to hack...")
              (else
                (set `self.StartTracking` false)
                (set `self.TrackedActor` null)
                (`/Engine/EditorBlueprintResources/StandardMacros.DoOnce` false :!label _label_5
                  (:`Completed`
                    (`KismetSystemLibrary.Delay` 1.5)
                    (`/Game/Blueprints/Widgets/W_TestHackLine.event Console` _widget_3 "Trying to reconnect... \nPlease wait...")))))))))))

(event `EventHack`
  (bind _baseactionnpc (`self.BaseActionNpc`))
  (bind _trackedactor (`self.TrackedActor`))
  (`|ExecutionSequence`
    (:`then_0`
      (goto _label_2 :!via `Reset`))
    (:`then_2`
      (bind _asbase_action_npc (cast `/Game/Blueprints/Ai/Enemies/BaseActionNPC` _trackedactor)
        (:`then`
          (set `self.ReadyToTrack` false)
          (set `self.Timer` 0.0)
          (set `self.StartTracking` false)
          (set `/Game/Blueprints/BaseCharacterClass.ResetThrow` true (`self.Player`))
          (`GameplayStatics.SetGamePaused` false)
          (`GameplayStatics.SetGlobalTimeDilation` 1.0)
          (`/Game/Blueprints/Widgets/W_TestHackLine.event Console` (`self.Widget`) "hack successful")
          (`self.HackingEventDispatcher`)
          (bind _mesh (`Character.Mesh` _asbase_action_npc))
          (`PrimitiveComponent.SetRenderCustomDepth` _mesh true)
          (`PrimitiveComponent.SetCustomDepthStencilValue` _mesh 252)
          (set `/Game/Blueprints/Ai/Enemies/BaseActionNPC.Hacked` true _asbase_action_npc)
          (set `self.BaseActionNpc` _asbase_action_npc)
          (set `/Game/Blueprints/BaseCharacterClass.ResetThrow` true _asbase_action_npc)
          (bind _enemiesarray (`/Game/Blueprints/Ai/Enemies/BaseActionNPC.EnemiesArray` _asbase_action_npc))
          (`KismetArrayLibrary.Array_Set` _enemiesarray (`KismetArrayLibrary.Array_Find` _enemiesarray (`GameplayStatics.GetObjectClass` (`GameplayStatics.GetPlayerCharacter` 0))) (`GameplayStatics.GetObjectClass` _trackedactor) true)
          (bind _tags (`Actor.Tags` _asbase_action_npc))
          (`KismetArrayLibrary.Array_Set` _tags 2 "player" true)
          (`KismetSystemLibrary.Delay` 0.5)
          (set `/Game/Blueprints/Ai/Enemies/BaseActionNPC.Enemy` null _asbase_action_npc)
          (if (not (`/Game/Blueprints/BaseCharacterClass.Dead` (`self.Player`)))
            (`KismetSystemLibrary.Delay` 8.0)
            (`KismetArrayLibrary.Array_Set` _enemiesarray (`KismetArrayLibrary.Array_Find` _enemiesarray (`GameplayStatics.GetObjectClass` (`self.Actor`))) (`GameplayStatics.GetObjectClass` (`GameplayStatics.GetPlayerCharacter` 0)) true)
            (`KismetArrayLibrary.Array_Set` _tags 2 "mafia" true)
            (for _array_element (`/Game/Blueprints/Ai/Enemies/BaseActionNPC.Group` _baseactionnpc)
              (bind _asbase_action_npc_2 (cast `/Game/Blueprints/Ai/Enemies/BaseActionNPC` _array_element))
              (if (== (`/Game/Blueprints/Ai/Enemies/BaseActionNPC.GroupmateEnemy` _asbase_action_npc_2) (`/Game/Blueprints/Ai/Enemies/BaseActionNPC.GroupmateEnemy` _baseactionnpc))
                (set `/Game/Blueprints/Ai/Enemies/BaseActionNPC.GroupmateEnemy` null _asbase_action_npc_2)))
            (set `/Game/Blueprints/BaseCharacterClass.ResetThrow` true _baseactionnpc)
            (set `/Game/Blueprints/Ai/Enemies/BaseActionNPC.Hacked` false _baseactionnpc)
            (`PrimitiveComponent.SetCustomDepthStencilValue` (`Character.Mesh` _baseactionnpc) 254)))
        (:`CastFailed`
          (set `self.ReadyToTrack` true)
          (set `self.Timer` 15.0))))))