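; TraceComponent is a player component that detects an AI pawn in a short box trace and clears its attack flags.
; EventTrace casts the box along the target component's right vector, ignoring the player character cached at BeginPlay.
; On hitting an "ai"-tagged BaseNPC, it sets NpcAttack and its held weapon's StopAttack to false.
; A DoOnce reset after a delay throttles repeated traces.
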(event `self.ReceiveBeginPlay`
  (bind _asplayers_character (cast `/Game/Blueprints/PlayersCharacter` (`GameplayStatics.GetPlayerCharacter` 0)))
  (set `self.Player` _asplayers_character))

(event `EventTrace`
  (params (TargetComponent :type "SceneComponent Object Reference"))
  (bind _returnvalue (`SceneComponent.GetRightVector` TargetComponent))
  (bind _returnvalue_2 (+ (`SceneComponent.K2_GetComponentLocation` TargetComponent) (* _returnvalue 5.0)))
  (`/Engine/EditorBlueprintResources/StandardMacros.DoOnce` false :!label _label
    (:`Completed`
      (bind _outhit (`KismetSystemLibrary.BoxTraceSingleForObjects` _returnvalue_2 (+ _returnvalue_2 (* _returnvalue 200.0)) (50.0 50.0 50.0) (struct) (`|MakeArray` "ObjectTypeQuery3" :!type "EObjectTypeQuery Enum") false (`|MakeArray` (`self.Player`) :!type "Actor Object Reference")))
      (`/Engine/EditorBlueprintResources/StandardMacros.IsValid` (`.HitActor` (`GameplayStatics.BreakHitResult` _outhit))
        (:`Is Valid`
          (if (`Actor.ActorHasTag` (`.HitActor` (`GameplayStatics.BreakHitResult` _outhit)) "ai")
            (bind _asbase_npc (cast `/Game/Blueprints/Ai/BaseNPC` (`.HitActor` (`GameplayStatics.BreakHitResult` _outhit)))
              (:`then`
                (set `/Game/Blueprints/Ai/BaseNPC.NpcAttack` false _asbase_npc)
                (bind _asweapon_base (cast `/Game/Blueprints/Weapons/Weapons/WeaponBase` (`ChildActorComponent.ChildActor` (`/Game/Blueprints/BaseCharacterClass.PickableItem` _asbase_npc)))
                  (:`then`
                    (set `/Game/Blueprints/Weapons/Weapons/WeaponBase.StopAttack` false _asweapon_base))
                  (:`CastFailed`
                    _)))
              (:`CastFailed`
                _))))
        (:`Is Not Valid`
          _))
      (`KismetSystemLibrary.Delay` 2.0)
      (goto _label :!via `Reset`))))