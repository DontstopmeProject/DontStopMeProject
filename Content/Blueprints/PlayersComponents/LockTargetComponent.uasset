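; Player lock-on component that drives the player's cursor and locks it onto the nearest enemy.
; GetClosestTarget picks from ClosestPawns by distance, outlines the target via custom depth stencil, slightly narrows camera FOV and shows a widget.
; Tick holds the cursor on the target, with release logic for death or dodge.
; Unlocked, the cursor follows mouse hits or gamepad stick offsets, or snaps ahead of the player when dodge is ready.
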(event Custom|MakeLock
  (params (Condition :type Boolean))
  (if Condition
    (Game|SetGamePaused false)
    (Variables|Default|SetMoveToLock true)
    (else
      (Variables|Default|SetMoveToLock true)))
  (if Condition
    (Utilities|FlowControl|Delay 0.2)
    (bind _asplayers_character (Utilities|Casting|CastToPlayersCharacter (Game|GetPlayerCharacter 0)))
    (if (Variables|/Game/Blueprints/PlayersCharacter.PlayersCharacter_C|GetChangeTimeDilationInPlayersClass _asplayers_character)
      (Game|SetGamePaused true))))

(event EventBeginPlay
  (bind _asplayers_character (Utilities|Casting|CastToPlayersCharacter (Game|GetPlayerCharacter 0)))
  (bind _output_get (Variables|Default|SetPlayer _asplayers_character))
  (Variables|Default|SetOriginal%20Rotation (Pawn|GetControlRotation _output_get :!class /Script/Engine.Pawn)))

(event EventTick
  (params (DeltaSeconds :type Float%20%28single-precision%29))
  (bind _returnvalue (Game|GetPlayerController 0))
  (bind _player (Variables|Default|GetPlayer))
  (bind _player_2 (Variables|Default|GetPlayer))
  (bind _player_3 (Variables|Default|GetPlayer))
  (bind _player_4 (Variables|Default|GetPlayer))
  (bind _rotationtarget (Variables|Default|GetRotationTarget))
  (bind _player_5 (Variables|Default|GetPlayer))
  (bind _returnvalue_2 (Transformation|GetActorLocation _rotationtarget))
  (bind _hitresult (Game|Player|GetHitResultUnderCursorbyChannel _returnvalue "TraceTypeQuery1" false))
  (bind _cursor (Variables|/Game/Blueprints/PlayersCharacter.PlayersCharacter_C|GetCursor _player_4))
  (bind _cursor_2 (Variables|/Game/Blueprints/PlayersCharacter.PlayersCharacter_C|GetCursor _player))
  (bind _returnvalue_3 (Transformation|GetRelativeTransform _cursor))
  (bind (_bblockinghit _binitialoverlap _time _location _impactpoint) (Collision|BreakHitResult _hitresult))
  (if (not (or (Variables|/Game/Blueprints/BaseCharacterClass.BaseCharacterClass_C|GetDead _player_2) (Variables|/Game/Blueprints/PlayersCharacter.PlayersCharacter_C|GetGamePaused _player_2)))
    (if (Variables|Default|GetLock)
      (Utilities|IsValid (Variables|Default|GetRotationTarget)
        (:Is%20Valid
          (bind _asbase_character_class (Utilities|Casting|CastToBaseCharacterClass (Variables|Default|GetRotationTarget))
            (:then
              (if (Variables|/Game/Blueprints/BaseCharacterClass.BaseCharacterClass_C|GetDead _asbase_character_class)
                (Camera|SetFieldOfView (Variables|/Game/Blueprints/PlayersCharacter.PlayersCharacter_C|GetCamera (Variables|Default|GetPlayer)) (Variables|Default|GetPlayersFOV) :!label _label)
                (Variables|Default|SetLock false)
                (Widget|RemovefromParent (Variables|Default|GetWidget))
                (Variables|Default|SetReturnToZero true)
                (elif (Variables|/Game/Blueprints/BaseCharacterClass.BaseCharacterClass_C|GetDodge _asbase_character_class)
                  (goto _label_2 Reset)
                  (else
                    (bind _output_get (Variables|Default|SetTargetLocation (Math|Vector|MakeVector (.x _returnvalue_2) (.y _returnvalue_2) (.z (Transformation|GetWorldLocation _cursor_2)))))
                    (if (CallFunction|CanMoveCursor)
                      (Transformation|SetWorldLocationAndRotation _cursor_2 _output_get (Transformation|GetWorldRotation _cursor_2) false false)
                      (goto _label_2 Reset)
                      (else
                        (goto _label_2 Reset)))))))
            (:CastFailed
              (goto _label_2 Reset))))
        (:Is%20Not%20Valid
          (goto _label_2 Reset)))
      (elif (Variables|/Game/Blueprints/PlayersComponents/Dodge/DodgeComponent1.DodgeComponent1_C|GetReadyForDodge (Variables|/Game/Blueprints/PlayersCharacter.PlayersCharacter_C|GetDodgeComponent1 (Variables|Default|GetPlayer)))
        (goto _label_3 Reset)
        (else
          (bind _asdsm_game_instance (Utilities|Casting|CastToDsm_GameInstance (Game|GetGameInstance)))
          (switch Utilities|FlowControl|Switch|SwitchonInputTypeEnum (Variables|/Game/Blueprints/Dsm_GameInstance.Dsm_GameInstance_C|GetInputType _asdsm_game_instance)
            (:NewEnumerator0
              (Variables|Default|SetTargetLocation (Math|Vector|MakeVector (.x _location) (.y _location) (.z _location)))
              (Variables|Default|SetOriginal%20Rotation "19.687439, 0, 0")
              (if (CallFunction|CanMoveCursor)
                (Transformation|SetWorldLocationAndRotation (Variables|/Game/Blueprints/PlayersCharacter.PlayersCharacter_C|GetCursor (Variables|Default|GetPlayer)) (Variables|Default|GetTargetLocation) (Variables|Default|GetOriginal%20Rotation) false false))
              (Utilities|FlowControl|Sequence
                (:then_0
                  (goto _label_3 Reset))
                (:then_1
                  (Utilities|FlowControl|DoOnce true :!label _label_2
                    (:Completed
                      (bind _asbase_action_npc (Utilities|Casting|CastToBaseActionNPC (Variables|Default|GetRotationTarget))
                        (:then
                          (Rendering|SetCustomDepthStencilValue (Variables|/Script/Engine.Character|GetMesh _asbase_action_npc) 254)
                          (goto _label))
                        (:CastFailed
                          (goto _label))))))))
            (:NewEnumerator1
              (Utilities|FlowControl|Sequence
                (:then_0
                  (Utilities|FlowControl|DoOnce false :!label _label_3
                    (:Completed
                      (if (CallFunction|CanMoveCursor)
                        (Transformation|SetRelativeLocation _cursor "100.000000, 0,-90.000000" false false)
                        (Transformation|SetRelativeRotation _cursor "19.687439, 0, 0" false false)))))
                (:then_1
                  (if (!= (Math|Vector2D|Vector2DLength (Math|Vector2D|MakeVector2D (Variables|/Game/Blueprints/PlayersCharacter.PlayersCharacter_C|GetLookF/B _player_5) (Variables|/Game/Blueprints/BaseCharacterClass.BaseCharacterClass_C|GetTurn _player_5))) 0.0)
                    (bind _result (Math|Float|NegateFloat (* (Variables|/Game/Blueprints/PlayersCharacter.PlayersCharacter_C|GetLookF/B _player_3) 18.0))
                      (:%20%20
                        (if (CallFunction|CanMoveCursor)
                          (Transformation|AddLocalOffset _cursor (Math|Vector|MakeVector _result (* (Variables|/Game/Blueprints/BaseCharacterClass.BaseCharacterClass_C|GetTurn _player_3) 18.0) 0.0) true false)
                          (Transformation|SetRelativeLocation _cursor (Math|Vector|MakeVector (.x (.location _returnvalue_3)) (.y (.location _returnvalue_3)) -9e+01) false false)
                          (goto _label_2))))
                    (else
                      (goto _label_2))))))))))))

(fn GetClosestTarget
  (params (Owner :type Actor%20Object%20Reference))
  (bind _asplayers_character (Utilities|Casting|CastToPlayersCharacter Owner))
  (Variables|Default|SetPlayer _asplayers_character)
  (for (_array_element _array_index) (Variables|Default|GetClosestPawns)
    (if (== _array_index 0)
      (bind _asbase_action_npc (Utilities|Casting|CastToBaseActionNPC _array_element))
      (if (Variables|/Game/Blueprints/Ai/Enemies/BaseActionNPC.BaseActionNPC_C|GetActive _asbase_action_npc)
        (LocalVariables|SetClosestRange (|(sqrt((((x*x)+(y*y))+(z*z)))) (.x (Math|Vector|MakeVector (- (.x (Transformation|GetActorLocation _array_element)) (.x (Transformation|GetActorLocation (Variables|Default|GetPlayer)))) (- (.y (Transformation|GetActorLocation _array_element)) (.y (Transformation|GetActorLocation (Variables|Default|GetPlayer)))) (- (.z (Transformation|GetActorLocation _array_element)) (.z (Transformation|GetActorLocation (Variables|Default|GetPlayer)))))) (.y (Math|Vector|MakeVector (- (.x (Transformation|GetActorLocation _array_element)) (.x (Transformation|GetActorLocation (Variables|Default|GetPlayer)))) (- (.y (Transformation|GetActorLocation _array_element)) (.y (Transformation|GetActorLocation (Variables|Default|GetPlayer)))) (- (.z (Transformation|GetActorLocation _array_element)) (.z (Transformation|GetActorLocation (Variables|Default|GetPlayer)))))) (.z (Math|Vector|MakeVector (- (.x (Transformation|GetActorLocation _array_element)) (.x (Transformation|GetActorLocation (Variables|Default|GetPlayer)))) (- (.y (Transformation|GetActorLocation _array_element)) (.y (Transformation|GetActorLocation (Variables|Default|GetPlayer)))) (- (.z (Transformation|GetActorLocation _array_element)) (.z (Transformation|GetActorLocation (Variables|Default|GetPlayer))))))))
        (LocalVariables|SetFIndedActor _array_element))
      (elif (>= (LocalVariables|GetClosestRange) (|(sqrt((((x*x)+(y*y))+(z*z)))) (.x (Math|Vector|MakeVector (- (.x (Transformation|GetActorLocation _array_element)) (.x (Transformation|GetActorLocation (Variables|Default|GetPlayer)))) (- (.y (Transformation|GetActorLocation _array_element)) (.y (Transformation|GetActorLocation (Variables|Default|GetPlayer)))) (- (.z (Transformation|GetActorLocation _array_element)) (.z (Transformation|GetActorLocation (Variables|Default|GetPlayer)))))) (.y (Math|Vector|MakeVector (- (.x (Transformation|GetActorLocation _array_element)) (.x (Transformation|GetActorLocation (Variables|Default|GetPlayer)))) (- (.y (Transformation|GetActorLocation _array_element)) (.y (Transformation|GetActorLocation (Variables|Default|GetPlayer)))) (- (.z (Transformation|GetActorLocation _array_element)) (.z (Transformation|GetActorLocation (Variables|Default|GetPlayer)))))) (.z (Math|Vector|MakeVector (- (.x (Transformation|GetActorLocation _array_element)) (.x (Transformation|GetActorLocation (Variables|Default|GetPlayer)))) (- (.y (Transformation|GetActorLocation _array_element)) (.y (Transformation|GetActorLocation (Variables|Default|GetPlayer)))) (- (.z (Transformation|GetActorLocation _array_element)) (.z (Transformation|GetActorLocation (Variables|Default|GetPlayer))))))))
        (LocalVariables|SetClosestRange (|(sqrt((((x*x)+(y*y))+(z*z)))) (.x (Math|Vector|MakeVector (- (.x (Transformation|GetActorLocation _array_element)) (.x (Transformation|GetActorLocation (Variables|Default|GetPlayer)))) (- (.y (Transformation|GetActorLocation _array_element)) (.y (Transformation|GetActorLocation (Variables|Default|GetPlayer)))) (- (.z (Transformation|GetActorLocation _array_element)) (.z (Transformation|GetActorLocation (Variables|Default|GetPlayer)))))) (.y (Math|Vector|MakeVector (- (.x (Transformation|GetActorLocation _array_element)) (.x (Transformation|GetActorLocation (Variables|Default|GetPlayer)))) (- (.y (Transformation|GetActorLocation _array_element)) (.y (Transformation|GetActorLocation (Variables|Default|GetPlayer)))) (- (.z (Transformation|GetActorLocation _array_element)) (.z (Transformation|GetActorLocation (Variables|Default|GetPlayer)))))) (.z (Math|Vector|MakeVector (- (.x (Transformation|GetActorLocation _array_element)) (.x (Transformation|GetActorLocation (Variables|Default|GetPlayer)))) (- (.y (Transformation|GetActorLocation _array_element)) (.y (Transformation|GetActorLocation (Variables|Default|GetPlayer)))) (- (.z (Transformation|GetActorLocation _array_element)) (.z (Transformation|GetActorLocation (Variables|Default|GetPlayer))))))))
        (LocalVariables|SetFIndedActor _array_element))))
  (Utilities|IsValid (LocalVariables|GetFIndedActor)
    (:Is%20Valid
      (bind _aspawn (Utilities|Casting|CastToPawn (LocalVariables|GetFIndedActor)))
      (bind _asbase_character_class (Utilities|Casting|CastToBaseCharacterClass (LocalVariables|GetFIndedActor)))
      (if (not (Variables|/Game/Blueprints/BaseCharacterClass.BaseCharacterClass_C|GetDead _asbase_character_class))
        (bind _output_get (Variables|Default|SetRotationTarget _aspawn))
        (Variables|Default|SetTargetLocation (Transformation|GetActorLocation (Variables|Default|GetRotationTarget)))
        (Variables|Default|SetLock true)
        (bind _asbase_action_npc_2 (Utilities|Casting|CastToBaseActionNPC _output_get))
        (Rendering|SetRenderCustomDepth (Variables|/Script/Engine.Character|GetMesh _asbase_action_npc_2) true)
        (Rendering|SetCustomDepthStencilValue (Variables|/Script/Engine.Character|GetMesh _asbase_action_npc_2) 253)
        (bind _output_get_2 (Variables|Default|SetPlayersFOV (Variables|/Script/Engine.CameraComponent|GetFieldOfView (Variables|/Game/Blueprints/PlayersCharacter.PlayersCharacter_C|GetCamera (Variables|Default|GetPlayer)))))
        (Camera|SetFieldOfView (Variables|/Game/Blueprints/PlayersCharacter.PlayersCharacter_C|GetCamera (Variables|Default|GetPlayer)) (* _output_get_2 0.98))
        (Utilities|IsValid (Variables|Default|GetWidget)
          (:Is%20Valid
            (UserInterface|Viewport|AddtoViewport (Variables|Default|GetWidget) 0))
          (:Is%20Not%20Valid
            (bind _returnvalue (UserInterface|CreateWidget "/Game/Blueprints/Widgets/BaseWidgets/CS.CS_C"))
            (bind _output_get_3 (Variables|Default|SetWidget _returnvalue))
            (UserInterface|Viewport|AddtoViewport _output_get_3 0)))
        (Utilities|Casting|CastToPlayersCharacter (Components|GetOwner))
        (CallFunction|MakeLock (Game|IsGamePaused))))))

(fn CanMoveCursor
  (return (Variables|/Game/Blueprints/PlayersComponents/CameraControlComponent.CameraControlComponent_C|GetCanMoveCursor (Variables|/Game/Blueprints/PlayersCharacter.PlayersCharacter_C|GetCameraControlComponent (Variables|Default|GetPlayer)))))