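; Character component that handles melee blocking by checking for an opposing character in front of its owner.
; SetBlockArea enables a per-tick pawn sphere trace, which continues only while a character is found whose held weapon is no tougher than the owner's.
; DoOnce gates fire the owner weapon's EventBlock with or without a target, resetting when tracing stops.
; For player-tagged owners, the hit path also sets Blocked on the stored target weapon.
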(event `self.ReceiveBeginPlay`
  (bind _asbase_character_class (cast `/Game/Blueprints/BaseCharacterClass` (`self.GetOwner`)))
  (set `self.OwnerBaseCharacter` _asbase_character_class))

(event `SetBlockArea`
  (set `self.Bool` true))

(event `self.ReceiveTick`
  (params (DeltaSeconds :type "Float (single-precision)"))
  (bind _ownerbasecharacter (`self.OwnerBaseCharacter`))
  (bind _returnvalue (+ (`Actor.K2_GetActorLocation` _ownerbasecharacter) (* (`Actor.GetActorForwardVector` _ownerbasecharacter) 80.0)))
  (if (`self.Bool`)
    (bind _outhit (`KismetSystemLibrary.SphereTraceSingleForObjects` _returnvalue (+ _returnvalue (* (`Actor.GetActorForwardVector` _ownerbasecharacter) 30.0)) 40.0 (`|MakeArray` "ObjectTypeQuery3" :!type "EObjectTypeQuery Enum")))
    (`/Engine/EditorBlueprintResources/StandardMacros.IsValid` (`.HitActor` (`GameplayStatics.BreakHitResult` _outhit))
      (:`Is Valid`
        (bind _asbase_character_class (cast `/Game/Blueprints/BaseCharacterClass` (`.HitActor` (`GameplayStatics.BreakHitResult` _outhit)))
          (:`then`
            (set `self.TargetCharater` _asbase_character_class)
            (bind _asweapon_base (cast `/Game/Blueprints/Weapons/Weapons/WeaponBase` (`ChildActorComponent.ChildActor` (`/Game/Blueprints/BaseCharacterClass.PickableItem` (`self.OwnerBaseCharacter`)))))
            (bind _asweapon_base_2 (cast `/Game/Blueprints/Weapons/Weapons/WeaponBase` (`ChildActorComponent.ChildActor` (`/Game/Blueprints/BaseCharacterClass.PickableItem` (`self.TargetCharater`)))))
            (if (>= (`KismetMathLibrary.Conv_ByteToInt` (`/Game/Blueprints/Weapons/Weapons/WeaponBase.WeaponToughnessEnum` _asweapon_base)) (`KismetMathLibrary.Conv_ByteToInt` (`/Game/Blueprints/Weapons/Weapons/WeaponBase.WeaponToughnessEnum` _asweapon_base_2)))
              (set `self.Bool` true)
              (set `self.TargetWeapon` _asweapon_base_2)
              (else
                (set `self.Bool` false)))
            (`/Engine/EditorBlueprintResources/StandardMacros.DoOnce` false :!label _label
              (:`Completed`
                (`/Game/Blueprints/Weapons/Weapons/WeaponBase.EventBlock` _asweapon_base)
                (if (`Actor.ActorHasTag` (`self.OwnerBaseCharacter`) "player")
                  (set `/Game/Blueprints/Weapons/Weapons/WeaponBase.Blocked` true (`self.TargetWeapon`))))))
          (:`CastFailed`
            (set `self.TargetCharater` null :!label _label_2)
            (set `self.Bool` false)
            (set `self.TargetWeapon` null)
            (`/Engine/EditorBlueprintResources/StandardMacros.DoOnce` false :!label _label_3
              (:`Completed`
                (bind _asweapon_base_3 (cast `/Game/Blueprints/Weapons/Weapons/WeaponBase` (`ChildActorComponent.ChildActor` (`/Game/Blueprints/BaseCharacterClass.PickableItem` (`self.OwnerBaseCharacter`)))))
                (`/Game/Blueprints/Weapons/Weapons/WeaponBase.EventBlock` _asweapon_base_3))))))
      (:`Is Not Valid`
        (goto _label_2)))
    (else
      (`|ExecutionSequence`
        (:`then_0`
          (goto _label_3 :!via `Reset`))
        (:`then_1`
          (goto _label :!via `Reset`))))))