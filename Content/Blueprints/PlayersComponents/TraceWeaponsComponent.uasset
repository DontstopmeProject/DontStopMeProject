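; Weapon detection component for player and NPC characters that finds the pickable weapon in front of the owner.
; When Trace is on, TraceWeapons box-traces along control rotation, rejecting weapons that are character-held, destroyed, flagged MustHit or blocked by CanFinish.
; NPCs store the result directly in PickableItemVar.
; Players go through ToggleOutlineForPlayer, which applies the OnlyChosenWeapnsGM filter when active and moves the custom-depth outline to the new pickup.
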(event `self.ReceiveBeginPlay`
  (bind _asbase_character_class (cast `/Game/Blueprints/BaseCharacterClass` (`self.GetOwner`)))
  (set `self.OwnerCharacter` _asbase_character_class)
  (bind _asplayers_character (cast `/Game/Blueprints/PlayersCharacter` (`self.GetOwner`))
    (:`then`
      (set `self.OwnerPlayerCharacter` _asplayers_character))
    (:`CastFailed`
      (bind _asbase_npc (cast `/Game/Blueprints/Ai/BaseNPC` (`self.GetOwner`)))
      (set `self.BaseNpc` _asbase_npc))))

(event `TraceWeapons`
  (bind _ownercharacter (`self.OwnerCharacter`))
  (bind _ownercharacter_2 (`self.OwnerCharacter`))
  (bind _ownercharacter_3 (`self.OwnerCharacter`))
  (bind _asweapon_base (cast `/Game/Blueprints/Weapons/Weapons/WeaponBase` (`self.TracedWeapon`) :!pure true))
  (bind _mesh (`Character.Mesh` (`self.OwnerCharacter`)))
  (bind _returnvalue (+ (+ (`SceneComponent.K2_GetComponentLocation` _mesh) (0.0 0.0 90.0)) (* (`SceneComponent.GetRightVector` _mesh) 20.0)))
  (`/Engine/EditorBlueprintResources/StandardMacros.IsValid` _ownercharacter
    (:`Is Valid`
      (if (`/Game/Blueprints/BaseCharacterClass.Trace` _ownercharacter)
        (`/Engine/EditorBlueprintResources/StandardMacros.IsValid` (`self.OwnerPlayerCharacter`)
          (:`Is Valid`
            (set `self.WeaponTraceSize` (45.0 70.0 100.0)))
          (:`Is Not Valid`
            (set `self.WeaponTraceSize` (100.0 100.0 100.0))))
        (bind _outhit (`KismetSystemLibrary.BoxTraceSingleForObjects` _returnvalue (+ _returnvalue (* (`KismetMathLibrary.GetForwardVector` (`Pawn.GetControlRotation` _ownercharacter_2)) 70.0)) (`self.WeaponTraceSize`) (`SceneComponent.K2_GetComponentRotation` (`Character.Mesh` _ownercharacter_2)) (`|MakeArray` "ObjectTypeQuery10" "ObjectTypeQuery4" :!type "EObjectTypeQuery Enum") false (`|MakeArray` (`ChildActorComponent.ChildActor` (`/Game/Blueprints/BaseCharacterClass.PickableItem` _ownercharacter_3)) (`ChildActorComponent.ChildActor` (`/Game/Blueprints/BaseCharacterClass.PickableItemL` _ownercharacter_3)) (`ChildActorComponent.ChildActor` (`/Game/Blueprints/BaseCharacterClass.FootActorL` _ownercharacter_3)) (`ChildActorComponent.ChildActor` (`/Game/Blueprints/BaseCharacterClass.FootActorR` _ownercharacter_3))) "None" false))
        (`/Engine/EditorBlueprintResources/StandardMacros.IsValid` (`.HitActor` (`GameplayStatics.BreakHitResult` _outhit))
          (:`Is Valid`
            (cast `/Game/Blueprints/Weapons/Weapons/WeaponBase` (`.HitActor` (`GameplayStatics.BreakHitResult` _outhit))
              (:`then`
                (cast `/Game/Blueprints/BaseCharacterClass` (`Actor.GetParentActor` (`.HitActor` (`GameplayStatics.BreakHitResult` _outhit)))
                  (:`then`
                    (set `self.TracedWeapon` null :!label _label)
                    (`/Engine/EditorBlueprintResources/StandardMacros.IsValid` (`self.OwnerPlayerCharacter`)
                      (:`Is Valid`
                        (`self.ToggleOutlineForPlayer`))
                      (:`Is Not Valid`
                        (set `/Game/Blueprints/BaseCharacterClass.PickableItemVar` null (`self.OwnerCharacter`)))))
                  (:`CastFailed`
                    (set `self.TracedWeapon` (`.HitActor` (`GameplayStatics.BreakHitResult` _outhit)))
                    (if (or (not (`/Game/Blueprints/Weapons/Weapons/WeaponBase.Destroy` _asweapon_base)) (not (<= (`/Game/Blueprints/Weapons/Weapons/WeaponBase.WeaponHealth` _asweapon_base) 0.0)))
                      (if (`/Game/Blueprints/Weapons/Weapons/WeaponBase.MustHit` _asweapon_base)
                        (goto _label)
                        (elif (!= (`/Game/Blueprints/BaseCharacterClass.PickableItemVar` (`self.OwnerCharacter`)) (`self.TracedWeapon`))
                          (if (`/Game/Blueprints/BaseCharacterClass.CanFinish` (`self.OwnerCharacter`))
                            (goto _label)
                            (else
                              (`/Engine/EditorBlueprintResources/StandardMacros.IsValid` (`self.OwnerPlayerCharacter`)
                                (:`Is Valid`
                                  (`self.ToggleOutlineForPlayer`))
                                (:`Is Not Valid`
                                  (set `/Game/Blueprints/BaseCharacterClass.PickableItemVar` (`self.TracedWeapon`) (`self.OwnerCharacter`))
                                  (set `self.TracedWeapon` null)))))))
                      (else
                        (goto _label))))))
              (:`CastFailed`
                (set `self.TracedWeapon` null :!label _label_2)
                (`/Engine/EditorBlueprintResources/StandardMacros.IsValid` (`self.OwnerPlayerCharacter`)
                  (:`Is Valid`
                    (`self.ToggleOutlineForPlayer`))
                  (:`Is Not Valid`
                    (set `/Game/Blueprints/BaseCharacterClass.PickableItemVar` null (`self.OwnerCharacter`)))))))
          (:`Is Not Valid`
            (goto _label_2)))))))

(fn `ToggleOutlineForPlayer`
  (bind _tracedweapon (`self.TracedWeapon`))
  (bind _pickableitemvar (`/Game/Blueprints/BaseCharacterClass.PickableItemVar` (`self.OwnerCharacter`)))
  (bind _asweapon_base (cast `/Game/Blueprints/Weapons/Weapons/WeaponBase` _pickableitemvar :!pure true))
  (bind _asonly_chosen_weapns_gm (cast `/Game/Blueprints/OnlyCHosenWeapnsGM` (`GameplayStatics.GetGameMode`))
    (:`then`
      (if (`/Game/Blueprints/OnlyCHosenWeapnsGM.CheckPickableWeapon` _asonly_chosen_weapns_gm (`self.TracedWeapon`) (`self.OwnerCharacter`))
        (`/Engine/EditorBlueprintResources/StandardMacros.IsValid` _pickableitemvar :!label _label
          (:`Is Valid`
            (`/Game/Blueprints/Weapons/Weapons/WeaponBase.EventSetRenderCustomDepth` _asweapon_base _pickableitemvar false)
            (set `/Game/Blueprints/BaseCharacterClass.PickableItemVar` (`self.TracedWeapon`) (`self.OwnerCharacter`) :!label _label_2)
            (`/Game/Blueprints/Weapons/Weapons/WeaponBase.EventSetRenderCustomDepth` (cast `/Game/Blueprints/Weapons/Weapons/WeaponBase` _tracedweapon :!pure true) _tracedweapon true)
            (set `self.TracedWeapon` null))
          (:`Is Not Valid`
            (`/Engine/EditorBlueprintResources/StandardMacros.IsValid` (`self.TracedWeapon`)
              (:`Is Valid`
                (goto _label_2))
              (:`Is Not Valid`
                (set `self.TracedWeapon` null)))))
        (else
          (`/Engine/EditorBlueprintResources/StandardMacros.IsValid` _pickableitemvar
            (:`Is Valid`
              (`/Game/Blueprints/Weapons/Weapons/WeaponBase.EventSetRenderCustomDepth` _asweapon_base _pickableitemvar false)
              (set `/Game/Blueprints/BaseCharacterClass.PickableItemVar` null (`self.OwnerCharacter`))
              (set `self.TracedWeapon` null))
            (:`Is Not Valid`
              (set `self.TracedWeapon` null))))))
    (:`CastFailed`
      (goto _label))))