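; Player component that plays an aberration pulse on the player camera's post-process settings when ChangeAberLevel is set.
; Tick waits on an accumulated-time check, then raises the value in fixed per-frame steps.
; At the threshold, a short delay and DoOnce zero the value and clear the flag.
; The timer is never reset here, so once WaitTime has elapsed it stops gating the ramp.
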(event `self.ReceiveBeginPlay`
  (bind _asplayers_character (cast `/Game/Blueprints/PlayersCharacter` (`GameplayStatics.GetPlayerCharacter` 0)))
  (set `self.Player` _asplayers_character))

(event `self.ReceiveTick`
  (params (DeltaSeconds :type "Float (single-precision)"))
  (if (`self.ChangeAberLevel`)
    (bind _ready (`self.Timer`))
    (if _ready
      (set `self.Value` (+ (`self.Value`) 0.2))
      (set `CameraComponent.PostProcessSettings` (make `PostProcessSettings` :`SceneFringeIntensity` (`self.Value`)) (`/Game/Blueprints/PlayersCharacter.Camera` (`self.Player`)))
      (if (>= (`self.Value`) 3.0)
        (`KismetSystemLibrary.Delay` 0.001)
        (`/Engine/EditorBlueprintResources/StandardMacros.DoOnce` false :!label _label
          (:`Completed`
            (set `self.ChangeAberLevel` false)
            (set `self.Value` 0.0)
            (set `CameraComponent.PostProcessSettings` (make `PostProcessSettings` :`SceneFringeIntensity` (`self.Value`)) (`/Game/Blueprints/PlayersCharacter.Camera` (`self.Player`)))))
        (else
          (goto _label :!via `Reset`))))))

(fn `Timer`
  (returns (Ready :type Boolean))
  (bind _output_get (set `self.TimerVar` (+ (`GameplayStatics.GetWorldDeltaSeconds`) (`self.TimerVar`))))
  (return (>= _output_get (`self.WaitTime`))))