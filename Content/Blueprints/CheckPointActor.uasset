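; Checkpoint trigger actor that saves level progress and the player's weapon, with a box sized in the construction script.
; On player overlap, if Increment is set and ActorIndex differs from LevelsIndex, it increments that index, resets GameMode kills and stores weapon class, ammo and health in the GameInstance.
; It then respawns the weapon from that data and briefly shows the HUD save icon.
; An unused SaveWeapon macro writes to the GameMode instead.
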(event `self.ReceiveBeginPlay`
  (bind _asdsm_game_instance (cast `/Game/Blueprints/Dsm_GameInstance` (`GameplayStatics.GetGameInstance`)))
  (set `self.GI` _asdsm_game_instance))

(event `self.Box.OnComponentBeginOverlap`
  (params (OverlappedComponent :type "PrimitiveComponent Object Reference") (OtherActor :type "Actor Object Reference") (OtherComp :type "PrimitiveComponent Object Reference") (OtherBodyIndex :type Integer) (bFromSweep :type Boolean) (SweepResult :type "HitResult Structure (by ref)"))
  (bind _asplayers_character (cast `/Game/Blueprints/PlayersCharacter` OtherActor))
  (bind _asdsm_game_instance (cast `/Game/Blueprints/Dsm_GameInstance` (`GameplayStatics.GetGameInstance`)))
  (if (`self.Increment`)
    (bind _levelsindex (`/Game/Blueprints/Dsm_GameInstance.LevelsIndex` _asdsm_game_instance))
    (if (!= (`self.ActorIndex`) _levelsindex)
      (`/Engine/EditorBlueprintResources/StandardMacros.IncrementInt` _levelsindex
        (:`  `
          (bind _asdsm_gamemode (cast `/Game/Blueprints/DsmGamemode` (`GameplayStatics.GetGameMode`)))
          (set `/Game/Blueprints/DsmGamemode.kills` 0 _asdsm_gamemode)
          (bind _equipedweapon (`/Game/Blueprints/BaseCharacterClass.EquipedWeapon` _asplayers_character))
          (bind _asweapon_base (cast `/Game/Blueprints/Weapons/Weapons/WeaponBase` _equipedweapon))
          (bind _asdsm_game_instance_2 (cast `/Game/Blueprints/Dsm_GameInstance` (`GameplayStatics.GetGameInstance`))
            (:`then`
              (bind _returnvalue (`GameplayStatics.GetObjectClass` _equipedweapon))
              (if (`KismetSystemLibrary.IsValidClass` _returnvalue)
                (set `/Game/Blueprints/Dsm_GameInstance.CurrentWeapon` (make `/Game/Blueprints/Weapons/Weapons/CurrentWeaponStruct` _returnvalue (`/Game/Blueprints/Weapons/Weapons/WeaponBase.AmmoCounter` _asweapon_base) (`/Game/Blueprints/Weapons/Weapons/WeaponBase.WeaponHealth` _asweapon_base)) _asdsm_game_instance_2)
                (bind _asdsm_game_instance_3 (cast `/Game/Blueprints/Dsm_GameInstance` (`GameplayStatics.GetGameInstance`)))
                (bind _asplayers_character_2 (cast `/Game/Blueprints/PlayersCharacter` (`GameplayStatics.GetPlayerCharacter` 0)))
                (`/Game/Blueprints/BaseCharacterClass.EventThrowAway` _asplayers_character_2 false false)
                (`self.K2_DestroyActor` (`/Game/Blueprints/BaseCharacterClass.ThrowedWeapon` _asplayers_character_2))
                (bind (_currentweapon_currentweapon _currentweapon_ammo _currentweapon_health) (break `/Game/Blueprints/Weapons/Weapons/CurrentWeaponStruct` (`/Game/Blueprints/Dsm_GameInstance.CurrentWeapon` _asdsm_game_instance_3)))
                (`/Game/Blueprints/BaseCharacterClass.EventPickUp` _asplayers_character_2 _currentweapon_currentweapon null false)
                (bind _hudwidget (`/Game/Blueprints/PlayersCharacter.HudWidget` _asplayers_character_2))
                (set `/Game/Blueprints/Widgets/BaseWidgets/W_HudWidget.SaveIconVis` "Visible" _hudwidget)
                (set `/Game/Blueprints/PlayersCharacter.HudHidden` true _asplayers_character_2)
                (set `/Game/Blueprints/PlayersCharacter.ShowAmmo` false _asplayers_character_2) ; Если да, то переменная устанавливается в false, чтобы не было повторного вызова
                (`Widget.SetVisibility` _hudwidget "Visible")
                (bind _asweapon_base_2 (cast `/Game/Blueprints/Weapons/Weapons/WeaponBase` (`/Game/Blueprints/BaseCharacterClass.EquipedWeapon` _asplayers_character_2)))
                (set `/Game/Blueprints/Weapons/Weapons/WeaponBase.AmmoCounter` _currentweapon_ammo _asweapon_base_2)
                (set `/Game/Blueprints/Weapons/Weapons/WeaponBase.WeaponHealth` _currentweapon_health _asweapon_base_2)
                (`KismetSystemLibrary.Delay` 2.0)
                (set `/Game/Blueprints/Widgets/BaseWidgets/W_HudWidget.SaveIconVis` "Hidden" _hudwidget)
                (`Widget.SetVisibility` _hudwidget "Hidden")
                (set `/Game/Blueprints/PlayersCharacter.ShowAmmo` true _asplayers_character_2) ; Если да, то переменная устанавливается в false, чтобы не было повторного вызова
                (else
                  (`KismetSystemLibrary.PrintString` "Not valid Gamemode" true true (struct :`R` 1.0 :`B` 0.00845 :`A` 1.0) :!label _label))))
            (:`CastFailed`
              (goto _label))))))))

(fn `SaveWaeponFunc`)

(fn `UserConstructionScript`
  (`BoxComponent.SetBoxExtent` (`self.Box`) (`self.BoxExtent`) true))