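; Game mode, judging by its name, for restricting which weapons the player can pick up.
; CheckPickableWeapon rejects non-weapons and any weapon whose exact class is in the Weapons array, so despite the "only chosen" name the list reads as a blocklist.
; An empty list allows every weapon, and non-player characters always pass.
; BeginPlay caches the first player's character, though the check uses its own Player input.
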(event `self.ReceiveBeginPlay`
  (`parent.ReceiveBeginPlay`)
  (bind _asplayers_character (cast `/Game/Blueprints/PlayersCharacter` (`GameplayStatics.GetPlayerCharacter` 0)))
  (set `self.Player` _asplayers_character))

(fn `CheckPickableWeapon`
  (params (Weapon :type "Actor Object Reference") (Player :type "Actor Object Reference"))
  (returns (CanPick :type Boolean))
  (cast `/Game/Blueprints/PlayersCharacter` Player
    (:`then`
      (bind _asweapon_base (cast `/Game/Blueprints/Weapons/Weapons/WeaponBase` Weapon)
        (:`then`
          (if (> (`KismetArrayLibrary.Array_Length` (`self.Weapons`)) 0)
            (for _array_element (`self.Weapons`)
              (if (== _array_element (`GameplayStatics.GetObjectClass` _asweapon_base))
                (`|ExecutionSequence`
                  (:`then_0`
                    (break))
                  (:`then_1`
                    (return false)))))
            (return true)
            (else
              (return true))))
        (:`CastFailed`
          (return false))))
    (:`CastFailed`
      (return true))))

(fn `UserConstructionScript`
  (`parent.UserConstructionScript`))