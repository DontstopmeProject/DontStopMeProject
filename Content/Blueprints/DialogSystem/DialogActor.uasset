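; DialogActor is a trigger box that plays a timed dialog sequence among characters, started by an overlap or by characters already inside at BeginPlay.
; SayText walks DialogStrings, showing each line on its speaker's DialogText for that entry's delay, then calls itself for the next.
; The sequence ends, calling CallDialogFinished and setting Finished, after the last line or when the next speaker is dead, punched or stunned.
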(event `self.ReceiveBeginPlay`
  (for _array_element (`PrimitiveComponent.GetOverlappingActors` (`self.Box`) "/Script/Engine.Character")
    (cast `/Game/Blueprints/BaseCharacterClass` _array_element)
    (`self.SayText`)))

(event `SayText`
  (bind (_text _textmember _delay) (break `/Game/Blueprints/DialogSystem/DialogStructure` (`|GetArrayItem` (`self.DialogStrings`) (`self.CurrentText`))))
  (bind _dialogtext (`/Game/Blueprints/BaseCharacterClass.DialogText` _textmember))
  (if (not (`self.Finished`))
    (`TextRenderComponent.K2_SetText` _dialogtext _text)
    (`SceneComponent.SetVisibility` _dialogtext true false)
    (`KismetSystemLibrary.Delay` _delay)
    (`SceneComponent.SetVisibility` _dialogtext false false)
    (bind _output_get (set `self.CurrentText` (+ (`self.CurrentText`) 1)))
    (if (== _output_get (`KismetArrayLibrary.Array_Length` (`self.DialogStrings`)))
      (`self.DialogFinished` :!label _label)
      (set `self.Finished` true)
      (elif (or (`/Game/Blueprints/BaseCharacterClass.Dead` _textmember) (`/Game/Blueprints/BaseCharacterClass.PunchedVar` _textmember) (`/Game/Blueprints/BaseCharacterClass.Stuned` _textmember))
        (goto _label)
        (else
          (`self.SayText`))))))

(event `self.Box.OnComponentBeginOverlap`
  (params (OverlappedComponent :type "PrimitiveComponent Object Reference") (OtherActor :type "Actor Object Reference") (OtherComp :type "PrimitiveComponent Object Reference") (OtherBodyIndex :type Integer) (bFromSweep :type Boolean) (SweepResult :type "HitResult Structure (by ref)"))
  (set `self.Actor` OtherActor)
  (if (not (`self.Retriggereble`))
    (`/Engine/EditorBlueprintResources/StandardMacros.DoOnce` false
      (:`Completed`
        _)))
  (set `self.CurrentText` 0)
  (`self.SayText`))

(fn `UserConstructionScript`)