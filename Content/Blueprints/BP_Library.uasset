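; Blueprint function library of gameplay helpers for AI, cutscenes, menus and level progression.
; AI helpers spawn armed, grouped Mafia NPCs and toggle movement and sensing, while CleanScene destroys destructibles, projectiles, weapons and non-player humans.
; CS uses paired DoOnce gates to lock and restore the player around a Level Sequence.
; Menu functions provide keyboard, gamepad and hover button highlighting; level helpers use the GameInstance's level index for streaming checks and checkpoint teleports.
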(fn `CheckLevelStreamingValidation`
  (returns (ReturnValue :type Boolean))
  (bind _asdsm_game_instance (cast `/Game/Blueprints/Dsm_GameInstance` (`GameplayStatics.GetGameInstance` null)))
  (bind _returnvalue (`GameplayStatics.GetStreamingLevel` null (`|GetArrayItem` (`/Game/Blueprints/Dsm_GameInstance.LevelsArray` _asdsm_game_instance) (`/Game/Blueprints/Dsm_GameInstance.LevelsIndex` _asdsm_game_instance))))
  (if (`KismetSystemLibrary.IsValid` _returnvalue)
    (return (`LevelStreaming.IsLevelLoaded` _returnvalue))
    (else
      (return false))))

(fn `CleanScene`
  (bind _outactors (`GameplayStatics.GetAllActorsOfClass` null "/Script/Engine.DestructibleActor"))
  (for _array_element _outactors
    (`Actor.K2_DestroyActor` _array_element))
  (bind _outactors_2 (`GameplayStatics.GetAllActorsWithTag` null "projectile"))
  (for _array_element_2 _outactors_2
    (`Actor.K2_DestroyActor` _array_element_2))
  (bind _outactors_3 (`GameplayStatics.GetAllActorsWithTag` null "weapons"))
  (for _array_element_3 _outactors_3
    (`Actor.K2_DestroyActor` _array_element_3))
  (bind _outactors_4 (`GameplayStatics.GetAllActorsWithTag` null "human"))
  (for _array_element_4 _outactors_4
    (if (not (`Actor.ActorHasTag` _array_element_4 "player"))
      (`Actor.K2_DestroyActor` _array_element_4))))

(fn `CS`
  (params (`Level Sequence` :type "MovieSceneSequencePlayer Object Reference") (PlayerCharacter :type "Object Object Reference") (PlayerController :type "PlayerController Object Reference"))
  (if (`KismetSystemLibrary.IsValid` `Level Sequence`)
    (`|ExecutionSequence`
      (:`then_0`
        (if (`MovieSceneSequencePlayer.IsPlaying` `Level Sequence`)
          (`/Engine/EditorBlueprintResources/StandardMacros.DoOnce` false :!label _label
            (:`Completed`
              (bind _asplayers_character (cast `/Game/Blueprints/PlayersCharacter` (`GameplayStatics.GetPlayerCharacter` null)))
              (`ActorComponent.Deactivate` (`Character.CharacterMovement` _asplayers_character))
              (`/Game/Blueprints/PlayersCharacter.Cutscene` _asplayers_character true)
              (set `/Game/Blueprints/PlayersCharacter.ChangeTimeDilationInPlayersClass` false _asplayers_character)
              (`GameplayStatics.SetGlobalTimeDilation` null 1.0)
              (`/Game/Blueprints/PlayersCharacter.EventToggleInput` _asplayers_character true)
              (set `/Game/Blueprints/BaseCharacterClass.StopChangingCustomTime` true _asplayers_character)
              (set `Actor.CustomTimeDilation` 1.0 _asplayers_character)
              (goto _label_2 :!via `Reset`)))
          (else
            (`/Engine/EditorBlueprintResources/StandardMacros.DoOnce` false :!label _label_2
              (:`Completed`
                (bind _asplayers_character_2 (cast `/Game/Blueprints/PlayersCharacter` (`GameplayStatics.GetPlayerCharacter` null)))
                (`ActorComponent.Activate` (`Character.CharacterMovement` _asplayers_character_2) false)
                (`/Game/Blueprints/PlayersCharacter.Cutscene` _asplayers_character_2 false)
                (set `/Game/Blueprints/BaseCharacterClass.StopChangingCustomTime` false _asplayers_character_2)
                (`/Game/Blueprints/PlayersCharacter.EventToggleInput` _asplayers_character_2 false)
                (set `/Game/Blueprints/PlayersCharacter.ChangeTimeDilationInPlayersClass` true _asplayers_character_2)
                (goto _label :!via `Reset`))))))
      (:`then_1`
        (`KismetSystemLibrary.PrintString` null)
        (return)))))

(fn `OnButtonHoveredFunc`
  (params (Button :type "Button Object Reference") (ButtonsArray :type "Array of Button Object Reference") (index :type Integer) (PlayerController :type "PlayerController Object Reference"))
  (`Widget.SetUserFocus` Button PlayerController)
  (`Button.SetBackgroundColor` Button (struct :`G` 0.116382 :`B` 1.0 :`A` 1.0))
  (for (_array_element _array_index) ButtonsArray
    (if (!= _array_index index)
      (`Button.SetBackgroundColor` _array_element (struct :`R` 1.0 :`G` 1.0 :`B` 1.0 :`A` 1.0))))
  (return))

(fn `OnKeyDownFunc`
  (params (Input :type "KeyEvent Structure (by ref)") (`Button Index` :type "Integer (by ref)") (ButtonsArray :type "Array of Button Object Reference (by ref)") (TargetWidget :type "Widget Object Reference") (`Left/Right` :type Boolean))
  (returns (`PressedButton?` :type Boolean) (ButtonIndexReturn :type Integer))
  (locals (ButtonsArrayLocal :type "Array of Button Object Reference") (PressedKey :type "Key Structure") (ButtonIndex :type Integer) (FirstDisiredKeys :type "Array of Key Structure") (SecondDisiredKeys :type "Array of Key Structure") (TargetWidgetLocal :type "Widget Object Reference"))
  (bind _firstdisiredkeys (`local.FirstDisiredKeys`))
  (bind _seconddisiredkeys (`local.SecondDisiredKeys`))
  (bind _firstdisiredkeys_2 (`local.FirstDisiredKeys`))
  (bind _seconddisiredkeys_2 (`local.SecondDisiredKeys`))
  (bind _pressedkey (`local.PressedKey`))
  (set `local.TargetWidgetLocal` TargetWidget)
  (set `local.ButtonsArrayLocal` ButtonsArray)
  (set `local.PressedKey` (`KismetInputLibrary.GetKey` Input))
  (set `local.ButtonIndex` `Button Index`)
  (if `Left/Right`
    ;[1 1 1] Setting disired keys
    (`KismetArrayLibrary.Array_Add` _firstdisiredkeys "Left")
    (`KismetArrayLibrary.Array_Add` _firstdisiredkeys "A")
    (`KismetArrayLibrary.Array_Add` _firstdisiredkeys "Gamepad_DPad_Left")
    (`KismetArrayLibrary.Array_Add` _firstdisiredkeys "Gamepad_LeftStick_Left")
    (`KismetArrayLibrary.Array_Add` _seconddisiredkeys "Right")
    (`KismetArrayLibrary.Array_Add` _seconddisiredkeys "D")
    (`KismetArrayLibrary.Array_Add` _seconddisiredkeys "Gamepad_DPad_Right")
    (`KismetArrayLibrary.Array_Add` _seconddisiredkeys "Gamepad_LeftStick_Right")
    (else
      ;[1 1 1] Setting second disired keys
      (`KismetArrayLibrary.Array_Add` _firstdisiredkeys_2 "Up")
      (`KismetArrayLibrary.Array_Add` _firstdisiredkeys_2 "W")
      (`KismetArrayLibrary.Array_Add` _firstdisiredkeys_2 "Gamepad_DPad_Up")
      (`KismetArrayLibrary.Array_Add` _firstdisiredkeys_2 "Gamepad_LeftStick_Up")
      (`KismetArrayLibrary.Array_Add` _seconddisiredkeys_2 "Down")
      (`KismetArrayLibrary.Array_Add` _seconddisiredkeys_2 "S")
      (`KismetArrayLibrary.Array_Add` _seconddisiredkeys_2 "Gamepad_DPad_Down")
      (`KismetArrayLibrary.Array_Add` _seconddisiredkeys_2 "Gamepad_LeftStick_Down")))
  (for _array_element (`local.FirstDisiredKeys`)
    (if (== _array_element (`local.PressedKey`))
      (`|ExecutionSequence`
        (:`then_0`
          (break))
        (:`then_1`
          (bind _buttonindex (`self.SwitchUmgButtons` true (`local.ButtonIndex`) (`local.ButtonsArrayLocal`) (`local.TargetWidgetLocal`)))
          (set `local.ButtonIndex` _buttonindex)
          (set `PlayerController.bShowMouseCursor` false (`GameplayStatics.GetPlayerController` null) :!label _label)
          (return (or (== _pressedkey "Enter") (== _pressedkey "SpaceBar") (== _pressedkey "Gamepad_FaceButton_Bottom")) (`local.ButtonIndex`))))))
  (for _array_element_2 (`local.SecondDisiredKeys`)
    (if (== _array_element_2 (`local.PressedKey`))
      (`|ExecutionSequence`
        (:`then_0`
          (break))
        (:`then_1`
          (bind _buttonindex_2 (`self.SwitchUmgButtons` false (`local.ButtonIndex`) (`local.ButtonsArrayLocal`) (`local.TargetWidgetLocal`)))
          (set `local.ButtonIndex` _buttonindex_2)
          (goto _label)))))
  (goto _label))

(fn `SpawnAiOkay`
  (params (PawnClass :type "Pawn Class Reference") (AIControllerClass :type "Controller Class Reference") (BehaviorTree :type "BehaviorTree Object Reference") (Location :type "Vector Structure") (Rotation :type "Rotator Structure") (bNoCollisionFail :type Boolean) (WeaponActor :type "Actor Class Reference") (GroupIndex :type Integer))
  (returns (Array :type "Array of /Game/Blueprints/Ai/Enemies/Mafia_NPC Object Reference"))
  (bind _returnvalue (`AIBlueprintHelperLibrary.SpawnAIFromClass` null PawnClass BehaviorTree Location Rotation bNoCollisionFail))
  (set `Pawn.AIControllerClass` AIControllerClass _returnvalue)
  (bind _asmafia_npc (cast `/Game/Blueprints/Ai/Enemies/Mafia_NPC` _returnvalue))
  (`/Game/Blueprints/BaseCharacterClass.EventPickUp` _asmafia_npc WeaponActor)
  (set `/Game/Blueprints/Ai/BaseNPC.GroupIndex` GroupIndex _asmafia_npc)
  (return (`|MakeArray` _asmafia_npc)))

(fn `SpawnPlayerAtTheCheckpoint`
  (params (CheckPointsArray :type "Array of Actor Object Reference"))
  (bind _asdsm_game_instance (cast `/Game/Blueprints/Dsm_GameInstance` (`GameplayStatics.GetGameInstance` null)))
  (bind _output (`|GetArrayItem` CheckPointsArray (`/Game/Blueprints/Dsm_GameInstance.LevelsIndex` _asdsm_game_instance)))
  (`Actor.K2_SetActorLocationAndRotation` (`GameplayStatics.GetPlayerCharacter` null) (`Actor.K2_GetActorLocation` _output) (`Actor.K2_GetActorRotation` _output) false true)
  (return))

(fn `SwitchUmgButtons`
  (params (Up :type Boolean) (`Button Index` :type "Integer (by ref)") (ButtonsArray :type "Array of Button Object Reference (by ref)") (Target :type "Widget Object Reference"))
  (returns (ButtonIndex :type "Integer (by ref)"))
  (locals (ButtonIndexLocal :type Integer) (ButtonsArrayLocal :type "Array of Button Object Reference"))
  (bind _buttonindexlocal (`local.ButtonIndexLocal`))
  (bind _buttonsarraylocal (`local.ButtonsArrayLocal`))
  (bind _buttonsarraylocal_2 (`local.ButtonsArrayLocal`))
  (bind _output (`|GetArrayItem` (`local.ButtonsArrayLocal`) (`local.ButtonIndexLocal`)))
  (set `local.ButtonIndexLocal` `Button Index`)
  (set `local.ButtonsArrayLocal` ButtonsArray)
  (if Up
    (bind _result (`/Engine/EditorBlueprintResources/StandardMacros.DecrementInt` _buttonindexlocal)
      (:`  `
        (if (< _result 0)
          (set `local.ButtonIndexLocal` (`KismetArrayLibrary.Array_LastIndex` _buttonsarraylocal))
          (`Button.SetBackgroundColor` (`|GetArrayItem` _buttonsarraylocal) (struct :`R` 1.0 :`G` 1.0 :`B` 1.0 :`A` 1.0))
          (else
            (`Button.SetBackgroundColor` (`|GetArrayItem` (`local.ButtonsArrayLocal`) (+ (`local.ButtonIndexLocal`) 1)) (struct :`R` 1.0 :`G` 1.0 :`B` 1.0 :`A` 1.0))))))
    (else
      (bind _result_2 (`/Engine/EditorBlueprintResources/StandardMacros.IncrementInt` _buttonindexlocal)
        (:`  `
          (if (> _result_2 (`KismetArrayLibrary.Array_LastIndex` (`local.ButtonsArrayLocal`)))
            (`Button.SetBackgroundColor` (`|GetArrayItem` _buttonsarraylocal_2 (`KismetArrayLibrary.Array_LastIndex` _buttonsarraylocal_2)) (struct :`R` 1.0 :`G` 1.0 :`B` 1.0 :`A` 1.0))
            (set `local.ButtonIndexLocal` 0)
            (else
              (`Button.SetBackgroundColor` (`|GetArrayItem` (`local.ButtonsArrayLocal`) (- (`local.ButtonIndexLocal`) 1)) (struct :`R` 1.0 :`G` 1.0 :`B` 1.0 :`A` 1.0))))))))
  (`Widget.SetUserFocus` _output (`GameplayStatics.GetPlayerController` null))
  (`Button.SetBackgroundColor` _output (struct :`G` 0.116382 :`B` 1.0 :`A` 1.0))
  (`Widget.SetKeyboardFocus` Target)
  (return (`local.ButtonIndexLocal`)))

(fn `ToggleAiMovement`
  (params (AI :type "Actor Object Reference") (Disable :type Boolean))
  (bind _asbase_npc (cast `/Game/Blueprints/Ai/BaseNPC` AI)
    (:`then`
      (if Disable
        (`ActorComponent.Deactivate` (`Character.CharacterMovement` _asbase_npc))
        (`ActorComponent.Deactivate` (`/Game/Blueprints/Ai/BaseNPC.PawnSensing` _asbase_npc))
        (else
          (`ActorComponent.Activate` (`/Game/Blueprints/Ai/BaseNPC.PawnSensing` _asbase_npc) false)
          (`ActorComponent.Activate` (`Character.CharacterMovement` _asbase_npc) false))))
    (:`CastFailed`
      (`KismetSystemLibrary.PrintString` null "Failed To Cast to Base NPC in Toggle Ai Movement" true true (struct :`R` 1.0 :`B` 0.011505 :`A` 1.0) 5.0))))