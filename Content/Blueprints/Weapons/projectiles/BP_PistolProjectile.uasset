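; BP_PistolProjectile is a pistol projectile that colors its trail and light by who fired it.
; On BeginPlay, after the parent's logic, it checks a valid owner for the "player" tag.
; Player shots get a blue point light and their own trail material instance, while other owners' shots get red and another instance.
; Tick only calls the parent, and a damage falloff subtraction is left unconnected.
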(event `self.ReceiveBeginPlay`
  (bind _returnvalue (`self.GetOwner`))
  (bind _particlesystem (`self.ParticleSystem`))
  (bind _pointlight (`self.PointLight`))
  (`parent.ReceiveBeginPlay`)
  (`/Engine/EditorBlueprintResources/StandardMacros.IsValid` _returnvalue
    (:`Is Valid`
      (if (`self.ActorHasTag` _returnvalue "player")
        (`PrimitiveComponent.SetMaterial` _particlesystem 0 "/Game/Assets/Materials/M_SnipeTrail_Inst2.M_SnipeTrail_Inst2")
        (`LightComponent.SetLightColor` _pointlight (struct :`B` 1.0 :`A` 1.0) true)
        (else
          (`PrimitiveComponent.SetMaterial` _particlesystem 0 "/Game/Assets/Materials/M_SnipeTrail_Inst.M_SnipeTrail_Inst")
          (`LightComponent.SetLightColor` _pointlight (struct :`R` 1.0 :`A` 1.0) true))))))

(event `self.ReceiveTick`
  (params (DeltaSeconds :type "Float (single-precision)"))
  (`parent.ReceiveTick` DeltaSeconds))

(fn `UserConstructionScript`
  (`parent.UserConstructionScript`))