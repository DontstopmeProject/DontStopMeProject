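; Ricochet pistol projectile that bounces off surfaces, with trail material and light colored blue for a player owner and red otherwise.
; On each bounce, SurfaceDetectionMacro1 plays impact feedback and separates ordinary ricochets from stopping hits on humans, projectiles, weapons or StopBounce actors.
; Stopping hits remove the mesh, apply tag-dependent damage and destroy the projectile after a short delay.
; The damage falloff logic is unconnected, and physics impulses use zero direction vectors.
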(event `self.ReceiveBeginPlay`
  (bind _particlesystem (`self.ParticleSystem`))
  (bind _pointlight (`self.PointLight`))
  (`parent.ReceiveBeginPlay`)
  (if (`self.ActorHasTag` (`self.GetOwner`) "player")
    (`PrimitiveComponent.SetMaterial` _particlesystem 0 "/Game/Assets/Materials/M_SnipeTrail_Inst2.M_SnipeTrail_Inst2")
    (`LightComponent.SetLightColor` _pointlight (struct :`B` 1.0 :`A` 1.0) true)
    (else
      (`PrimitiveComponent.SetMaterial` _particlesystem 0 "/Game/Assets/Materials/M_SnipeTrail_Inst.M_SnipeTrail_Inst")
      (`LightComponent.SetLightColor` _pointlight (struct :`R` 1.0 :`A` 1.0) true))))

(event `self.ReceiveTick`
  (params (DeltaSeconds :type "Float (single-precision)"))
  (`parent.ReceiveTick` DeltaSeconds))

(event `self.ProjectileMovement.OnProjectileBounce`
  (params (ImpactResult :type "HitResult Structure (by ref)") (ImpactVelocity :type "Vector Structure (by ref)"))
  (bind _staticmesh (`self.StaticMesh`))
  (bind _hitcomponent (`self.HitComponent`))
  (bind _returnvalue (* (`KismetMathLibrary.Normal` (`KismetMathLibrary.GetDirectionUnitVector` (0.0 0.0 0.0))) (`self.DamageVelocity`)))
  (`/Engine/EditorBlueprintResources/StandardMacros.IsValid` ImpactResult_HitActor
    (:`Is Valid`
      (set `self.HitComponent` ImpactResult_HitComponent)
      (set `self.HitActor` ImpactResult_HitActor)
      (set `self.HitBoneName` ImpactResult_HitBoneName)
      (`self.SurfaceDetectionMacro1` (`self.HitActor`) ImpactResult_Location
        (:`then`
          (`/Engine/EditorBlueprintResources/StandardMacros.IsValid` _staticmesh
            (:`Is Valid`
              (set `self.WorldRotation` (`SceneComponent.K2_GetComponentRotation` _staticmesh))
              (`ActorComponent.K2_DestroyComponent` (`self.StaticMesh`)))
            (:`Is Not Valid`
              _))
          (if (`self.ActorHasTag` (`self.HitActor`) "human")
            (bind _asbase_character_class (cast `/Game/Blueprints/BaseCharacterClass` (`self.HitActor`))
              (:`then`
                (set `/Game/Blueprints/BaseCharacterClass.DeathEnumVar` (`self.DeathEnumVar`) _asbase_character_class)
                (if (not (`/Game/Blueprints/BaseCharacterClass.Chuck` _asbase_character_class))
                  (`GameplayStatics.ApplyDamage` (`self.HitActor`) 100.0 null self))
                (if (`SceneComponent.IsSimulatingPhysics` (`self.HitComponent`) (`self.HitBoneName`))
                  (`PrimitiveComponent.AddImpulse` (`Character.Mesh` _asbase_character_class) _returnvalue (`self.HitBoneName`) true)))
              (:`CastFailed`
                (`GameplayStatics.ApplyDamage` (`self.HitActor`) (`self.Damage`) null self :!label _label)))
            (elif (`self.ActorHasTag` (`self.HitActor`) "weapon")
              (`GameplayStatics.ApplyDamage` (`self.HitActor`) (`self.Damage`) null self)
              (`KismetSystemLibrary.Delay` 0.05)
              (`GameplayStatics.ApplyDamage` (`self.HitActor`) (`self.Damage`) null self)
              (else
                (`/Engine/EditorBlueprintResources/StandardMacros.IsValid` _hitcomponent
                  (:`Is Valid`
                    (if (`SceneComponent.IsSimulatingPhysics` _hitcomponent "None")
                      (`PrimitiveComponent.AddImpulseAtLocation` (`self.HitComponent`) _returnvalue (0.0 0.0 0.0) "None")
                      (goto _label)
                      (else
                        (goto _label))))
                  (:`Is Not Valid`
                    _)))))
          (`KismetSystemLibrary.Delay` 0.05)
          (`self.K2_DestroyActor`))))))

(fn `UserConstructionScript`
  (`parent.UserConstructionScript`))