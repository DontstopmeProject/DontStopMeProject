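; Base projectile for weapons that damages what it hits, pushes physics bodies and spawns impact effects.
; BeginPlay briefly delays sphere collision and can enable bullet blocking, which Tick switches back to Ignore after a short time.
; On stop, it branches on human and weapon tags for damage, impulse and blood or generic effects, then destroys itself.
; Tick adjusts its time dilation during global slow motion and syncs the hit particles to the player's dilation.
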(event `self.ReceiveBeginPlay`
  (bind _sphere (`self.Sphere`))
  (`KismetArrayLibrary.Array_Add` (`self.Tags`) (`|GetArrayItem` (`Actor.Tags` (`self.GetOwner`)) 2))
  (bind _asdsm_game_instance (cast `/Game/Blueprints/Dsm_GameInstance` (`GameplayStatics.GetGameInstance`)))
  (set `self.GameInstance` _asdsm_game_instance)
  (`PrimitiveComponent.SetCollisionEnabled` _sphere "NoCollision")
  (`KismetSystemLibrary.Delay` 0.04)
  (`PrimitiveComponent.SetCollisionEnabled` _sphere "QueryAndPhysics")
  (`KismetSystemLibrary.Delay` 0.04)
  (if (`self.BlockBullets`)
    (`PrimitiveComponent.SetCollisionResponseToChannel` (`self.Sphere`) "ECC_GameTraceChannel1" "ECR_Block")
    (`KismetSystemLibrary.Delay` 4.0)
    (`self.K2_DestroyActor`)))

(event `self.ReceiveTick`
  (params (DeltaSeconds :type "Float (single-precision)"))
  (bind _returnvalue (`GameplayStatics.GetGlobalTimeDilation`))
  (bind _sphere (`self.Sphere`))
  (bind _hit_ps (`self.Hit_PS`))
  (bind _output_get (set `self.Time` (+ DeltaSeconds (`self.Time`))))
  (`/Engine/EditorBlueprintResources/StandardMacros.IsValid` _hit_ps
    (:`Is Valid`
      (set `ParticleSystemComponent.CustomTimeDilation` (`Actor.CustomTimeDilation` (`GameplayStatics.GetPlayerCharacter` 0)) _hit_ps))
    (:`Is Not Valid`
      _))
  (if (>= _output_get 0.06)
    (`/Engine/EditorBlueprintResources/StandardMacros.IsValid` _sphere
      (:`Is Valid`
        (`PrimitiveComponent.SetCollisionResponseToChannel` _sphere "ECC_GameTraceChannel1" "ECR_Ignore"))
      (:`Is Not Valid`
        _)))
  (if (`self.SetCustomTimeManualy`)
    _
    (elif (<= _returnvalue 0.7)
      (`/Engine/EditorBlueprintResources/StandardMacros.DoOnce` false :!label _label
        (:`Completed`
          (set `self.CustomTimeDilation` (/ _returnvalue 15.0))
          (`|ExecutionSequence`
            (:`then_0`
              (goto _label_2 :!via `Reset`)))))
      (else
        (`/Engine/EditorBlueprintResources/StandardMacros.DoOnce` false :!label _label_2
          (:`Completed`
            (set `self.CustomTimeDilation` 1.0)
            (`|ExecutionSequence`
              (:`then_0`
                (goto _label :!via `Reset`)))))))))

(event `self.ProjectileMovement.OnProjectileStop`
  (params (ImpactResult :type "HitResult Structure (by ref)"))
  (bind _staticmesh (`self.StaticMesh`))
  (bind _hitcomponent (`self.HitComponent`))
  (bind _staticmesh_2 (`self.StaticMesh`))
  (bind _returnvalue (* (`KismetMathLibrary.Normal` (`KismetMathLibrary.GetDirectionUnitVector` ImpactResult_TraceStart ImpactResult_TraceEnd)) (`self.DamageVelocity`)))
  (`/Engine/EditorBlueprintResources/StandardMacros.IsValid` ImpactResult_HitActor
    (:`Is Valid`
      (set `self.HitComponent` ImpactResult_HitComponent)
      (set `self.HitBoneName` ImpactResult_HitBoneName)
      (`self.SurfaceDetectionMacro` ImpactResult_Location ImpactResult_HitActor)
      (`/Engine/EditorBlueprintResources/StandardMacros.IsValid` _staticmesh
        (:`Is Valid`
          (set `self.WorldRotation` (`SceneComponent.K2_GetComponentRotation` _staticmesh))
          (`ActorComponent.K2_DestroyComponent` (`self.StaticMesh`)))
        (:`Is Not Valid`
          _))
      (if (`self.ActorHasTag` ImpactResult_HitActor "human")
        (bind _asbase_character_class (cast `/Game/Blueprints/BaseCharacterClass` ImpactResult_HitActor)
          (:`then`
            (set `/Game/Blueprints/BaseCharacterClass.DeathEnumVar` (`self.DeathEnumVar`) _asbase_character_class)
            (if (not (`/Game/Blueprints/BaseCharacterClass.Chuck` _asbase_character_class))
              (`GameplayStatics.ApplyDamage` ImpactResult_HitActor 100.0 null self))
            (if (`SceneComponent.IsSimulatingPhysics` (`self.HitComponent`) (`self.HitBoneName`))
              (`PrimitiveComponent.AddImpulse` (`Character.Mesh` _asbase_character_class) _returnvalue (`self.HitBoneName`) true)))
          (:`CastFailed`
            (`GameplayStatics.ApplyDamage` ImpactResult_HitActor (`self.Damage`) null self :!label _label_3)))
        (elif (`self.ActorHasTag` ImpactResult_HitActor "weapon")
          (`GameplayStatics.ApplyDamage` ImpactResult_HitActor (`self.Damage`) null self)
          (`KismetSystemLibrary.Delay` 0.05)
          (`GameplayStatics.ApplyDamage` ImpactResult_HitActor (`self.Damage`) null self)
          (else
            (`/Engine/EditorBlueprintResources/StandardMacros.IsValid` _hitcomponent
              (:`Is Valid`
                (if (`SceneComponent.IsSimulatingPhysics` _hitcomponent "None")
                  (`PrimitiveComponent.AddImpulseAtLocation` (`self.HitComponent`) _returnvalue ImpactResult_Location "None")
                  (goto _label_3)
                  (else
                    (goto _label_3))))
              (:`Is Not Valid`
                (goto _label_3)))))))
    (:`Is Not Valid`
      (`GameplayStatics.SpawnEmitterAtLocation` "/Game/Assets/FPS_Weapons_Pack/Effects/ParticlesSystems/Impacts/Enviroment/P_Metal_Impact.P_Metal_Impact" ImpactResult_ImpactPoint)
      (`GameplayStatics.PlaySoundAtLocation` "/Game/Assets/AIBehaviorToolkit/Assets/Sounds/Sword/S_Sword_Hit01.S_Sword_Hit01" ImpactResult_ImpactPoint (struct) (`/Game/Blueprints/Dsm_GameInstance.Volume` (`self.GameInstance`)) 1.0 0.0 "/Game/Blueprints/SoundBlueprints/SoundAttenuationSettings.SoundAttenuationSettings")))
  (`/Engine/EditorBlueprintResources/StandardMacros.IsValid` _staticmesh_2
    (:`Is Valid`
      (`SceneComponent.SetVisibility` _staticmesh_2 false false)
      (`SceneComponent.SetVisibility` (`self.PointLight`) false false))
    (:`Is Not Valid`
      (`SceneComponent.SetVisibility` (`self.PointLight`) false false)))
  (`KismetSystemLibrary.Delay` 1.0)
  (`self.K2_DestroyActor`))

(event `self.Sphere.OnComponentBeginOverlap`
  (params (OverlappedComponent :type "PrimitiveComponent Object Reference") (OtherActor :type "Actor Object Reference") (OtherComp :type "PrimitiveComponent Object Reference") (OtherBodyIndex :type Integer) (bFromSweep :type Boolean) (SweepResult :type "HitResult Structure (by ref)")))

(fn `UserConstructionScript`)