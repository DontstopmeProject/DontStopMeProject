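; Shotgun weapon Blueprint that configures an inherited weapon base for this gun.
; BeginPlay calls the parent's spawn event with the shotgun's attack rate, ammo and weapon type.
; The construction script sets the Remington 870 destructible mesh and icon, clears the hit flag and snaps a point light to the sphere.
; Tick only calls the parent, while leftover physics-toggle and sphere-rotation logic is disconnected and never runs.
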(event `self.ReceiveBeginPlay`
  (`parent.ReceiveBeginPlay`)
  (`self.EventSpawned` 1.3 2 "NewEnumerator5"))

(event `self.ReceiveTick`
  (params (DeltaSeconds :type "Float (single-precision)"))
  (`parent.ReceiveTick` DeltaSeconds))

(fn `UserConstructionScript`
  (`parent.UserConstructionScript`)
  (set `self.HitEnemy` false)
  (set `self.Destructible` "/Game/Assets/FPS_Weapons_Pack/Weapons/Meshes/Rem870/SM_Rem870_DM.SM_Rem870_DM")
  (set `self.ImageWeapon` "/Game/Assets/Images/ShotgunIcon.ShotgunIcon")
  (`SceneComponent.K2_AttachToComponent` (`self.PointLight`) (`self.Sphere`) "None" "SnapToTarget" "KeepWorld" "KeepWorld" true))