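; AP5 weapon Blueprint that fires three-round bursts of pistol projectiles from its Sphere transform, with smoke, shells, sound, montage and camera shake.
; EventBaseAttack traces, then nested gates repeat bursts until StopAttack is set or the wielder cannot attack.
; Each burst suspends the wielder's and player's time-dilation changes, restoring them after a delay.
; An empty-ammo branch exists, but shots never increment AmmoCounter because that node is disconnected.
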(event `EventBaseAttack`
  (bind _player (`self.player`))
  (bind _player_2 (`self.player`))
  (bind _newvar_0_0 (`self.NewVar_0_0`))
  (bind _sphere (`self.Sphere`))
  (bind _firecounter (`self.FireCounter`))
  (bind _player_3 (`self.player`))
  (bind _returnvalue_location (`KismetMathLibrary.BreakTransform` (`SceneComponent.K2_GetComponentToWorld` (`self.Sphere`))))
  (bind (_returnvalue_location_2 _returnvalue_rotation) (`KismetMathLibrary.BreakTransform` (`SceneComponent.K2_GetComponentToWorld` (`self.Sphere`))))
  (bind (_returnvalue_location_3 _returnvalue_rotation_2) (`KismetMathLibrary.BreakTransform` (`SceneComponent.K2_GetComponentToWorld` (`self.Sphere`))))
  (`/Engine/EditorBlueprintResources/StandardMacros.DoOnce` false :!label _label
    (:`Completed`
      (`self.Trace` 0.0)
      (`|ExecutionSequence`
        (:`then_0`
          (goto _label_2 :!via `Close`))
        (:`then_1`
          (goto _label_2 :!via `Open`))
        (:`then_2`
          (`/Engine/EditorBlueprintResources/StandardMacros.Gate` true :!label _label_2
            (:`Exit`
              (if (not (`self.StopAttack`))
                (if (not (`/Game/Blueprints/BaseCharacterClass.CanAttack` (`self.NewVar_0_0`)))
                  (goto _label_2 :!via `Close`)
                  (elif (< (`self.AmmoCounter`) (`self.Ammo`))
                    (set `/Game/Blueprints/BaseCharacterClass.StopChangingCustomTime` true _newvar_0_0)
                    (set `Actor.CustomTimeDilation` 1.0 _newvar_0_0)
                    (`/Engine/EditorBlueprintResources/StandardMacros.IsValid` _player_3
                      (:`Is Valid`
                        (set `/Game/Blueprints/PlayersCharacter.ChangeTimeDilationInPlayersClass` false _player_3)
                        (set `/Game/Blueprints/PlayersCharacter.ShowAmmo` false _player_3)
                        (`GameplayStatics.SetGlobalTimeDilation` 1.0))
                      (:`Is Not Valid`
                        _))
                    (bind _output_get (set `self.ProjectileTransform` (`KismetMathLibrary.MakeTransform` _returnvalue_location_2 _returnvalue_rotation (0.5 0.5 0.5))))
                    (`self.ShotEventDispatcher`)
                    (set `self.StopRotate` true)
                    (`|ExecutionSequence`
                      (:`then_0`
                        (set `self.FireCounter` 0)
                        (goto _label_3 :!via `Open`))
                      (:`then_1`
                        (`/Engine/EditorBlueprintResources/StandardMacros.Gate` true :!label _label_3
                          (:`Exit`
                            (`self.ShakePlayersCamera` null 1.0)
                            (if (and (< _firecounter 3) (< (`self.AmmoCounter`) (`self.Ammo`)))
                              (`/Engine/EditorBlueprintResources/StandardMacros.IncrementInt` _firecounter
                                (:`  `
                                  (`/Engine/EditorBlueprintResources/StandardMacros.IsValid` (`self.player`)
                                    (:`Is Valid`
                                      _)
                                    (:`Is Not Valid`
                                      _))
                                  (bind _returnvalue (`|SpawnActorFromClass` "/Game/Blueprints/Weapons/projectiles/BP_PistolProjectile.BP_PistolProjectile_C" (`KismetMathLibrary.MakeTransform` _returnvalue_location_3 _returnvalue_rotation_2 (0.5 0.5 0.5)) "AlwaysSpawn" "OverrideRootScale" (`self.GetParentActor`) (`self.GetInstigator`)))
                                  (set `/Game/Blueprints/Weapons/projectiles/BP_ProjectileBase.DeathEnumVar` "NewEnumerator2" _returnvalue)
                                  (set `/Game/Blueprints/Weapons/projectiles/BP_ProjectileBase.DamageVelocity` 1200.0 _returnvalue)
                                  (`GameplayStatics.SpawnEmitterAtLocation` "/Game/Assets/FPS_Weapons_Pack/Effects/ParticlesSystems/Weapons/AP5/P_AP5_Barrel_Smoke.P_AP5_Barrel_Smoke" (`SceneComponent.K2_GetComponentLocation` _sphere) (`SceneComponent.K2_GetComponentRotation` _sphere))
                                  (`GameplayStatics.SpawnEmitterAtLocation` "/Game/Assets/FPS_Weapons_Pack/Effects/ParticlesSystems/Weapons/AP5/P_AP5_Shells.P_AP5_Shells")
                                  (`GameplayStatics.PlaySoundAtLocation` "/Game/Assets/AIBehaviorToolkit/Assets/Sounds/Rifle/S_AssaultRifle_Shot01.S_AssaultRifle_Shot01" _returnvalue_location (struct) 1.0 1.0 0.0 "/Game/Blueprints/SoundBlueprints/SoundAttenuationSettings.SoundAttenuationSettings")
                                  (`Character.PlayAnimMontage` (`self.NewVar_0_0`) "/Game/Assets/AIBehaviorToolkit/Assets/Mannequin/Animations/AM_FireRifle.AM_FireRifle" 1.0 "spine_01")
                                  (`KismetSystemLibrary.Delay` 0.15)
                                  (goto _label_3)))
                              (else
                                (`|ExecutionSequence`
                                  (:`then_0`
                                    (goto _label_3 :!via `Close`))
                                  (:`then_1`
                                    (`KismetSystemLibrary.Delay` 0.3)
                                    (set `/Game/Blueprints/BaseCharacterClass.StopChangingCustomTime` false (`self.NewVar_0_0`))
                                    (`/Engine/EditorBlueprintResources/StandardMacros.IsValid` _player
                                      (:`Is Valid`
                                        (set `/Game/Blueprints/PlayersCharacter.ChangeTimeDilationInPlayersClass` true _player)
                                        (set `/Game/Blueprints/PlayersCharacter.ShowAmmo` true _player))
                                      (:`Is Not Valid`
                                        _))
                                    (`KismetSystemLibrary.Delay` 0.3)
                                    (`self.ShotEventDispatcher`)
                                    (set `self.StopRotate` false)
                                    (`|ExecutionSequence`
                                      (:`then_0`
                                        (goto _label :!via `Reset`))
                                      (:`then_1`
                                        (goto _label_2)))))))))))
                    (else
                      (`/Engine/EditorBlueprintResources/StandardMacros.IsValid` _player_2
                        (:`Is Valid`
                          (bind _returnvalue_2 (`|CreateWidget` "/Game/Blueprints/Widgets/BaseWidgets/DamageWidget.DamageWidget_C"))
                          (bind _output_get_2 (set `/Game/Blueprints/BaseCharacterClass.DamgeHud` _returnvalue_2 _player_2))
                          (`UserWidget.AddToViewport` _output_get_2 0))
                        (:`Is Not Valid`
                          _))
                      (`GameplayStatics.PlaySoundAtLocation` "/Game/Assets/Sounds/Effects/EmptyPistol__WAV_.EmptyPistol__WAV_" (`self.K2_GetActorLocation` (`self.NewVar_0_0`)) (struct) (`/Game/Blueprints/Dsm_GameInstance.Volume` (`self.GameInstance`)) 1.0 0.0 "/Game/Blueprints/SoundBlueprints/SoundAttenuationSettings.SoundAttenuationSettings")
                      (`KismetSystemLibrary.Delay` 0.1)
                      (goto _label :!via `Reset`))))
                (else
                  (goto _label :!via `Reset`))))))))))

(fn `UserConstructionScript`
  (`parent.UserConstructionScript`))