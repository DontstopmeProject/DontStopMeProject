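; Ricochet pistol weapon that sets up its ammo, attack rate and type through its parent, plus icon and destructible.
; When held by the player it adjusts the aim sprite and each tick debug-draws a line trace with one mirrored bounce off the hit normal.
; When thrown it starts at the last owner's sphere, and its first hit on a differently tagged actor damages both target and pistol.
; Firing is not in this graph.
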(event `EventHitThrowedHuman`
  (if (not (`self.ActorHasTag` (`self.HitActor`) (`|GetArrayItem` (`self.Tags`) 2)))
    (`/Engine/EditorBlueprintResources/StandardMacros.DoOnce` false
      (:`Completed`
        (`GameplayStatics.ApplyDamage` (`self.HitActor`) 49.0 null self)
        (`PrimitiveComponent.SetCollisionResponseToChannel` (`self.StaticMesh`) "ECC_GameTraceChannel5" "ECR_Ignore")
        (`GameplayStatics.PlaySoundAtLocation` null (`self.K2_GetActorLocation`) (struct) (`/Game/Blueprints/Dsm_GameInstance.Volume` (`self.GameInstance_0`)) 1.0 0.0 "/Game/Blueprints/SoundBlueprints/SoundAttenuationSettings.SoundAttenuationSettings")
        (`GameplayStatics.ApplyDamage` self 50.0 null self)))))

(event `self.ReceiveBeginPlay`
  (bind _returnvalue (`self.GetParentActor`))
  (bind _sphere (`/Game/Blueprints/BaseCharacterClass.Sphere` (`self.LastOwnerActor`)))
  (`parent.ReceiveBeginPlay`)
  (`self.EventSpawned` 0.5 10 "NewEnumerator4")
  (bind _asdsm_game_instance (cast `/Game/Blueprints/Dsm_GameInstance` (`GameplayStatics.GetGameInstance`)))
  (set `self.GameInstance_0` _asdsm_game_instance)
  (if (`self.Throw`)
    (`SceneComponent.K2_SetWorldLocationAndRotation` (`self.StaticMesh`) (`SceneComponent.K2_GetComponentLocation` _sphere) (`KismetMathLibrary.Conv_VectorToRotator` (`SceneComponent.GetForwardVector` _sphere)) false false))
  (`/Engine/EditorBlueprintResources/StandardMacros.IsValid` _returnvalue
    (:`Is Valid`
      (bind _asbase_character_class (cast `/Game/Blueprints/BaseCharacterClass` _returnvalue))
      (set `self.NewVar_0_0` _asbase_character_class)
      (if (`self.ActorHasTag` (`self.GetParentActor`) "player")
        (bind _asplayers_character (cast `/Game/Blueprints/PlayersCharacter` (`self.NewVar_0_0`)))
        (bind _output_get (set `self.player_0` _asplayers_character))
        (`SceneComponent.K2_SetRelativeLocation` (`/Game/Blueprints/PlayersCharacter.AimSprite` _output_get) (101.0 10.0 63.419262) false false)))))

(event `self.ReceiveTick`
  (params (DeltaSeconds :type "Float (single-precision)"))
  (bind _sphere (`self.Sphere`))
  (bind _returnvalue (`SceneComponent.K2_GetComponentLocation` _sphere))
  (bind _returnvalue_2 (+ _returnvalue (* (`SceneComponent.GetForwardVector` _sphere) 5000.0)))
  (`parent.ReceiveTick` DeltaSeconds)
  (`/Engine/EditorBlueprintResources/StandardMacros.IsValid` (`self.player_0`)
    (:`Is Valid`
      (bind _outhit (`KismetSystemLibrary.LineTraceSingle` :`Start` _returnvalue :`End` _returnvalue_2 :`TraceChannel` "TraceTypeQuery1" :`DrawDebugType` "ForOneFrame"))
      (bind (_bblockinghit _binitialoverlap _time _location _impactpoint _normal _impactnormal) (`GameplayStatics.BreakHitResult` _outhit))
      (bind _outhit_2 (`KismetSystemLibrary.LineTraceSingle` :`Start` (+ _impactpoint _normal) :`End` (+ _impactpoint (`KismetMathLibrary.MirrorVectorByNormal` (- _returnvalue_2 _returnvalue) _impactnormal)) :`TraceChannel` "TraceTypeQuery1" :`DrawDebugType` "ForOneFrame")))))

(fn `UserConstructionScript`
  (`parent.UserConstructionScript`)
  (set `self.HitEnemy` false)
  (set `self.Destructible` "/Game/Assets/FPS_Weapons_Pack/Weapons/Meshes/Sock17/SM_Sock17_DM.SM_Sock17_DM")
  (set `self.ImageWeapon` "/Game/Assets/Images/PistolIcon.PistolIcon"))