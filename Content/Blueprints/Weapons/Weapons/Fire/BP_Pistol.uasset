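; Pistol weapon, built on a parent weapon class and held as a child actor by a player or other character.
; BaseAttack traces, then spawns a projectile with montage, shake and effects, or clicks when empty; ammo only counts down for players.
; When thrown, it damages the character hit and itself.
; A finisher event plays an attack animation on the owner, pausing movement and player input and resetting time dilation.
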(event `EventHitThrowedHuman`
  (if (not (`self.ActorHasTag` (`self.HitActor`) (`|GetArrayItem` (`self.Tags`) 2)))
    (`/Engine/EditorBlueprintResources/StandardMacros.DoOnce` false
      (:`Completed`
        (`GameplayStatics.ApplyDamage` (`self.HitActor`) 49.0 null self)
        (`PrimitiveComponent.SetCollisionResponseToChannel` (`self.StaticMesh`) "ECC_GameTraceChannel5" "ECR_Ignore")
        (`GameplayStatics.PlaySoundAtLocation` "/Game/Assets/Sounds/Effects/Weapons/WeaponThrowed_WAV_.WeaponThrowed_WAV_" (`self.K2_GetActorLocation`) (struct) (`/Game/Blueprints/Dsm_GameInstance.Volume` (`self.GameInstance`)) 1.0 0.0 "/Game/Blueprints/SoundBlueprints/SoundAttenuationSettings.SoundAttenuationSettings")
        (`GameplayStatics.ApplyDamage` self 50.0 null self)))))

(event `EventFinish`
  (bind _player (`self.player`))
  (bind _player_2 (`self.player`))
  (bind _newvar_0_0 (`self.NewVar_0_0`))
  (bind _newvar_0_0_2 (`self.NewVar_0_0`))
  (bind _mesh (`Character.Mesh` _newvar_0_0_2))
  (if (`/Game/Blueprints/BaseCharacterClass.CanFinish` (`self.NewVar_0_0`))
    (`/Engine/EditorBlueprintResources/StandardMacros.DoOnce` false :!label _label
      (:`Completed`
        (if (`self.ActorHasTag` "player")
          (`self.DisableInput` (`GameplayStatics.GetPlayerController` 0)))
        (`/Engine/EditorBlueprintResources/StandardMacros.IsValid` _player_2
          (:`Is Valid`
            (set `/Game/Blueprints/PlayersCharacter.ChangeTimeDilationInPlayersClass` false _player_2))
          (:`Is Not Valid`
            _))
        (`GameplayStatics.SetGlobalTimeDilation` 1.0)
        (`ActorComponent.Deactivate` (`Character.CharacterMovement` (`self.NewVar_0_0`)))
        (`/Game/Blueprints/BaseCharacterClass.FinishDispatcher` (`self.NewVar_0_0`))
        (`self.ShotEventDispatcher`)
        (`SkeletalMeshComponent.PlayAnimation` (`Character.Mesh` _newvar_0_0) "/Game/Assets/SwordAnimSet/Animations/InPlace/Attack_Run_Jump_T.Attack_Run_Jump_T" false)
        (set `/Game/Blueprints/BaseCharacterClass.CanFinish` false _newvar_0_0)
        (`KismetSystemLibrary.Delay` 0.3)
        (`GameplayStatics.PlaySoundAtLocation` "/Game/Assets/AIBehaviorToolkit/Assets/Sounds/Sword/S_Sword_Stab01.S_Sword_Stab01" (`self.K2_GetActorLocation` (`self.NewVar_0_0`)) (struct) (`/Game/Blueprints/Dsm_GameInstance.Volume` (`self.GameInstance`)) 1.0 0.0 "/Game/Blueprints/SoundBlueprints/SoundAttenuationSettings.SoundAttenuationSettings")
        (`KismetSystemLibrary.Delay` 1.0)
        (`self.ShotEventDispatcher`)
        (`/Game/Blueprints/BaseCharacterClass.FinishDispatcher` (`self.NewVar_0_0`))
        (`KismetSystemLibrary.Delay` 0.2)
        (if (`self.ActorHasTag` (`self.NewVar_0_0`) "player")
          (`self.EnableInput` (`GameplayStatics.GetPlayerController` 0)))
        (`ActorComponent.Activate` (`Character.CharacterMovement` _newvar_0_0_2) false)
        (`PrimitiveComponent.SetCollisionEnabled` (`self.Sphere`) "NoCollision")
        (`/Engine/EditorBlueprintResources/StandardMacros.IsValid` _player
          (:`Is Valid`
            (set `/Game/Blueprints/PlayersCharacter.ChangeTimeDilationInPlayersClass` true _player))
          (:`Is Not Valid`
            _))
        (`SkeletalMeshComponent.SetAnimationMode` _mesh "AnimationBlueprint")
        (`SkeletalMeshComponent.SetAnimInstanceClass` _mesh "/Game/Assets/AnimStarterPack/UE4ASP_HeroTPP_AnimBlueprint.UE4ASP_HeroTPP_AnimBlueprint_C")
        (goto _label :!via `Reset`)))))

(event `self.ReceiveBeginPlay`
  (bind _returnvalue (`self.GetParentActor`))
  (bind _sphere (`/Game/Blueprints/BaseCharacterClass.Sphere` (`self.LastOwnerActor`)))
  (`parent.ReceiveBeginPlay`)
  (`self.EventSpawned` 0.5 5 "NewEnumerator4")
  (bind _asdsm_game_instance (cast `/Game/Blueprints/Dsm_GameInstance` (`GameplayStatics.GetGameInstance`)))
  (set `self.GameInstance` _asdsm_game_instance)
  (if (`self.Throw`)
    (`SceneComponent.K2_SetWorldLocationAndRotation` (`self.StaticMesh`) (`SceneComponent.K2_GetComponentLocation` _sphere) (`KismetMathLibrary.Conv_VectorToRotator` (`SceneComponent.GetForwardVector` _sphere)) false false))
  (`/Engine/EditorBlueprintResources/StandardMacros.IsValid` _returnvalue
    (:`Is Valid`
      (bind _asbase_character_class (cast `/Game/Blueprints/BaseCharacterClass` _returnvalue))
      (set `self.NewVar_0_0` _asbase_character_class)
      (if (`self.ActorHasTag` (`self.GetParentActor`) "player")
        (bind _asplayers_character (cast `/Game/Blueprints/PlayersCharacter` (`self.NewVar_0_0`)))
        (bind _output_get (set `self.player` _asplayers_character))
        (`SceneComponent.K2_SetRelativeLocation` (`/Game/Blueprints/PlayersCharacter.AimSprite` _output_get) (101.0 10.0 63.419262) false false))
      (set `self.StopAttack` false))))

(event `self.ReceiveTick`
  (params (DeltaSeconds :type "Float (single-precision)"))
  (bind _returnvalue (`self.K2_GetActorRotation`))
  (bind _returnvalue_2 (`self.GetParentActor`))
  (bind _sphere (`self.Sphere`))
  (bind _returnvalue_3 (`self.K2_GetActorRotation` _returnvalue_2))
  (`parent.ReceiveTick` DeltaSeconds)
  (`self.EventTogglePhysics`)
  (`/Engine/EditorBlueprintResources/StandardMacros.IsValid` _returnvalue_2
    (:`Is Valid`
      (if (!= _returnvalue_3 _returnvalue)
        (if (`self.StopRotate`)
          (`SceneComponent.K2_SetWorldRotation` _sphere (`KismetMathLibrary.MakeRotator` (.roll _returnvalue_3) (.pitch _returnvalue) (.yaw _returnvalue_3)) false false)
          (else
            (`SceneComponent.K2_SetWorldRotation` _sphere _returnvalue_3 false false)))))))

(event `EventBaseAttack`
  (bind _player (`self.player`))
  (bind _projectiletransform (`self.ProjectileTransform`))
  (bind _player_2 (`self.player`))
  (bind (_returnvalue_location _returnvalue_rotation) (`KismetMathLibrary.BreakTransform` (`SceneComponent.K2_GetComponentToWorld` (`self.Sphere`))))
  (bind _volume (`/Game/Blueprints/Dsm_GameInstance.Volume` (`self.GameInstance`)))
  (if (`self.ResetAttack`)
    (`self.Trace` 2000.0)
    (if (not (`self.StopAttack`))
      (if (< (`self.AmmoCounter`) (`self.Ammo`))
        (set `self.ResetAttack` false)
        (`/Engine/EditorBlueprintResources/StandardMacros.IsValid` _player_2
          (:`Is Valid`
            (set `/Game/Blueprints/PlayersCharacter.ShowAmmo` false _player_2)
            (`/Engine/EditorBlueprintResources/StandardMacros.IncrementInt` (`self.AmmoCounter`)
              (:`  `
                _)))
          (:`Is Not Valid`
            _))
        (bind _output_get (set `self.ProjectileTransform` (`KismetMathLibrary.MakeTransform` _returnvalue_location _returnvalue_rotation (0.5 0.5 0.5))))
        (`self.ShotEventDispatcher`)
        (`GameplayStatics.PlaySoundAtLocation` "/Game/Assets/Sounds/Effects/Weapons/10mm_Gun-box_o_bu-8676_hifi__WAV_.10mm_Gun-box_o_bu-8676_hifi__WAV_" (.location _output_get) (struct) 1.0 1.0 0.0 "/Game/Blueprints/SoundBlueprints/SoundAttenuationSettings.SoundAttenuationSettings")
        (set `self.StopRotate` true)
        (`self.ShakePlayersCamera` null 2.0)
        (`Character.PlayAnimMontage` (`self.NewVar_0_0`) "/Game/Assets/AnimStarterPack/Pistol/AM_PistolFire.AM_PistolFire" 3.0 "spine_01")
        (`GameplayStatics.SpawnEmitterAtLocation` "/Game/Assets/FPS_Weapons_Pack/Effects/ParticlesSystems/Weapons/Sock17/P_Sock17_Barrel_Smoke.P_Sock17_Barrel_Smoke" (`SceneComponent.K2_GetComponentLocation` (`self.Sphere`)))
        (`GameplayStatics.SpawnEmitterAtLocation` "/Game/Assets/FPS_Weapons_Pack/Effects/ParticlesSystems/Weapons/Sock17/P_Sock17_Shells.P_Sock17_Shells" (`SceneComponent.K2_GetComponentLocation` (`self.Sphere1`)))
        (bind _returnvalue (`|SpawnActorFromClass` "/Game/Blueprints/Weapons/projectiles/BP_PistolProjectile.BP_PistolProjectile_C" _projectiletransform "AdjustIfPossibleButAlwaysSpawn" "OverrideRootScale" (`self.GetParentActor`) (`self.GetInstigator`)))
        (`GameplayStatics.PlaySoundAtLocation` "/Game/Assets/Sounds/Effects/Weapons/ShellFelt_WAV_.ShellFelt_WAV_" (.location _projectiletransform) (.rotation _projectiletransform) 0.3 1.0 0.0 "/Game/Blueprints/SoundBlueprints/SoundAttenuationSettings.SoundAttenuationSettings")
        (set `/Game/Blueprints/Weapons/projectiles/BP_ProjectileBase.DeathEnumVar` "NewEnumerator2" _returnvalue)
        (set `/Game/Blueprints/Weapons/projectiles/BP_ProjectileBase.DamageVelocity` 800.0 _returnvalue)
        (set `self.StopRotate` false)
        (else
          (set `self.ResetAttack` false)
          (`/Engine/EditorBlueprintResources/StandardMacros.IsValid` _player
            (:`Is Valid`
              (bind _returnvalue_2 (`|CreateWidget` "/Game/Blueprints/Widgets/BaseWidgets/DamageWidget.DamageWidget_C"))
              (bind _output_get_2 (set `/Game/Blueprints/BaseCharacterClass.DamgeHud` _returnvalue_2 _player))
              (`UserWidget.AddToViewport` _output_get_2 0))
            (:`Is Not Valid`
              _))
          (`GameplayStatics.PlaySoundAtLocation` "/Game/Assets/Sounds/Effects/EmptyPistol__WAV_.EmptyPistol__WAV_" (`self.K2_GetActorLocation` (`self.NewVar_0_0`)) (struct) (+ _volume (* _volume 0.3)) 1.0 0.0 "/Game/Blueprints/SoundBlueprints/SoundAttenuationSettings.SoundAttenuationSettings")
          (`KismetSystemLibrary.Delay` 0.2)
          (set `self.ResetAttack` true))))))

(fn `Fire`)

(fn `UserConstructionScript`
  (`parent.UserConstructionScript`)
  (set `self.HitEnemy` false)
  (set `self.Destructible` "/Game/Assets/FPS_Weapons_Pack/Weapons/Meshes/Sock17/SM_Sock17_DM.SM_Sock17_DM")
  (set `self.SeeAmmoMontage` "/Game/Assets/AIBehaviorToolkit/Assets/Mannequin/Animations/AM_SeePistolAmmo.AM_SeePistolAmmo")
  (set `self.ImageWeapon` "/Game/Assets/Images/PistolIcon.PistolIcon"))