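; Child weapon Blueprint for the AP5 (MP5-style) fire weapon, supplying its fire rate, ammo, type, icon, ammo-check montage and destructible mesh to the parent class.
; BeginPlay initializes these stats through EventSpawned, caches the game instance and aligns the mesh to the last owner's sphere when thrown.
; When parented to a player, it repositions that player's aim sprite and rotates itself along the parent's right vector.
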(event `self.ReceiveBeginPlay`
  (bind _returnvalue (`self.GetParentActor`))
  (bind _sphere (`/Game/Blueprints/BaseCharacterClass.Sphere` (`self.LastOwnerActor`)))
  (`parent.ReceiveBeginPlay`)
  (`self.EventSpawned` 0.233 20 "NewEnumerator5")
  (bind _asdsm_game_instance (cast `/Game/Blueprints/Dsm_GameInstance` (`GameplayStatics.GetGameInstance`)))
  (set `self.GameInstance_0` _asdsm_game_instance)
  (if (`self.Throw`)
    (`SceneComponent.K2_SetWorldLocationAndRotation` (`self.StaticMesh`) (`SceneComponent.K2_GetComponentLocation` _sphere) (`KismetMathLibrary.Conv_VectorToRotator` (`SceneComponent.GetForwardVector` _sphere)) false false))
  (`/Engine/EditorBlueprintResources/StandardMacros.IsValid` _returnvalue
    (:`Is Valid`
      (bind _asbase_character_class (cast `/Game/Blueprints/BaseCharacterClass` _returnvalue))
      (set `self.NewVar_0_0` _asbase_character_class)
      (if (`self.ActorHasTag` (`self.GetParentActor`) "player")
        (bind _asplayers_character (cast `/Game/Blueprints/PlayersCharacter` (`self.NewVar_0_0`)))
        (bind _output_get (set `self.player_0` _asplayers_character))
        (`SceneComponent.K2_SetRelativeLocation` (`/Game/Blueprints/PlayersCharacter.AimSprite` _output_get) (100.0 10.0 63.419262) false false)
        (`self.K2_SetActorRotation` (`KismetMathLibrary.Conv_VectorToRotator` (`KismetMathLibrary.GetRightVector` (`self.K2_GetActorRotation` (`self.GetParentActor`)))) true)))))

(event `self.ReceiveTick`
  (params (DeltaSeconds :type "Float (single-precision)"))
  (`parent.ReceiveTick` DeltaSeconds))

(fn `UserConstructionScript`
  (`parent.UserConstructionScript`)
  (set `self.HitEnemy` false)
  (set `self.Destructible` "/Game/Assets/FPS_Weapons_Pack/Weapons/Meshes/AP5/SM_AP5_X_DM.SM_AP5_X_DM")
  (set `self.SeeAmmoMontage` "/Game/Assets/AIBehaviorToolkit/Assets/Mannequin/Animations/AM_SeeRifleAmmo.AM_SeeRifleAmmo")
  (set `self.ImageWeapon` "/Game/Assets/Images/Mp5Icon.Mp5Icon")
  (`SceneComponent.K2_AttachToComponent` (`self.PointLight`) (`self.Sphere`) "None" "SnapToTarget" "KeepWorld" "KeepWorld" true))