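; MP5K submachine gun weapon, a child of a shared weapon base, usable by player or other characters and throwable.
; BaseAttack loops through a gate until stopped, spawning pistol projectiles with effects until ammo runs out, then clicking empty.
; Shots and the timed finisher animation reset time dilation and suspend the player's control of it.
; Tick aligns the gun to its parent; thrown hits stun characters and damage the gun itself.
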(event `EventFinish`
  (bind _player (`self.player`))
  (bind _player_2 (`self.player`))
  (bind _newvar_0_0 (`self.NewVar_0_0`))
  (bind _newvar_0_0_2 (`self.NewVar_0_0`))
  (bind _mesh (`Character.Mesh` _newvar_0_0_2))
  (if (`/Game/Blueprints/BaseCharacterClass.CanFinish` (`self.NewVar_0_0`))
    (`/Engine/EditorBlueprintResources/StandardMacros.DoOnce` false :!label _label
      (:`Completed`
        (if (`self.ActorHasTag` (`self.NewVar_0_0`) "player")
          (`self.DisableInput` (`GameplayStatics.GetPlayerController` 0)))
        (`/Engine/EditorBlueprintResources/StandardMacros.IsValid` _player_2
          (:`Is Valid`
            (set `/Game/Blueprints/PlayersCharacter.ChangeTimeDilationInPlayersClass` false _player_2))
          (:`Is Not Valid`
            _))
        (`GameplayStatics.SetGlobalTimeDilation` 1.0)
        (`ActorComponent.Deactivate` (`Character.CharacterMovement` (`self.NewVar_0_0`)))
        (`/Game/Blueprints/BaseCharacterClass.FinishDispatcher` (`self.NewVar_0_0`))
        (`self.ShotEventDispatcher`)
        (`SkeletalMeshComponent.PlayAnimation` (`Character.Mesh` _newvar_0_0) "/Game/Assets/SwordAnimSet/Animations/InPlace/Attack_Run_Jump_T.Attack_Run_Jump_T" false)
        (set `/Game/Blueprints/BaseCharacterClass.CanFinish` false _newvar_0_0)
        (`KismetSystemLibrary.Delay` 0.3)
        (`GameplayStatics.PlaySoundAtLocation` "/Game/Assets/AIBehaviorToolkit/Assets/Sounds/Sword/S_Sword_Stab01.S_Sword_Stab01" (`self.K2_GetActorLocation` (`self.NewVar_0_0`)) (struct) (`/Game/Blueprints/Dsm_GameInstance.Volume` (`self.GameInstance`)) 1.0 0.0 "/Game/Blueprints/SoundBlueprints/SoundAttenuationSettings.SoundAttenuationSettings")
        (`KismetSystemLibrary.Delay` 1.0)
        (`self.ShotEventDispatcher`)
        (`/Game/Blueprints/BaseCharacterClass.FinishDispatcher` (`self.NewVar_0_0`))
        (`KismetSystemLibrary.Delay` 0.2)
        (if (`self.ActorHasTag` (`self.NewVar_0_0`) "player")
          (`self.EnableInput` (`GameplayStatics.GetPlayerController` 0)))
        (`ActorComponent.Activate` (`Character.CharacterMovement` _newvar_0_0_2) false)
        (`PrimitiveComponent.SetCollisionEnabled` (`self.Sphere`) "NoCollision")
        (`/Engine/EditorBlueprintResources/StandardMacros.IsValid` _player
          (:`Is Valid`
            (set `/Game/Blueprints/PlayersCharacter.ChangeTimeDilationInPlayersClass` true _player))
          (:`Is Not Valid`
            _))
        (`SkeletalMeshComponent.SetAnimationMode` _mesh "AnimationBlueprint")
        (`SkeletalMeshComponent.SetAnimInstanceClass` _mesh "/Game/Assets/AnimStarterPack/UE4ASP_HeroTPP_AnimBlueprint.UE4ASP_HeroTPP_AnimBlueprint_C")
        (goto _label :!via `Reset`)))))

(event `self.ReceiveBeginPlay`
  (bind _returnvalue (`self.GetParentActor`))
  (bind _sphere (`/Game/Blueprints/BaseCharacterClass.Sphere` (`self.LastOwnerActor`)))
  (`parent.ReceiveBeginPlay`)
  (`self.EventSpawned` 0.233 20 "NewEnumerator5")
  (bind _asdsm_game_instance (cast `/Game/Blueprints/Dsm_GameInstance` (`GameplayStatics.GetGameInstance`)))
  (set `self.GameInstance` _asdsm_game_instance)
  (if (`self.Throw`)
    (`SceneComponent.K2_SetWorldLocationAndRotation` (`self.StaticMesh`) (`SceneComponent.K2_GetComponentLocation` _sphere) (`KismetMathLibrary.Conv_VectorToRotator` (`SceneComponent.GetForwardVector` _sphere)) false false))
  (`/Engine/EditorBlueprintResources/StandardMacros.IsValid` _returnvalue
    (:`Is Valid`
      (bind _asbase_character_class (cast `/Game/Blueprints/BaseCharacterClass` _returnvalue))
      (set `self.NewVar_0_0` _asbase_character_class)
      (if (`self.ActorHasTag` (`self.GetParentActor`) "player")
        (bind _asplayers_character (cast `/Game/Blueprints/PlayersCharacter` (`self.NewVar_0_0`)))
        (bind _output_get (set `self.player` _asplayers_character))
        (`SceneComponent.K2_SetRelativeLocation` (`/Game/Blueprints/PlayersCharacter.PaperSprite` _output_get) (100.0 10.0 63.419262) false false)
        (`self.K2_SetActorRotation` (`KismetMathLibrary.Conv_VectorToRotator` (`KismetMathLibrary.GetRightVector` (`self.K2_GetActorRotation` (`self.GetParentActor`)))) true)))))

(event `EventHitThrowedHuman`
  (bind _tags (`self.Tags`))
  (if (`KismetArrayLibrary.Array_IsValidIndex` _tags 2)
    (if (not (`self.ActorHasTag` (`self.HitActor`) (`|GetArrayItem` _tags 2)))
      (`/Engine/EditorBlueprintResources/StandardMacros.DoOnce` false :!label _label_2
        (:`Completed`
          (bind _asbase_character_class (cast `/Game/Blueprints/BaseCharacterClass` (`self.HitActor`))
            (:`then`
              (`/Game/Blueprints/BaseCharacterClass.EventStun` _asbase_character_class)
              (`PrimitiveComponent.SetCollisionResponseToChannel` (`self.StaticMesh`) "ECC_GameTraceChannel4" "ECR_Ignore"))
            (:`CastFailed`
              _))
          (`GameplayStatics.ApplyDamage` self 50.0 null self)
          (`PrimitiveComponent.SetCollisionResponseToChannel` (`self.StaticMesh`) "ECC_GameTraceChannel5" "ECR_Ignore")
          (`GameplayStatics.PlaySoundAtLocation` "/Game/Assets/Sounds/Effects/Weapons/WeaponThrowed_WAV_.WeaponThrowed_WAV_" (`self.K2_GetActorLocation`) (struct) (`/Game/Blueprints/Dsm_GameInstance.Volume` (`self.GameInstance`)) 1.0 0.0 "/Game/Blueprints/SoundBlueprints/SoundAttenuationSettings.SoundAttenuationSettings"))))
    (else
      (goto _label_2))))

(event `self.ReceiveTick`
  (params (DeltaSeconds :type "Float (single-precision)"))
  (bind _returnvalue (`self.GetParentActor`))
  (bind _returnvalue_2 (`KismetMathLibrary.GetRightVector` (`self.K2_GetActorRotation` _returnvalue)))
  (bind (_returnvalue_roll _returnvalue_pitch _returnvalue_yaw) (`KismetMathLibrary.BreakRotator` (`KismetMathLibrary.Conv_VectorToRotator` _returnvalue_2)))
  (`parent.ReceiveTick` DeltaSeconds)
  (`self.EventTogglePhysics`)
  (`/Engine/EditorBlueprintResources/StandardMacros.IsValid` _returnvalue
    (:`Is Valid`
      (if (`self.StopRotate`)
        (`self.K2_SetActorRotation` (`KismetMathLibrary.MakeRotator` (.roll (`self.K2_GetActorRotation`)) (.pitch (`self.K2_GetActorRotation`)) _returnvalue_yaw) true)
        (else
          (`self.K2_SetActorRotation` (`KismetMathLibrary.Conv_VectorToRotator` _returnvalue_2) true))))))

(event `EventBaseAttack`
  (bind _player (`self.player`))
  (bind _player_2 (`self.player`))
  (bind _newvar_0_0 (`self.NewVar_0_0`))
  (bind _sphere (`self.Sphere`))
  (bind (_returnvalue_location _returnvalue_rotation) (`KismetMathLibrary.BreakTransform` (`SceneComponent.K2_GetComponentToWorld` (`self.Sphere`))))
  (`/Engine/EditorBlueprintResources/StandardMacros.DoOnce` false :!label _label_3
    (:`Completed`
      (`|ExecutionSequence`
        (:`then_0`
          (goto _label_4 :!via `Close`))
        (:`then_1`
          (goto _label_4 :!via `Open`))
        (:`then_2`
          (`/Engine/EditorBlueprintResources/StandardMacros.Gate` true :!label _label_4
            (:`Exit`
              (if (or (`self.StopAttack`) (not (`/Game/Blueprints/BaseCharacterClass.CanAttack` (`self.NewVar_0_0`))))
                (goto _label_4 :!via `Close`)
                (elif (< (`self.AmmoCounter`) (`self.Ammo`))
                  (`/Engine/EditorBlueprintResources/StandardMacros.IncrementInt` (`self.AmmoCounter`)
                    (:`  `
                      (set `/Game/Blueprints/BaseCharacterClass.StopChangingCustomTime` true _newvar_0_0)
                      (set `Actor.CustomTimeDilation` 1.0 _newvar_0_0)
                      (`/Engine/EditorBlueprintResources/StandardMacros.IsValid` _player_2
                        (:`Is Valid`
                          (set `/Game/Blueprints/PlayersCharacter.ChangeTimeDilationInPlayersClass` false _player_2)
                          (`GameplayStatics.SetGlobalTimeDilation` 1.0))
                        (:`Is Not Valid`
                          _))
                      (bind _output_get (set `self.ProjectileTransform` (`KismetMathLibrary.MakeTransform` _returnvalue_location _returnvalue_rotation (0.5 0.5 0.5))))
                      (`self.ShotEventDispatcher`)
                      (`GameplayStatics.PlaySoundAtLocation` "/Game/Assets/AIBehaviorToolkit/Assets/Sounds/Rifle/S_AssaultRifle_Shot01.S_AssaultRifle_Shot01" (.location _output_get) (struct) (`/Game/Blueprints/Dsm_GameInstance.Volume` (`self.GameInstance`)) 1.0 0.0 "/Game/Blueprints/SoundBlueprints/SoundAttenuationSettings.SoundAttenuationSettings")
                      (`self.Trace`)
                      (set `self.StopRotate` true)
                      (bind _returnvalue (`|SpawnActorFromClass` "/Game/Blueprints/Weapons/projectiles/BP_PistolProjectile.BP_PistolProjectile_C" (`self.ProjectileTransform`) "AdjustIfPossibleButAlwaysSpawn" "OverrideRootScale" (`self.GetParentActor`) (`self.GetInstigator`)))
                      (set `/Game/Blueprints/Weapons/projectiles/BP_ProjectileBase.DeathEnumVar` "NewEnumerator2" _returnvalue)
                      (set `/Game/Blueprints/Weapons/projectiles/BP_ProjectileBase.DamageVelocity` 1200.0 _returnvalue)
                      (`GameplayStatics.SpawnEmitterAtLocation` "/Game/Assets/FPS_Weapons_Pack/Effects/ParticlesSystems/Weapons/AP5/P_AP5_Barrel_Smoke.P_AP5_Barrel_Smoke" (`SceneComponent.K2_GetComponentLocation` _sphere) (`SceneComponent.K2_GetComponentRotation` _sphere))
                      (`GameplayStatics.SpawnEmitterAtLocation` "/Game/Assets/FPS_Weapons_Pack/Effects/ParticlesSystems/Weapons/AP5/P_AP5_Shells.P_AP5_Shells" (`SceneComponent.K2_GetComponentLocation` (`self.Sphere1`)))
                      (`KismetSystemLibrary.Delay` 0.216)
                      (set `/Game/Blueprints/BaseCharacterClass.StopChangingCustomTime` false (`self.NewVar_0_0`))
                      (`/Engine/EditorBlueprintResources/StandardMacros.IsValid` _player
                        (:`Is Valid`
                          (set `/Game/Blueprints/PlayersCharacter.ChangeTimeDilationInPlayersClass` true _player))
                        (:`Is Not Valid`
                          _))
                      (`KismetSystemLibrary.Delay` (- (`self.AttackRate`) 0.216))
                      (`self.ShotEventDispatcher`)
                      (set `self.StopRotate` false)
                      (`|ExecutionSequence`
                        (:`then_0`
                          (goto _label_3 :!via `Reset`))
                        (:`then_1`
                          (goto _label_4)))))
                  (else
                    (`KismetSystemLibrary.Delay` 0.1)
                    (`|ExecutionSequence`
                      (:`then_0`
                        (goto _label_5 :!via `Reset`))
                      (:`then_1`
                        (`/Engine/EditorBlueprintResources/StandardMacros.DoOnce` false :!label _label_5
                          (:`Completed`
                            (`GameplayStatics.PlaySoundAtLocation` "/Game/Assets/Sounds/Effects/EmptyPistol__WAV_.EmptyPistol__WAV_" (`self.K2_GetActorLocation` (`self.NewVar_0_0`)) (struct) (`/Game/Blueprints/Dsm_GameInstance.Volume` (`self.GameInstance`)) 1.0 0.0 "/Game/Blueprints/SoundBlueprints/SoundAttenuationSettings.SoundAttenuationSettings")
                            (goto _label_4)))))))))))))))

(fn `UserConstructionScript`
  (`parent.UserConstructionScript`)
  (set `self.Arms` false)
  (set `self.Destructible` "/Game/Assets/FPS_Weapons_Pack/Weapons/Meshes/AP5/SM_AP5_X_DM.SM_AP5_X_DM"))