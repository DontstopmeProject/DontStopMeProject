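; Shotgun weapon child Blueprint, held as a child actor by characters, that never increments its ammo counter itself.
; Attacking briefly restores normal time dilation, runs a trace, spawns randomly spread pistol projectiles, then plays delayed reload effects before the attack gate resets.
; Tick matches the owner's rotation, keeping its own pitch while firing.
; When thrown, it stuns the character it hits and damages itself.
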(event `self.ReceiveBeginPlay`
  (bind _returnvalue (`self.GetParentActor`))
  (bind _sphere (`/Game/Blueprints/BaseCharacterClass.Sphere` (`self.LastOwnerActor`)))
  (`parent.ReceiveBeginPlay`)
  (`self.EventSpawned` 1.0 2 "NewEnumerator5")
  (bind _asdsm_game_instance (cast `/Game/Blueprints/Dsm_GameInstance` (`GameplayStatics.GetGameInstance`)))
  (set `self.GameInstance` _asdsm_game_instance)
  (if (`self.Throw`)
    (`SceneComponent.K2_SetWorldLocationAndRotation` (`self.StaticMesh`) (`SceneComponent.K2_GetComponentLocation` _sphere) (`KismetMathLibrary.Conv_VectorToRotator` (`SceneComponent.GetForwardVector` _sphere)) false false))
  (`/Engine/EditorBlueprintResources/StandardMacros.IsValid` _returnvalue
    (:`Is Valid`
      (bind _asbase_character_class (cast `/Game/Blueprints/BaseCharacterClass` (`self.GetParentActor`)))
      (set `self.NewVar_0_0` _asbase_character_class)
      (if (`self.ActorHasTag` _returnvalue "player")
        (bind _asplayers_character (cast `/Game/Blueprints/PlayersCharacter` (`self.NewVar_0_0`)))
        (bind _output_get (set `self.Player` _asplayers_character))
        (`SceneComponent.K2_SetRelativeLocation` (`/Game/Blueprints/PlayersCharacter.AimSprite` _output_get) (125.0 18.0 63.419262) false false)))))

(event `EventHitThrowedHuman`
  (if (not (`self.ActorHasTag` (`self.HitActor`) (`|GetArrayItem` (`self.Tags`) 2)))
    (`/Engine/EditorBlueprintResources/StandardMacros.DoOnce` false
      (:`Completed`
        (bind _asbase_character_class (cast `/Game/Blueprints/BaseCharacterClass` (`self.HitActor`)))
        (`/Game/Blueprints/BaseCharacterClass.EventStun` _asbase_character_class)
        (`PrimitiveComponent.SetCollisionResponseToChannel` (`self.StaticMesh`) "ECC_GameTraceChannel4" "ECR_Ignore")
        (`GameplayStatics.ApplyDamage` self 50.0 null self)
        (`PrimitiveComponent.SetCollisionResponseToChannel` (`self.StaticMesh`) "ECC_GameTraceChannel5" "ECR_Ignore")
        (`GameplayStatics.PlaySoundAtLocation` "/Game/Assets/Sounds/Effects/Weapons/WeaponThrowed_WAV_.WeaponThrowed_WAV_" (`self.K2_GetActorLocation`) (struct) (`/Game/Blueprints/Dsm_GameInstance.Volume` (`self.GameInstance`)) 1.0 0.0 "/Game/Blueprints/SoundBlueprints/SoundAttenuationSettings.SoundAttenuationSettings")))))

(event `self.ReceiveTick`
  (params (DeltaSeconds :type "Float (single-precision)"))
  (bind _returnvalue (`self.GetParentActor`))
  (`parent.ReceiveTick` DeltaSeconds)
  (`self.EventTogglePhysics`)
  (`/Engine/EditorBlueprintResources/StandardMacros.IsValid` _returnvalue
    (:`Is Valid`
      (if (!= (`self.K2_GetActorRotation` _returnvalue) (`self.K2_GetActorRotation`))
        (if (`self.StopRotate`)
          (`self.K2_SetActorRotation` (`KismetMathLibrary.MakeRotator` (.roll (`self.K2_GetActorRotation` (`self.GetParentActor`))) (.pitch (`self.K2_GetActorRotation`)) (.yaw (`self.K2_GetActorRotation` (`self.GetParentActor`)))) true)
          (else
            (`self.K2_SetActorRotation` (`self.K2_GetActorRotation` _returnvalue) true)))))))

(event `EventBaseAttack`
  (bind _player (`self.player`))
  (bind _newvar_0_0 (`self.NewVar_0_0`))
  (bind _sphere (`self.Sphere`))
  (bind _player_2 (`self.player`))
  (bind (_projectiletransform_location _projectiletransform_rotation) (`KismetMathLibrary.BreakTransform` (`self.ProjectileTransform`)))
  (bind (_returnvalue_location _returnvalue_rotation) (`KismetMathLibrary.BreakTransform` (`SceneComponent.K2_GetComponentToWorld` (`self.Sphere`))))
  (bind _returnvalue_location_2 (`KismetMathLibrary.BreakTransform` (`SceneComponent.K2_GetComponentToWorld` (`self.Sphere`))))
  (bind (_returnvalue_x _returnvalue_y _returnvalue_z) (`KismetMathLibrary.BreakVector` (+ _projectiletransform_location (`KismetMathLibrary.MakeVector` (`KismetMathLibrary.RandomFloatInRange` 2.0 4.0) (`KismetMathLibrary.RandomFloatInRange` 1.0 5.0) (`KismetMathLibrary.RandomFloatInRange` -2.0 -5.0)))))
  (`/Engine/EditorBlueprintResources/StandardMacros.DoOnce` false :!label _label
    (:`Completed`
      (if (and (not (`self.StopAttack`)) (< (`self.AmmoCounter`) (`self.Ammo`)))
        (set `/Game/Blueprints/BaseCharacterClass.StopChangingCustomTime` true _newvar_0_0)
        (set `Actor.CustomTimeDilation` 1.0 _newvar_0_0)
        (`/Engine/EditorBlueprintResources/StandardMacros.IsValid` _player_2
          (:`Is Valid`
            (set `/Game/Blueprints/PlayersCharacter.ShowAmmo` false _player_2)
            (set `/Game/Blueprints/PlayersCharacter.ChangeTimeDilationInPlayersClass` false _player_2)
            (`GameplayStatics.SetGlobalTimeDilation` 1.0))
          (:`Is Not Valid`
            _))
        (set `self.StopRotate` true)
        (`self.ShotEventDispatcher`)
        (bind _output_get (set `self.ProjectileTransform` (`KismetMathLibrary.MakeTransform` (- _returnvalue_location (10.0 5.0 10.0)) (`KismetMathLibrary.ComposeRotators` _returnvalue_rotation (struct :`Yaw` -10.0)) (0.5 0.5 0.5))))
        (`GameplayStatics.PlaySoundAtLocation` "/Game/Assets/Sounds/Effects/Weapons/ShotgunFire.ShotgunFire" (.location _output_get) (struct) (`/Game/Blueprints/Dsm_GameInstance.Volume` (`self.GameInstance`)) 1.0 0.0 "/Game/Blueprints/SoundBlueprints/SoundAttenuationSettings.SoundAttenuationSettings")
        (`Character.PlayAnimMontage` (`self.NewVar_0_0`) "/Game/Assets/AIBehaviorToolkit/Assets/Mannequin/Animations/AM_FireShotgun.AM_FireShotgun" 1.0 "spine_01")
        (`GameplayStatics.SpawnEmitterAtLocation` "/Game/Assets/FPS_Weapons_Pack/Effects/ParticlesSystems/Weapons/Rem/P_Rem_Barrel_Smoke.P_Rem_Barrel_Smoke" (`SceneComponent.K2_GetComponentLocation` _sphere) (`SceneComponent.K2_GetComponentRotation` _sphere))
        (`self.Trace` 2000.0)
        (for _ (range 6)
          (set `self.ProjectileTransform` (`KismetMathLibrary.MakeTransform` (`KismetMathLibrary.MakeVector` _returnvalue_x _returnvalue_y _returnvalue_z) (`KismetMathLibrary.ComposeRotators` _projectiletransform_rotation (`KismetMathLibrary.MakeRotator` 0.0 0.0 (`KismetMathLibrary.RandomFloatInRange` 2.0 5.0))) (0.2 0.2 0.2)))
          (bind _returnvalue (`|SpawnActorFromClass` "/Game/Blueprints/Weapons/projectiles/BP_PistolProjectile.BP_PistolProjectile_C" (`self.ProjectileTransform`) "AdjustIfPossibleButAlwaysSpawn" "OverrideRootScale" (`self.GetParentActor`) (`self.GetInstigator`)))
          (set `/Game/Blueprints/Weapons/projectiles/BP_ProjectileBase.DeathEnumVar` "NewEnumerator3" _returnvalue)
          (set `/Game/Blueprints/Weapons/projectiles/BP_PistolProjectile.DamageDecrease` 0.0 _returnvalue)
          (set `/Game/Blueprints/Weapons/projectiles/BP_ProjectileBase.LifeTime` 4.0 _returnvalue)
          (set `/Game/Blueprints/Weapons/projectiles/BP_ProjectileBase.DamageVelocity` 1200.0 _returnvalue))
        (`KismetSystemLibrary.Delay` 0.1)
        (set `/Game/Blueprints/BaseCharacterClass.StopChangingCustomTime` false (`self.NewVar_0_0`))
        (`/Engine/EditorBlueprintResources/StandardMacros.IsValid` _player
          (:`Is Valid`
            (set `/Game/Blueprints/PlayersCharacter.ChangeTimeDilationInPlayersClass` true _player)
            (set `/Game/Blueprints/PlayersCharacter.ShowAmmo` true _player))
          (:`Is Not Valid`
            _))
        (`KismetSystemLibrary.Delay` 0.7)
        (if (not (`/Game/Blueprints/BaseCharacterClass.Dead` (`self.NewVar_0_0`)))
          (`GameplayStatics.PlaySoundAtLocation` "/Game/Assets/Sounds/Effects/Weapons/ShotgunReload.ShotgunReload" _returnvalue_location_2 (struct) (`/Game/Blueprints/Dsm_GameInstance.Volume` (`self.GameInstance`)) 1.0 0.0 "/Game/Blueprints/SoundBlueprints/SoundAttenuationSettings.SoundAttenuationSettings")
          (`GameplayStatics.SpawnEmitterAtLocation` "/Game/Assets/FPS_Weapons_Pack/Effects/ParticlesSystems/Weapons/AP5/P_AP5_Shells.P_AP5_Shells" (`SceneComponent.K2_GetComponentLocation` (`self.Sphere1`))))
        (`KismetSystemLibrary.Delay` (- (`self.AttackRate`) 0.8))
        (set `self.StopRotate` false)
        (`self.ShotEventDispatcher`)
        (goto _label :!via `Reset`)
        (else
          (`KismetSystemLibrary.Delay` 0.4)
          (`|ExecutionSequence`
            (:`then_0`
              (goto _label_2 :!via `Reset`))
            (:`then_1`
              (`/Engine/EditorBlueprintResources/StandardMacros.DoOnce` false :!label _label_2
                (:`Completed`
                  (`GameplayStatics.PlaySoundAtLocation` "/Game/Assets/Sounds/Effects/EmptyPistol__WAV_.EmptyPistol__WAV_" (`self.K2_GetActorLocation` (`self.NewVar_0_0`)) (struct) (`/Game/Blueprints/Dsm_GameInstance.Volume` (`self.GameInstance`)) 1.0 0.0 "/Game/Blueprints/SoundBlueprints/SoundAttenuationSettings.SoundAttenuationSettings")
                  (goto _label :!via `Reset`))))))))))

(fn `UserConstructionScript`
  (`parent.UserConstructionScript`)
  (set `self.HitEnemy` false)
  (set `self.Destructible` "/Game/Assets/FPS_Weapons_Pack/Weapons/Meshes/Rem870/SM_Rem870_DM.SM_Rem870_DM")
  (set `self.ImageWeapon` "/Game/Assets/Images/ShotgunIcon.ShotgunIcon"))