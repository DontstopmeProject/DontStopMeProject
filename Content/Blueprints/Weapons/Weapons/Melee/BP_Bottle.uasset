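; Breakable bottle melee weapon, held as a child actor by a character, that can also be thrown.
; Attacks alternate two montages, and capsule overlaps skip same-tag humans, then deal damage or trigger a block.
; Either outcome damages the bottle itself, breaking it, spawning blood on humans and making the owner discard it.
; Thrown impacts also shatter it, and a separate finisher pauses movement for a timed stab animation.
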(event `self.ReceiveAnyDamage`
  (params (Damage :type "Float (single-precision)") (DamageType :type "DamageType Object Reference") (InstigatedBy :type "Controller Object Reference") (DamageCauser :type "Actor Object Reference"))
  (bind _asplayers_character (cast `/Game/Blueprints/PlayersCharacter` (`self.GetParentActor`))
    (:`then`
      (bind _returnvalue (`|CreateWidget` "/Game/Blueprints/Widgets/BaseWidgets/DamageWidget.DamageWidget_C"))
      (bind _output_get (set `/Game/Blueprints/BaseCharacterClass.DamgeHud` _returnvalue _asplayers_character))
      (`UserWidget.AddToViewport` _output_get 0))
    (:`CastFailed`
      _))
  (`self.EventDestroyedMesh` :!label _label)
  (set `self.Destroyed` true :!label _label_2)
  (bind _asplayers_character_2 (cast `/Game/Blueprints/PlayersCharacter` (`self.GetParentActor`)))
  (`/Game/Blueprints/PlayersCharacter.EventSetHud` _asplayers_character_2))

(event `EventHitHuman`
  (`self.EventDestroyedMesh` :!label _label_3)
  (if (not (`self.ActorHasTag` (`self.HitActor`) (`|GetArrayItem` (`self.Tags`) 2)))
    (`GameplayStatics.ApplyDamage` (`self.HitActor`) 49.0 null self)
    (goto _label_2)))

(event `EventHitThrowedHuman`
  (if (not (`self.ActorHasTag` (`self.HitActor`) (`|GetArrayItem` (`self.Tags`) 2)))
    (goto _label_3)))

(event `self.Capsule.OnComponentBeginOverlap`
  (params (OverlappedComponent :type "PrimitiveComponent Object Reference") (OtherActor :type "Actor Object Reference") (OtherComp :type "PrimitiveComponent Object Reference") (OtherBodyIndex :type Integer) (bFromSweep :type Boolean) (SweepResult :type "HitResult Structure (by ref)"))
  (bind _hitactor (`self.HitActor`))
  (bind _returnvalue_location (`KismetMathLibrary.BreakTransform` (`SceneComponent.K2_GetComponentToWorld` (`self.HitComponent`))))
  (if (`/Game/Blueprints/BaseCharacterClass.Dead` (`self.NewVar_0_0`))
    _
    (elif (== OtherComp (`self.ProjectileCapsule`))
      _
      (elif (not (and (`self.ActorHasTag` OtherActor (`|GetArrayItem` (`Actor.Tags` (`self.GetParentActor`)) 2)) (`self.ActorHasTag` OtherActor "human")))
        (set `self.HitBone` SweepResult_HitBoneName)
        (set `self.HitComponent` OtherComp)
        (bind _output_get (set `self.HitActor` OtherActor))
        (`self.ShakePlayersCamera` null 1.0)
        (`self.ContactDispatcher`)
        (bind _asbase_character_class (cast `/Game/Blueprints/BaseCharacterClass` _output_get)
          (:`then`
            (if (`self.Blocked`)
              (set `self.ResetAttack` true)
              (`/Game/Blueprints/PlayersComponents/BlockOverlapComponent.EventBlockOverlap` (`self.BlockOverlapComponent`))
              (`GameplayStatics.PlaySoundAtLocation` "/Game/Assets/Sounds/Effects/MGS_Zvuk_obnaruzheniya__mp3cut_net_.MGS_Zvuk_obnaruzheniya__mp3cut_net_" (`self.K2_GetActorLocation` (`self.NewVar_0_0`)) (struct) 0.8 1.0 0.0 "/Game/Blueprints/SoundBlueprints/SoundAttenuationSettings.SoundAttenuationSettings")
              (else
                (set `/Game/Blueprints/BaseCharacterClass.DeathEnumVar` "NewEnumerator4" _asbase_character_class)
                (set `/Game/Blueprints/BaseCharacterClass.CounterI` 1 _asbase_character_class)
                (switch `int` (`self.I`)
                  (:`0`
                    (set `/Game/Blueprints/BaseCharacterClass.Hit_I` 0 _asbase_character_class))
                  (:`1`
                    (set `/Game/Blueprints/BaseCharacterClass.Hit_I` 2 _asbase_character_class)))
                (`GameplayStatics.ApplyDamage` _output_get 60.0 (`Pawn.GetController` (`Actor.Instigator` (`self.GetParentActor`))) self :!label _label_4))))
          (:`CastFailed`
            (goto _label_4)))
        (`GameplayStatics.ApplyDamage` self 100.0 null self)
        (`ActorComponent.K2_DestroyComponent` (`self.Capsule`))
        (`PrimitiveComponent.SetCollisionEnabled` (`self.Sphere`) "NoCollision")
        (if (`self.ActorHasTag` (`self.HitActor`) "human")
          (`GameplayStatics.PlaySoundAtLocation` "/Game/Assets/Sounds/Effects/Skull__FinalArms_.Skull__FinalArms_" (`self.K2_GetActorLocation` (`self.GetParentActor`)) (struct) 1.0 1.0 0.0 "/Game/Blueprints/SoundBlueprints/SoundAttenuationSettings.SoundAttenuationSettings")
          (`GameplayStatics.SpawnEmitterAtLocation` "/Game/Assets/FPS_Weapons_Pack/Effects/ParticlesSystems/Impacts/Human/P_Blood_Impact.P_Blood_Impact" (+ (+ (* (`self.GetActorForwardVector` _hitactor) 8.0) (+ _returnvalue_location (0.0 0.0 145.0))) (* (`self.GetActorRightVector` _hitactor) 2.0)))
          (`PrimitiveComponent.AddImpulse` (`self.HitComponent`) (* (`self.GetActorForwardVector` (`self.NewVar_0_0`)) 1000.0) "spine_02" true)
          (set `self.Destroy` true))
        (`KismetArrayLibrary.Array_Add` (`self.Tags`) "broken")
        (`KismetSystemLibrary.Delay` 0.3)
        (`/Game/Blueprints/BaseCharacterClass.EventThrowAway` (`self.NewVar_0_0`))))))

(event `EventHitSmth`
  (if (`self.Throw`)
    (goto _label)))

(event `EventFinish`
  (bind _player (`self.player`))
  (bind _newvar_0_0 (`self.NewVar_0_0`))
  (bind _newvar_0_0_2 (`self.NewVar_0_0`))
  (bind _player_2 (`self.player`))
  (bind _mesh (`Character.Mesh` _newvar_0_0_2))
  (if (`/Game/Blueprints/BaseCharacterClass.CanFinish` (`self.NewVar_0_0`))
    (`/Engine/EditorBlueprintResources/StandardMacros.DoOnce` false :!label _label_5
      (:`Completed`
        (if (`self.ActorHasTag` (`self.NewVar_0_0`) "player")
          (`self.DisableInput` (`GameplayStatics.GetPlayerController` 0)))
        (`/Engine/EditorBlueprintResources/StandardMacros.IsValid` _player_2
          (:`Is Valid`
            (set `/Game/Blueprints/PlayersCharacter.ChangeTimeDilationInPlayersClass` false _player_2))
          (:`Is Not Valid`
            _))
        (`GameplayStatics.SetGlobalTimeDilation` 1.0)
        (`ActorComponent.Deactivate` (`Character.CharacterMovement` (`self.NewVar_0_0`)))
        (`/Game/Blueprints/BaseCharacterClass.FinishDispatcher` (`self.NewVar_0_0`))
        (`self.ShotEventDispatcher`)
        (`SkeletalMeshComponent.PlayAnimation` (`Character.Mesh` _newvar_0_0) null false)
        (set `/Game/Blueprints/BaseCharacterClass.CanFinish` false _newvar_0_0)
        (`KismetSystemLibrary.Delay` 0.3)
        (`GameplayStatics.PlaySoundAtLocation` "/Game/Assets/AIBehaviorToolkit/Assets/Sounds/Sword/S_Sword_Stab01.S_Sword_Stab01" (`self.K2_GetActorLocation` (`self.NewVar_0_0`)) (struct) (`/Game/Blueprints/Dsm_GameInstance.Volume` (`self.GameInstance`)) 1.0 0.0 "/Game/Blueprints/SoundBlueprints/SoundAttenuationSettings.SoundAttenuationSettings")
        (`KismetSystemLibrary.Delay` 1.0)
        (`self.ShotEventDispatcher`)
        (`/Game/Blueprints/BaseCharacterClass.FinishDispatcher` (`self.NewVar_0_0`))
        (`KismetSystemLibrary.Delay` 0.2)
        (if (`self.ActorHasTag` (`self.NewVar_0_0`) "player")
          (`self.EnableInput` (`GameplayStatics.GetPlayerController` 0)))
        (`ActorComponent.Activate` (`Character.CharacterMovement` _newvar_0_0_2) false)
        (`PrimitiveComponent.SetCollisionEnabled` (`self.StaticMesh`) "NoCollision")
        (`PrimitiveComponent.SetCollisionEnabled` (`self.Capsule`) "NoCollision")
        (`/Engine/EditorBlueprintResources/StandardMacros.IsValid` _player
          (:`Is Valid`
            (set `/Game/Blueprints/PlayersCharacter.ChangeTimeDilationInPlayersClass` true _player))
          (:`Is Not Valid`
            _))
        (`SkeletalMeshComponent.SetAnimationMode` _mesh "AnimationBlueprint")
        (`SkeletalMeshComponent.SetAnimInstanceClass` _mesh "/Game/Assets/AnimStarterPack/Base_UE4ASP_HeroTPP_AnimBlueprint.Base_UE4ASP_HeroTPP_AnimBlueprint_C")
        (goto _label_5 :!via `Reset`)))))

(event `EventToggleHitCollisions`
  (params (EnableCollision :type Boolean))
  (`self.ToggleHitCollisions` (`|MakeArray` (`self.Capsule`) :!type "PrimitiveComponent Object Reference") EnableCollision))

(event `self.ReceiveBeginPlay`
  (bind _returnvalue (`self.GetParentActor`))
  (bind _sphere (`/Game/Blueprints/BaseCharacterClass.Sphere` (`self.LastOwnerActor`)))
  (`parent.ReceiveBeginPlay`)
  (`self.EventSpawned` 0.6 -1)
  (if (`self.Throw`)
    (`SceneComponent.K2_SetWorldLocationAndRotation` (`self.StaticMesh`) (`SceneComponent.K2_GetComponentLocation` _sphere) (`KismetMathLibrary.Conv_VectorToRotator` (`SceneComponent.GetForwardVector` _sphere)) false false))
  (bind _asdsm_game_instance (cast `/Game/Blueprints/Dsm_GameInstance` (`GameplayStatics.GetGameInstance`)))
  (set `self.GameInstance` _asdsm_game_instance)
  (`/Engine/EditorBlueprintResources/StandardMacros.IsValid` _returnvalue
    (:`Is Valid`
      (bind _asbase_character_class (cast `/Game/Blueprints/BaseCharacterClass` _returnvalue))
      (set `self.NewVar_0_0` _asbase_character_class)
      (set `/Game/Blueprints/BaseCharacterClass.Hit_I` (`self.I`) _asbase_character_class)
      (if (`self.ActorHasTag` (`self.GetParentActor`) "player")
        (bind _asplayers_character (cast `/Game/Blueprints/PlayersCharacter` (`self.NewVar_0_0`)))
        (bind _output_get (set `self.Player` _asplayers_character)))
      (`KismetSystemLibrary.Delay` 0.02)
      (if (`self.LeftHandAttack`)
        (set `self.I` 1)
        (else
          (set `self.I` 0)))
      (set `self.LeftHandAttack` false))))

(event `EventPunched`
  (`PrimitiveComponent.SetCollisionEnabled` (`self.Sphere`) "NoCollision"))

(event `self.ReceiveTick`
  (params (DeltaSeconds :type "Float (single-precision)"))
  (bind _bloodemitter (`self.BloodEmitter`))
  (bind _newvar_0_0 (`self.NewVar_0_0`))
  (`parent.ReceiveTick` DeltaSeconds)
  (`self.EventTogglePhysics`)
  (`/Engine/EditorBlueprintResources/StandardMacros.IsValid` _newvar_0_0
    (:`Is Valid`
      (`SceneComponent.K2_SetWorldRotation` (`self.Arrow`) (`SceneComponent.K2_GetComponentRotation` (`Character.Mesh` _newvar_0_0)) false false)
      (`/Engine/EditorBlueprintResources/StandardMacros.IsValid` _bloodemitter
        (:`Is Valid`
          (set `ParticleSystemComponent.CustomTimeDilation` (`Actor.CustomTimeDilation` (`self.GetParentActor`)) _bloodemitter))))))

(event `self.EventBlock`
  (if (`self.ResetAttack`)
    (`self.ToggleGlobalTimeDilation` false)
    (`Character.PlayAnimMontage` (`self.NewVar_0_0`) "/Game/Assets/AIBehaviorToolkit/Assets/Mannequin/Animations/AM_BlockArms.AM_BlockArms" 1.0 "spine_02")))

(event `EventBaseAttack`
  (bind _newvar_0_0 (`self.NewVar_0_0`))
  (bind _newvar_0_0_2 (`self.NewVar_0_0`))
  ;[1 1 1] attack
  (if (not (`/Game/Blueprints/BaseCharacterClass.Dead` _newvar_0_0_2))
    (if (`/Game/Blueprints/BaseCharacterClass.Blocked` _newvar_0_0_2)
      (set `self.ResetAttack` true))
    (if (`self.ResetAttack`)
      (if (not (`self.StopAttack`))
        (set `self.ResetAttack` false)
        (set `self.HitActor` null)
        (`self.TraceForShield`)
        (set `self.Blocked` false)
        (`self.ToggleGlobalTimeDilation` false)
        (`self.Trace` 700.0 "NewEnumerator1")
        (switch `int` (`self.I`)
          (:`0`
            (`Character.PlayAnimMontage` _newvar_0_0 "/Game/Assets/AIBehaviorToolkit/Assets/Mannequin/Animations/AM_Attack2.AM_Attack2" 1.0 "spine_02")
            (`/Engine/EditorBlueprintResources/StandardMacros.IncrementInt` (`self.I`)))
          (:`1`
            (`Character.PlayAnimMontage` _newvar_0_0 "/Game/Assets/AIBehaviorToolkit/Assets/Mannequin/Animations/AM_Attack1.AM_Attack1" 1.0 "spine_02")
            (set `self.I` 0)))
        (else
          (set `self.ResetAttack` true))))))

(event `self.ProjectileCapsule.OnComponentBeginOverlap`
  (params (OverlappedComponent :type "PrimitiveComponent Object Reference") (OtherActor :type "Actor Object Reference") (OtherComp :type "PrimitiveComponent Object Reference") (OtherBodyIndex :type Integer) (bFromSweep :type Boolean) (SweepResult :type "HitResult Structure (by ref)"))
  (if (not (== OtherActor self))
    (`/Engine/EditorBlueprintResources/StandardMacros.DoOnce` false
      (:`Completed`
        (`self.EventDestroyedMesh`)))))

(fn `UserConstructionScript`
  (`parent.UserConstructionScript`))