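; Melee wrench weapon, built on a parent weapon class, that can be swung or thrown at characters.
; Attacks alternate two montages, and capsule overlaps either hit a block or deal damage, setting the victim's hit reaction by swing and adding sounds, camera shake, blood and impulse.
; Thrown hits damage characters once, and both thrown and human melee hits also damage the wrench itself.
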(event `EventHitSmth`
  (`PrimitiveComponent.SetCollisionResponseToChannel` (`self.Capsule`) "ECC_GameTraceChannel5" "ECR_Ignore"))

(event `EventHitThrowedHuman`
  (if (not (`self.ActorHasTag` (`self.HitActor`) (`|GetArrayItem` (`self.Tags`) 1)))
    (`/Engine/EditorBlueprintResources/StandardMacros.DoOnce` false
      (:`Completed`
        (bind _asbase_character_class (cast `/Game/Blueprints/BaseCharacterClass` (`self.HitActor`)))
        (`GameplayStatics.ApplyDamage` _asbase_character_class 49.0 null self)
        (`PrimitiveComponent.SetCollisionResponseToChannel` (`self.StaticMesh`) "ECC_GameTraceChannel4" "ECR_Ignore")
        (`self.TraceForShield`)
        (`PrimitiveComponent.SetCollisionResponseToChannel` (`self.StaticMesh`) "ECC_GameTraceChannel5" "ECR_Ignore")
        (`GameplayStatics.PlaySoundAtLocation` null (`self.K2_GetActorLocation`) (struct) (`/Game/Blueprints/Dsm_GameInstance.Volume` (`self.GameInstance`)) 1.0 0.0 "/Game/Blueprints/SoundBlueprints/SoundAttenuationSettings.SoundAttenuationSettings")
        (`GameplayStatics.ApplyDamage` self 60.0 null self)))))

(event `self.Capsule.OnComponentBeginOverlap`
  (params (OverlappedComponent :type "PrimitiveComponent Object Reference") (OtherActor :type "Actor Object Reference") (OtherComp :type "PrimitiveComponent Object Reference") (OtherBodyIndex :type Integer) (bFromSweep :type Boolean) (SweepResult :type "HitResult Structure (by ref)"))
  (bind _newvar_0_0 (`self.NewVar_0_0`))
  (bind _hitactor (`self.HitActor`))
  (bind _returnvalue (`self.K2_GetActorLocation` (`self.NewVar_0_0`)))
  (bind _returnvalue_location (`KismetMathLibrary.BreakTransform` (`SceneComponent.K2_GetComponentToWorld` (`self.HitComponent`))))
  (if (or (`/Game/Blueprints/BaseCharacterClass.Dead` _newvar_0_0) (`/Game/Blueprints/BaseCharacterClass.Stuned` _newvar_0_0) (`/Game/Blueprints/BaseCharacterClass.Kicked` _newvar_0_0))
    _
    (elif (not (`self.ActorHasTag` OtherActor (`|GetArrayItem` (`Actor.Tags` (`self.GetParentActor`)) 2)))
      (set `self.NewVar_2` true)
      (if (not (== (`self.HitActor`) OtherActor))
        (set `self.HitBone` SweepResult_HitBoneName)
        (set `self.HitComponent` OtherComp)
        (bind _output_get (set `self.HitActor` OtherActor))
        (bind _asbase_character_class (cast `/Game/Blueprints/BaseCharacterClass` (`self.HitActor`))
          (:`then`
            (if (`self.Blocked`)
              (set `self.ResetAttack` true)
              (`GameplayStatics.PlaySoundAtLocation` "/Game/Assets/Sounds/Effects/MGS_Zvuk_obnaruzheniya__mp3cut_net_.MGS_Zvuk_obnaruzheniya__mp3cut_net_" (`self.K2_GetActorLocation` (`self.NewVar_0_0`)) (struct) 0.2 1.0 0.3 "/Game/Blueprints/SoundBlueprints/SoundAttenuationSettings.SoundAttenuationSettings")
              (`/Game/Blueprints/PlayersComponents/BlockOverlapComponent.EventBlockOverlap` (`self.BlockOverlapComponent`))
              (else
                (set `/Game/Blueprints/BaseCharacterClass.CounterI` 1 _asbase_character_class)
                (switch `int` (`self.I`)
                  (:`Default`
                    _)
                  (:`0`
                    (set `/Game/Blueprints/BaseCharacterClass.Hit_I` 2 _asbase_character_class)
                    (set `/Game/Blueprints/BaseCharacterClass.DeathEnumVar` "NewEnumerator4" _asbase_character_class :!label _label))
                  (:`1`
                    (set `/Game/Blueprints/BaseCharacterClass.Hit_I` 0 _asbase_character_class)
                    (goto _label)))
                (`self.ContactDispatcher` :!label _label_2)
                (bind _success (`self.ShakePlayersCamera` null 1.0))
                (`GameplayStatics.ApplyDamage` _output_get (`self.Damage`) null (`self.GetParentActor`))
                (if (`self.ActorHasTag` (`self.HitActor`) "human")
                  (bind _asbase_character_class_2 (cast `/Game/Blueprints/BaseCharacterClass` (`self.HitActor`))
                    (:`then`
                      (if (`/Game/Blueprints/BaseCharacterClass.Dead` _asbase_character_class_2)
                        (`GameplayStatics.PlaySoundAtLocation` null _returnvalue (struct) 1.0 1.0 0.0 "/Game/Blueprints/SoundBlueprints/SoundAttenuationSettings.SoundAttenuationSettings")
                        (`KismetSystemLibrary.Delay` 0.01)
                        (`GameplayStatics.PlaySoundAtLocation` "/Game/Assets/Sounds/Effects/Skull__Final_.Skull__Final_" _returnvalue (struct) 1.0 1.0 0.05 "/Game/Blueprints/SoundBlueprints/SoundAttenuationSettings.SoundAttenuationSettings")
                        (else
                          (`GameplayStatics.PlaySoundAtLocation` null _returnvalue (struct) 1.0 1.0 0.0 "/Game/Blueprints/SoundBlueprints/SoundAttenuationSettings.SoundAttenuationSettings" :!label _label_3))))
                    (:`CastFailed`
                      (goto _label_3)))
                  (`GameplayStatics.SpawnEmitterAtLocation` "/Game/Assets/FXVillesBloodVFXPack/Particles/PS_StyleBlood_Burst_02.PS_StyleBlood_Burst_02" (+ (+ (* (`self.GetActorForwardVector` _hitactor) 8.0) (+ _returnvalue_location (0.0 0.0 145.0))) (* (`self.GetActorRightVector` _hitactor) 2.0)) (struct :`Pitch` 40.0))
                  (`PrimitiveComponent.AddImpulse` (`self.HitComponent`) (* (`self.GetActorForwardVector` (`self.NewVar_0_0`)) 1000.0) "spine_02" true)
                  (`GameplayStatics.ApplyDamage` self 25.0 null self)))))
          (:`CastFailed`
            (goto _label_2)))))))

(event `self.EventBlock`
  (if (`self.ResetAttack`)
    (`self.ToggleGlobalTimeDilation` false)
    (`Character.PlayAnimMontage` (`self.NewVar_0_0`) "/Game/Assets/AIBehaviorToolkit/Assets/Mannequin/Animations/AM_BlockArms.AM_BlockArms" 1.0 "spine_02")))

(event `EventPunched`
  (`PrimitiveComponent.SetCollisionEnabled` (`self.Sphere`) "NoCollision"))

(event `self.ReceiveBeginPlay`
  (bind _returnvalue (`self.GetParentActor`))
  (bind _sphere (`/Game/Blueprints/BaseCharacterClass.Sphere` (`self.LastOwnerActor`)))
  (`parent.ReceiveBeginPlay`)
  (`self.EventSpawned` 0.62 -1)
  (`SceneComponent.SetVisibility` (`self.Capsule`) false false)
  (bind _asdsm_game_instance (cast `/Game/Blueprints/Dsm_GameInstance` (`GameplayStatics.GetGameInstance`)))
  (set `self.GameInstance` _asdsm_game_instance)
  (`/Engine/EditorBlueprintResources/StandardMacros.IsValid` _returnvalue
    (:`Is Valid`
      (bind _asbase_character_class (cast `/Game/Blueprints/BaseCharacterClass` _returnvalue))
      (set `self.NewVar_0_0` _asbase_character_class)
      (if (`self.Throw`)
        (`SceneComponent.K2_SetWorldLocationAndRotation` (`self.StaticMesh`) (`SceneComponent.K2_GetComponentLocation` _sphere) (`KismetMathLibrary.Conv_VectorToRotator` (`SceneComponent.GetForwardVector` _sphere)) false false))
      (if (`self.ActorHasTag` (`self.GetParentActor`) "player")
        _
        (else
          _))
      (bind _asplayers_character (cast `/Game/Blueprints/PlayersCharacter` (`self.NewVar_0_0`))
        (:`then`
          (bind _output_get (set `self.Player` _asplayers_character)))
        (:`CastFailed`
          _))
      (`KismetSystemLibrary.Delay` 0.02)
      (if (`self.LeftHandAttack`)
        (set `self.I` 0)
        (else
          (set `self.I` 1))))))

(event `EventToggleHitCollisions`
  (params (EnableCollision :type Boolean))
  (`self.ToggleHitCollisions` (`|MakeArray` (`self.Capsule`) :!type "PrimitiveComponent Object Reference") EnableCollision))

(event `self.ReceiveTick`
  (params (DeltaSeconds :type "Float (single-precision)"))
  (bind _bloodemitter (`self.BloodEmitter`))
  (bind _newvar_0_0 (`self.NewVar_0_0`))
  (`parent.ReceiveTick` DeltaSeconds)
  (`self.EventTogglePhysics`)
  (`/Engine/EditorBlueprintResources/StandardMacros.IsValid` _newvar_0_0
    (:`Is Valid`
      (if (`/Game/Blueprints/BaseCharacterClass.CanAttack` (`self.NewVar_0_0`))
        (`SceneComponent.K2_SetWorldRotation` (`self.Arrow`) (`KismetMathLibrary.Conv_VectorToRotator` (`KismetMathLibrary.GetRightVector` (`SceneComponent.K2_GetComponentRotation` (`Character.Mesh` _newvar_0_0)))) false false)
        (`/Engine/EditorBlueprintResources/StandardMacros.IsValid` _bloodemitter
          (:`Is Valid`
            (set `ParticleSystemComponent.CustomTimeDilation` (`Actor.CustomTimeDilation` (`self.GetParentActor`)) _bloodemitter)))))))

(event `EventBaseAttack`
  (bind _newvar_0_0 (`self.NewVar_0_0`))
  ;[1 1 1] attack
  (if (`/Game/Blueprints/BaseCharacterClass.Dead` (`self.NewVar_0_0`))
    _
    (elif (`self.ResetAttack`)
      (if (not (`self.StopAttack`))
        (set `self.ResetAttack` false)
        (set `self.HitActor` null)
        (`self.TraceForShield`)
        (`self.ToggleGlobalTimeDilation` false)
        (`self.Trace` 700.0 "NewEnumerator1")
        (switch `int` (`self.I`)
          (:`0`
            (`Character.PlayAnimMontage` _newvar_0_0 "/Game/Assets/AIBehaviorToolkit/Assets/Mannequin/Animations/AM_Attack1.AM_Attack1" 1.0 "spine_02")
            (`/Engine/EditorBlueprintResources/StandardMacros.IncrementInt` (`self.I`)))
          (:`1`
            (`Character.PlayAnimMontage` _newvar_0_0 "/Game/Assets/AIBehaviorToolkit/Assets/Mannequin/Animations/AM_Attack2.AM_Attack2" 1.0 "spine_02")
            (set `self.I` 0)))
        (else
          (set `self.ResetAttack` true))))))

(fn `UserConstructionScript`
  (`parent.UserConstructionScript`)
  (set `self.HitEnemy` false)
  (set `self.Destructible` null)
  (set `self.ImageWeapon` "/Game/Assets/Images/Bate.Bate"))