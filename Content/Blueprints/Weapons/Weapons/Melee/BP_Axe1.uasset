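; BP_Axe1 is a melee axe weapon Blueprint that removes itself when the game's level index changes.
; On BeginPlay it runs the parent logic, caches the Dsm_GameInstance and records its LevelsIndex as the spawn level.
; Tick polls that index and destroys the actor once it differs from the recorded value.
; The construction script runs the parent's version and clears the HitEnemy flag.
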(event `self.ReceiveBeginPlay`
  (`parent.ReceiveBeginPlay`)
  (bind _asdsm_game_instance (cast `/Game/Blueprints/Dsm_GameInstance` (`GameplayStatics.GetGameInstance`)))
  (bind _output_get (set `self.GameInstance` _asdsm_game_instance))
  (set `self.SpawnedLevelIndex` (`/Game/Blueprints/Dsm_GameInstance.LevelsIndex` _output_get)))

(event `self.ReceiveTick`
  (params (DeltaSeconds :type "Float (single-precision)"))
  (if (!= (`/Game/Blueprints/Dsm_GameInstance.LevelsIndex` (`self.GameInstance`)) (`self.SpawnedLevelIndex`))
    (`self.K2_DestroyActor`)))

(fn `UserConstructionScript`
  (`parent.UserConstructionScript`)
  (set `self.HitEnemy` false))