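; BP_Chair is a melee weapon child Blueprint for a chair that swings in two alternating heavy attacks.
; It disables its environment-blocking capsule collision when it has a parent actor, and removes the capsule when the destroyed dispatcher fires.
; The attack checks death, block and reset flags, then runs inherited shield and hit traces, turns off global time dilation, and plays left or right downswing montages.
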(event `self.ReceiveBeginPlay`
  (`parent.ReceiveBeginPlay`)
  (add `self.DestroyedtDispatcher` (delegate `EventDestroyed`))
  (`/Engine/EditorBlueprintResources/StandardMacros.IsValid` (`self.GetParentActor`)
    (:`Is Valid`
      (`PrimitiveComponent.SetCollisionEnabled` (`self.BlockEnvCapsule`) "NoCollision"))))

(event `EventDestroyed`
  (`ActorComponent.K2_DestroyComponent` (`self.BlockEnvCapsule`)))

(event `EventBaseAttack`
  (bind _newvar_0_0 (`self.NewVar_0_0`))
  (bind _newvar_0_0_2 (`self.NewVar_0_0`))
  ;[1 1 1] attack
  (if (not (`/Game/Blueprints/BaseCharacterClass.Dead` _newvar_0_0))
    (if (`/Game/Blueprints/BaseCharacterClass.Blocked` _newvar_0_0)
      (set `self.ResetAttack` true))
    (if (`self.ResetAttack`)
      (if (not (`self.StopAttack`))
        (set `self.ResetAttack` false)
        (set `self.HitActor` null)
        (`self.TraceForShield`)
        (`self.ToggleGlobalTimeDilation` false)
        (`self.Trace` 700.0 "NewEnumerator1")
        (switch `int` (`self.I`)
          (:`0`
            (`Character.PlayAnimMontage` _newvar_0_0_2 "/Game/Assets/MeleeAnimSet/AM_Attack_Move_strong_Ldown_1.AM_Attack_Move_strong_Ldown_1" 1.4 "spine_02")
            (`/Engine/EditorBlueprintResources/StandardMacros.IncrementInt` (`self.I`)))
          (:`1`
            (`Character.PlayAnimMontage` _newvar_0_0_2 "/Game/Assets/MeleeAnimSet/AM_Attack_Move_strong_Rdown_1.AM_Attack_Move_strong_Rdown_1" 1.5 "spine_02")
            (set `self.I` 0)))
        (else
          (set `self.ResetAttack` true))))))

(fn `UserConstructionScript`
  (`parent.UserConstructionScript`))