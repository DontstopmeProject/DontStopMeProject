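; Fire extinguisher melee weapon, built on the weapon base, that can also be thrown and explodes when destroyed.
; Attacks alternate two montages, while capsule overlaps handle blocks, damage, blood and impulses, damaging the extinguisher on human hits.
; Thrown impacts trigger destruction directly, and explosion-capsule contacts apply self-damage.
; Destruction swaps in a destructible mesh, then stuns nearby characters, damages props and environment weapons, and fires radial force, particles and camera shake.
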(event `EventHitSmth`
  (if (`self.Throw`)
    (`/Engine/EditorBlueprintResources/StandardMacros.DoOnce` false :!label _label
      (:`Completed`
        (`self.EventDestroyedMesh`)))))

(event `EventHitThrowedHuman`
  (if (not (`self.ActorHasTag` (`self.HitActor`) (`|GetArrayItem` (`self.Tags`) 1)))
    (goto _label)))

(event `self.Capsule.OnComponentBeginOverlap`
  (params (OverlappedComponent :type "PrimitiveComponent Object Reference") (OtherActor :type "Actor Object Reference") (OtherComp :type "PrimitiveComponent Object Reference") (OtherBodyIndex :type Integer) (bFromSweep :type Boolean) (SweepResult :type "HitResult Structure (by ref)"))
  (bind _newvar_0_0 (`self.NewVar_0_0`))
  (bind _hitactor (`self.HitActor`))
  (bind _returnvalue (`self.K2_GetActorLocation` (`self.NewVar_0_0`)))
  (bind _returnvalue_location (`KismetMathLibrary.BreakTransform` (`SceneComponent.K2_GetComponentToWorld` (`self.HitComponent`))))
  (bind _returnvalue_2 (+ (+ (* (`self.GetActorForwardVector` _hitactor) 8.0) (+ _returnvalue_location (0.0 0.0 145.0))) (* (`self.GetActorRightVector` _hitactor) 2.0)))
  (if (or (`/Game/Blueprints/BaseCharacterClass.Dead` _newvar_0_0) (`/Game/Blueprints/BaseCharacterClass.Stuned` _newvar_0_0) (`/Game/Blueprints/BaseCharacterClass.Kicked` _newvar_0_0))
    _
    (elif (not (`self.ActorHasTag` OtherActor (`|GetArrayItem` (`Actor.Tags` (`self.GetParentActor`)) 2)))
      (set `self.NewVar_2` true)
      (if (not (== (`self.HitActor`) OtherActor))
        (set `self.HitBone` SweepResult_HitBoneName)
        (set `self.HitComponent` OtherComp)
        (bind _output_get (set `self.HitActor` OtherActor))
        (bind _asbase_character_class (cast `/Game/Blueprints/BaseCharacterClass` (`self.HitActor`))
          (:`then`
            (if (`self.Blocked`)
              (set `self.ResetAttack` true)
              (`GameplayStatics.PlaySoundAtLocation` "/Game/Assets/Sounds/Effects/MGS_Zvuk_obnaruzheniya__mp3cut_net_.MGS_Zvuk_obnaruzheniya__mp3cut_net_" (`self.K2_GetActorLocation` (`self.NewVar_0_0`)) (struct) 0.2 1.0 0.3 "/Game/Blueprints/SoundBlueprints/SoundAttenuationSettings.SoundAttenuationSettings")
              (`/Game/Blueprints/PlayersComponents/BlockOverlapComponent.EventBlockOverlap` (`self.BlockOverlapComponent`))
              (else
                (set `/Game/Blueprints/BaseCharacterClass.CounterI` 1 _asbase_character_class)
                (switch `int` (`self.I`)
                  (:`Default`
                    _)
                  (:`0`
                    (set `/Game/Blueprints/BaseCharacterClass.Hit_I` 2 _asbase_character_class)
                    (set `/Game/Blueprints/BaseCharacterClass.DeathEnumVar` "NewEnumerator4" _asbase_character_class :!label _label_2))
                  (:`1`
                    (set `/Game/Blueprints/BaseCharacterClass.Hit_I` 0 _asbase_character_class)
                    (goto _label_2)))
                (`self.ContactDispatcher` :!label _label_3)
                (bind _success (`self.ShakePlayersCamera` null 1.0))
                (`GameplayStatics.ApplyDamage` _output_get (`self.Damage`) null (`self.GetParentActor`))
                (if (`self.ActorHasTag` (`self.HitActor`) "human")
                  (bind _asbase_character_class_2 (cast `/Game/Blueprints/BaseCharacterClass` (`self.HitActor`))
                    (:`then`
                      (if (`/Game/Blueprints/BaseCharacterClass.Dead` _asbase_character_class_2)
                        (`GameplayStatics.PlaySoundAtLocation` null _returnvalue (struct) 1.0 1.0 0.0 "/Game/Blueprints/SoundBlueprints/SoundAttenuationSettings.SoundAttenuationSettings")
                        (`KismetSystemLibrary.Delay` 0.01)
                        (`GameplayStatics.PlaySoundAtLocation` "/Game/Assets/Sounds/Effects/Skull__Final_.Skull__Final_" _returnvalue (struct) 1.0 1.0 0.05 "/Game/Blueprints/SoundBlueprints/SoundAttenuationSettings.SoundAttenuationSettings")
                        (`GameplayStatics.SpawnEmitterAtLocation` "/Game/Assets/FXVillesBloodVFXPack/Particles/PS_StyleBlood_Burst_02.PS_StyleBlood_Burst_02" _returnvalue_2 (struct :`Pitch` 40.0))
                        (`PrimitiveComponent.AddImpulse` (`self.HitComponent`) (* (`self.GetActorForwardVector` (`self.NewVar_0_0`)) 1000.0) "spine_02" true)
                        (`KismetSystemLibrary.Delay` 0.09)
                        (else
                          (`GameplayStatics.PlaySoundAtLocation` null _returnvalue (struct) 1.0 1.0 0.0 "/Game/Blueprints/SoundBlueprints/SoundAttenuationSettings.SoundAttenuationSettings" :!label _label_4)
                          (`GameplayStatics.SpawnEmitterAtLocation` "/Game/Assets/FXVillesBloodVFXPack/Particles/PS_StyleBlood_Burst_02.PS_StyleBlood_Burst_02" _returnvalue_2 (struct :`Pitch` 40.0))
                          (`PrimitiveComponent.AddImpulse` (`self.HitComponent`) (* (`KismetMathLibrary.GetRightVector` (`SceneComponent.K2_GetComponentRotation` (`Character.Mesh` (`self.NewVar_0_0`)))) 2.0) "spine_02" true))))
                    (:`CastFailed`
                      (goto _label_4)))
                  (`GameplayStatics.ApplyDamage` self 25.0 null self)))))
          (:`CastFailed`
            (goto _label_3)))))))

(event `self.EventBlock`
  (if (`self.ResetAttack`)
    (`self.ToggleGlobalTimeDilation` false)
    (`Character.PlayAnimMontage` (`self.NewVar_0_0`) "/Game/Assets/AIBehaviorToolkit/Assets/Mannequin/Animations/AM_BlockArms.AM_BlockArms" 1.0 "spine_02")))

(event `EventExplode`
  (bind _overlappingactors (`PrimitiveComponent.GetOverlappingActors` (`self.ExpSphere`) "/Script/Engine.Character"))
  ;[1 1 1] Explosion
  (`PrimitiveComponent.SetCollisionEnabled` (`self.ExpSphere`) "QueryAndPhysics")
  (for _array_element _overlappingactors
    (bind _asplayers_character (cast `/Game/Blueprints/PlayersCharacter` _array_element)
      (:`then`
        (bind _asweapon_base (cast `/Game/Blueprints/Weapons/Weapons/WeaponBase` (`ChildActorComponent.ChildActor` (`/Game/Blueprints/BaseCharacterClass.PickableItem` _asplayers_character)))
          (:`then`
            (set `/Game/Blueprints/Weapons/Weapons/WeaponBase.ResetAttack` true _asweapon_base))
          (:`CastFailed`
            _)))
      (:`CastFailed`
        _))
    (bind _asbase_character_class (cast `/Game/Blueprints/BaseCharacterClass` _array_element))
    (set `/Game/Blueprints/BaseCharacterClass.CounterI` 2 _asbase_character_class)
    (`/Game/Blueprints/BaseCharacterClass.EventStun` _asbase_character_class))
  (for _array_element_2 _overlappingactors
    (bind _asbase_character_class_2 (cast `/Game/Blueprints/BaseCharacterClass` _array_element_2))
    (set `/Game/Blueprints/BaseCharacterClass.CounterI` 0 _asbase_character_class_2))
  (for _array_element_3 (`PrimitiveComponent.GetOverlappingActors` (`self.ExpSphere`) "/Game/Blueprints/Weapons/Weapons/WeaponBase.WeaponBase_C")
    (bind _asweapon_base_2 (cast `/Game/Blueprints/Weapons/Weapons/WeaponBase` _array_element_3))
    (if (`/Game/Blueprints/Weapons/Weapons/WeaponBase.Enviroment?` _asweapon_base_2)
      (`GameplayStatics.ApplyDamage` _array_element_3 100.0 null self)))
  (for _array_element_4 (`PrimitiveComponent.GetOverlappingActors` (`self.Sphere`) "/Game/Blueprints/Props/Bp_Props.Bp_Props_C")
    (`GameplayStatics.ApplyDamage` _array_element_4 100.0 null self))
  (`ActorComponent.Activate` (`self.RadialForce`) false)
  (`ActorComponent.Activate` (`self.ExpPS`) false)
  (`ActorComponent.K2_DestroyComponent` (`self.ExpSphere`))
  (`ActorComponent.K2_DestroyComponent` (`self.ExpCapsule`))
  (`PlayerCameraManager.PlayCameraShake` :`self` (`GameplayStatics.GetPlayerCameraManager` 0) :`ShakeClass` "/Game/Blueprints/CameraShakes/KillCameraShake.KillCameraShake_C" :`Scale` 5.0))

(event `self.EventDestroyedMesh`
  (bind _staticmesh (`self.StaticMesh`))
  ;[1 1 1] DestroyedMesh
  (bind _asplayers_character (cast `/Game/Blueprints/PlayersCharacter` (`GameplayStatics.GetPlayerCharacter` 0)))
  (if (not (!= (`/Game/Blueprints/BaseCharacterClass.PickableItemVar` _asplayers_character) self))
    (set `/Game/Blueprints/BaseCharacterClass.PickableItemVar` null _asplayers_character))
  (`/Engine/EditorBlueprintResources/StandardMacros.DoOnce` false
    (:`Completed`
      (set `self.Destroy` true)
      (`SceneComponent.SetHiddenInGame` _staticmesh true false)
      (bind _returnvalue (`AddComponent|NODE_AddDestructibleComponent-0` :`bManualAttachment` true :`RelativeTransform` (`SceneComponent.K2_GetComponentToWorld` (`self.StaticMesh`))))
      (`DestructibleComponent.SetDestructibleMesh` _returnvalue (`self.Destructible`))
      (`DestructibleComponent.ApplyRadiusDamage` _returnvalue 100.0 (`SceneComponent.K2_GetComponentLocation` _returnvalue) 100.0 100.0 true)
      (`ActorComponent.K2_DestroyComponent` _staticmesh)
      (`self.EventExplode`)
      (`KismetSystemLibrary.Delay` 3.0)
      (`PrimitiveComponent.SetSimulatePhysics` _returnvalue false))))

(event `self.ExpCapsule.OnComponentBeginOverlap`
  (params (OverlappedComponent :type "PrimitiveComponent Object Reference") (OtherActor :type "Actor Object Reference") (OtherComp :type "PrimitiveComponent Object Reference") (OtherBodyIndex :type Integer) (bFromSweep :type Boolean) (SweepResult :type "HitResult Structure (by ref)"))
  ;[1 1 1] StaticContact
  (`GameplayStatics.ApplyDamage` self 100.0 null OtherActor))

(event `self.ReceiveBeginPlay`
  (bind _returnvalue (`self.GetParentActor`))
  (bind _expcapsule (`self.ExpCapsule`))
  (bind _sphere (`/Game/Blueprints/BaseCharacterClass.Sphere` (`self.LastOwnerActor`)))
  (`parent.ReceiveBeginPlay`)
  (`self.EventSpawned` 0.62 -1)
  (`SceneComponent.SetVisibility` (`self.Capsule`) false false)
  (bind _asdsm_game_instance (cast `/Game/Blueprints/Dsm_GameInstance` (`GameplayStatics.GetGameInstance`)))
  (set `self.GameInstance` _asdsm_game_instance)
  (`/Engine/EditorBlueprintResources/StandardMacros.IsValid` _returnvalue
    (:`Is Valid`
      (`PrimitiveComponent.SetCollisionEnabled` _expcapsule "NoCollision")
      (bind _asbase_character_class (cast `/Game/Blueprints/BaseCharacterClass` _returnvalue))
      (set `self.NewVar_0_0` _asbase_character_class)
      (if (`self.Throw`)
        (`SceneComponent.K2_SetWorldLocationAndRotation` (`self.StaticMesh`) (`SceneComponent.K2_GetComponentLocation` _sphere) (`KismetMathLibrary.Conv_VectorToRotator` (`SceneComponent.GetForwardVector` _sphere)) false false))
      (if (`self.ActorHasTag` (`self.GetParentActor`) "player")
        _
        (else
          _))
      (bind _asplayers_character (cast `/Game/Blueprints/PlayersCharacter` (`self.NewVar_0_0`))
        (:`then`
          (bind _output_get (set `self.Player` _asplayers_character)))
        (:`CastFailed`
          _))
      (`KismetSystemLibrary.Delay` 0.02)
      (if (`self.LeftHandAttack`)
        (set `self.I` 0)
        (else
          (set `self.I` 1))))
    (:`Is Not Valid`
      (`/Engine/EditorBlueprintResources/StandardMacros.IsValid` _expcapsule
        (:`Is Valid`
          (`PrimitiveComponent.SetCollisionEnabled` _expcapsule "QueryAndPhysics"))))))

(event `self.ExpCapsule.OnComponentHit`
  (params (HitComponent :type "PrimitiveComponent Object Reference") (OtherActor :type "Actor Object Reference") (OtherComp :type "PrimitiveComponent Object Reference") (NormalImpulse :type "Vector Structure") (Hit :type "HitResult Structure (by ref)"))
  ;[1 1 1] StaticContact
  (`GameplayStatics.ApplyDamage` self 100.0 null OtherActor))

(event `self.ReceiveTick`
  (params (DeltaSeconds :type "Float (single-precision)"))
  (bind _returnvalue (`GameplayStatics.GetGlobalTimeDilation`))
  (bind _bloodemitter (`self.BloodEmitter`))
  (bind _newvar_0_0 (`self.NewVar_0_0`))
  (bind _expps (`self.ExpPS`))
  (`parent.ReceiveTick` DeltaSeconds)
  (`self.EventTogglePhysics`)
  (`/Engine/EditorBlueprintResources/StandardMacros.IsValid` _newvar_0_0
    (:`Is Valid`
      (if (`/Game/Blueprints/BaseCharacterClass.CanAttack` (`self.NewVar_0_0`))
        (`SceneComponent.K2_SetWorldRotation` (`self.Arrow`) (`KismetMathLibrary.Conv_VectorToRotator` (`KismetMathLibrary.GetRightVector` (`SceneComponent.K2_GetComponentRotation` (`Character.Mesh` _newvar_0_0)))) false false)
        (`/Engine/EditorBlueprintResources/StandardMacros.IsValid` _bloodemitter
          (:`Is Valid`
            (set `ParticleSystemComponent.CustomTimeDilation` (`Actor.CustomTimeDilation` (`self.GetParentActor`)) _bloodemitter)))))
    (:`Is Not Valid`
      (if (< _returnvalue 1.0)
        (set `ParticleSystemComponent.CustomTimeDilation` (/ _returnvalue 15.0) _expps)
        (else
          (set `ParticleSystemComponent.CustomTimeDilation` 1.0 _expps))))))

(event `EventToggleHitCollisions`
  (params (EnableCollision :type Boolean))
  (`self.ToggleHitCollisions` (`|MakeArray` (`self.Capsule`) :!type "PrimitiveComponent Object Reference") EnableCollision))

(event `EventBaseAttack`
  (bind _newvar_0_0 (`self.NewVar_0_0`))
  (bind _newvar_0_0_2 (`self.NewVar_0_0`))
  ;[1 1 1] attack
  (if (`/Game/Blueprints/BaseCharacterClass.Dead` _newvar_0_0)
    (if (`/Game/Blueprints/BaseCharacterClass.Blocked` _newvar_0_0)
      (set `self.ResetAttack` true)))
  (if (`self.ResetAttack`)
    (if (not (`self.StopAttack`))
      (set `self.ResetAttack` false)
      (set `self.HitActor` null)
      (`self.TraceForShield`)
      (`self.ToggleGlobalTimeDilation` false)
      (`self.Trace` 700.0 "NewEnumerator1")
      (switch `int` (`self.I`)
        (:`0`
          (`Character.PlayAnimMontage` _newvar_0_0_2 "/Game/Assets/MeleeAnimSet/AM_Attack_Move_strong_Ldown_1.AM_Attack_Move_strong_Ldown_1" 1.4 "spine_02")
          (`/Engine/EditorBlueprintResources/StandardMacros.IncrementInt` (`self.I`)))
        (:`1`
          (`Character.PlayAnimMontage` _newvar_0_0_2 "/Game/Assets/MeleeAnimSet/AM_Attack_Move_strong_Rdown_1.AM_Attack_Move_strong_Rdown_1" 1.5 "spine_02")
          (set `self.I` 0)))
      (else
        (set `self.ResetAttack` true)))))

(fn `UserConstructionScript`
  (`parent.UserConstructionScript`)
  (set `self.HitEnemy` false)
  (set `self.Destructible` null)
  (set `self.ImageWeapon` "/Game/Assets/Images/Bate.Bate"))