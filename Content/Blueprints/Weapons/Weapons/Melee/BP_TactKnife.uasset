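; Tactical knife melee weapon that extends a parent weapon class, caching its parent actor as the owning character on BeginPlay.
; Its attack event, gated by owner death and reset/stop flags, clears the last hit, checks for shields, switches off global time dilation, emits noise and runs a trace.
; Successive attacks alternate between two swing montages via a counter.
; Construction resets hit state and sets the knife's weapon image.
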(event `self.ReceiveBeginPlay`
  (`parent.ReceiveBeginPlay`)
  (bind _asbase_character_class (cast `/Game/Blueprints/BaseCharacterClass` (`self.GetParentActor`)))
  (set `self.OwnerCharacter` _asbase_character_class))

(event `EventBaseAttack`
  (bind _ownercharacter (`self.OwnerCharacter`))
  (bind _ownercharacter_2 (`self.OwnerCharacter`))
  ;[1 1 1] attack
  (if (`/Game/Blueprints/BaseCharacterClass.Dead` (`self.OwnerCharacter`))
    _
    (elif (`self.ResetAttack`)
      (if (not (`self.StopAttack`))
        (set `self.ResetAttack` false)
        (set `self.HitActor` null)
        (`self.TraceForShield`)
        (`self.ToggleGlobalTimeDilation` false)
        (`self.MakeNoise` _ownercharacter_2 10.0 _ownercharacter_2 (`self.K2_GetActorLocation` _ownercharacter_2) 0.0 "None")
        (`self.Trace` 700.0 "NewEnumerator1")
        (switch `int` (`self.AttackCounter`)
          (:`0`
            (`Character.PlayAnimMontage` _ownercharacter "/Game/Assets/MeleeAnimSet/AM_Attack_Move_med_L_1.AM_Attack_Move_med_L_1" 1.0 "spine_02")
            (`/Engine/EditorBlueprintResources/StandardMacros.IncrementInt` (`self.AttackCounter`)))
          (:`1`
            (`Character.PlayAnimMontage` _ownercharacter "/Game/Assets/MeleeAnimSet/AM_Attack_Move_med_Rhigh_1.AM_Attack_Move_med_Rhigh_1" 1.0 "spine_02")
            (set `self.AttackCounter` 0)))
        (else
          (set `self.ResetAttack` true))))))

(fn `UserConstructionScript`
  (`parent.UserConstructionScript`)
  (set `self.HitEnemy` false)
  (set `self.Destructible` null)
  (set `self.ImageWeapon` "/Game/Assets/Images/knife.knife"))