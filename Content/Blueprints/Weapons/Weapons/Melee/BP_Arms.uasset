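; BP_Arms is the unarmed melee weapon, living as child actors on a character's hands and feet and self-destructing without a parent.
; Base attacks run target traces and alternate right and left hook montages, while a collision toggle enables the matching limb's hit sphere.
; Sphere overlaps filter targets through enemy class lists, then apply damage, camera shake and noise, plus blood, sound and impulse on humans.
; Blocking plays a montage; kick and knee logic is disconnected.
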(event `self.Sphere.OnComponentBeginOverlap`
  (params (OverlappedComponent :type "PrimitiveComponent Object Reference") (OtherActor :type "Actor Object Reference") (OtherComp :type "PrimitiveComponent Object Reference") (OtherBodyIndex :type Integer) (bFromSweep :type Boolean) (SweepResult :type "HitResult Structure (by ref)"))
  (bind _newvar_0_0 (`self.NewVar_0_0`))
  (bind _newvar_0_0_2 (`self.NewVar_0_0`))
  (bind _returnvalue (`self.K2_GetActorLocation` (`self.NewVar_0_0`)))
  (if (not (or (`/Game/Blueprints/BaseCharacterClass.Dead` _newvar_0_0_2) (`/Game/Blueprints/BaseCharacterClass.Stuned` _newvar_0_0_2) (`/Game/Blueprints/BaseCharacterClass.Kicked` _newvar_0_0_2)))
    (bind _detected (`self.TargetDetection` OtherActor))
    (if _detected
      (set `self.HitBone` SweepResult_HitBoneName)
      (set `self.HitComponent` OtherComp)
      (bind _output_get (set `self.HitActor` OtherActor))
      (bind _asbase_character_class (cast `/Game/Blueprints/BaseCharacterClass` _output_get)
        (:`then`
          (set `/Game/Blueprints/BaseCharacterClass.Hit_I` (`self.I`) _asbase_character_class)
          (`self.ContactDispatcher`)
          (set `/Game/Blueprints/BaseCharacterClass.DeathEnumVar` "NewEnumerator1" _asbase_character_class))
        (:`CastFailed`
          _))
      (`GameplayStatics.ApplyDamage` (`self.HitActor`) (`self.AttackDamage`) (`Pawn.GetController` (`self.NewVar_0_0`)) (`self.GetParentActor`) "/Script/Engine.DamageType")
      (`self.ShakePlayersCamera` null 2.0)
      (`self.MakeNoise` _newvar_0_0 10.0 _newvar_0_0 (`self.K2_GetActorLocation` _newvar_0_0) 0.0 "None")
      (if (`self.ActorHasTag` (`self.HitActor`) "human")
        (bind _asbase_character_class_2 (cast `/Game/Blueprints/BaseCharacterClass` (`self.HitActor`)))
        (if (`/Game/Blueprints/BaseCharacterClass.Dead` _asbase_character_class_2)
          (`GameplayStatics.PlaySoundAtLocation` "/Game/Assets/Sounds/Effects/FistPunch2__WAV_.FistPunch2__WAV_" _returnvalue (struct) 1.0 1.0 0.05 "/Game/Blueprints/SoundBlueprints/SoundAttenuationSettings.SoundAttenuationSettings")
          (`KismetSystemLibrary.RetriggerableDelay` 0.01)
          (`GameplayStatics.PlaySoundAtLocation` "/Game/Assets/Sounds/Effects/Skull__FinalArms_.Skull__FinalArms_" _returnvalue (struct) 1.0 1.0 0.05 "/Game/Blueprints/SoundBlueprints/SoundAttenuationSettings.SoundAttenuationSettings")
          (`KismetSystemLibrary.RetriggerableDelay` 0.08)
          (set `self.PunchBool` true)
          (else
            (`GameplayStatics.PlaySoundAtLocation` "/Game/Assets/Sounds/Effects/FistPunch__WAV_.FistPunch__WAV_" _returnvalue (struct) 1.0 1.0 0.3 "/Game/Blueprints/SoundBlueprints/SoundAttenuationSettings.SoundAttenuationSettings")
            (set `self.PunchDelay` 0.085)))
        (bind _asbase_character_class_3 (cast `/Game/Blueprints/BaseCharacterClass` (`self.HitActor`)))
        (bind _mesh (`Character.Mesh` _asbase_character_class_3))
        (bind _output_get_2 (set `self.HitComponent` _mesh))
        (bind _returnvalue_location (`KismetMathLibrary.BreakTransform` (`SceneComponent.K2_GetComponentToWorld` _mesh)))
        (set `self.BloodEmitterLoc` (+ _returnvalue_location (0.0 0.0 150.0)))
        (bind _returnvalue_2 (`GameplayStatics.SpawnEmitterAttached` "/Game/Assets/FXVillesBloodVFXPack/Particles/PS_StyleBlood_Slash_Z_MED.PS_StyleBlood_Slash_Z_MED" _output_get_2 "head" (`self.BloodEmitterLoc`) (struct) (1.0 1.0 1.0) "KeepWorldPosition"))
        (set `self.BloodEmitter` _returnvalue_2)
        (`PrimitiveComponent.AddImpulse` (`self.HitComponent`) (* (`self.GetActorForwardVector` (`self.NewVar_0_0`)) 10000.0) "spine_02" false)))))

(event `EventPunched`
  (`PrimitiveComponent.SetCollisionEnabled` (`self.Sphere`) "NoCollision"))

(event `EventToggleHitCollisions`
  (params (EnableCollision :type Boolean))
  (`self.SetAttackCollision` EnableCollision))

(event `self.Capsule.OnComponentBeginOverlap`
  (params (OverlappedComponent :type "PrimitiveComponent Object Reference") (OtherActor :type "Actor Object Reference") (OtherComp :type "PrimitiveComponent Object Reference") (OtherBodyIndex :type Integer) (bFromSweep :type Boolean) (SweepResult :type "HitResult Structure (by ref)")))

(event `self.EventBlock`
  (if (`self.ResetAttack`)
    (`self.ToggleGlobalTimeDilation` false)
    (`Character.PlayAnimMontage` (`self.NewVar_0_0`) "/Game/Assets/AIBehaviorToolkit/Assets/Mannequin/Animations/AM_BlockArms.AM_BlockArms" 1.0 "spine_02")))

(event `self.ReceiveBeginPlay`
  (bind _sphere (`self.Sphere`))
  (`parent.ReceiveBeginPlay`)
  (set `self.ChangeWeaponType` false)
  (`PrimitiveComponent.SetCollisionEnabled` _sphere "NoCollision")
  (if (`self.ActorHasTag` (`self.GetParentActor`) "ai")
    (`SphereComponent.SetSphereRadius` _sphere 4.0 false))
  (bind _asdsm_game_instance (cast `/Game/Blueprints/Dsm_GameInstance` (`GameplayStatics.GetGameInstance`)))
  (set `self.GameInstance` _asdsm_game_instance)
  (`/Engine/EditorBlueprintResources/StandardMacros.IsValid` (`self.GetParentActor`)
    (:`Is Valid`
      (bind _asbase_character_class (cast `/Game/Blueprints/BaseCharacterClass` (`self.GetParentActor`)))
      (set `self.NewVar_0_0` _asbase_character_class)
      (if (`self.ActorHasTag` (`self.GetParentActor`) "player")
        (set `self.AttackRate` 1.2)
        (bind _asplayers_character (cast `/Game/Blueprints/PlayersCharacter` (`self.GetParentActor`)))
        (set `self.Player` _asplayers_character)
        (else
          (set `self.AttackRate` 1.0)))
      (`KismetSystemLibrary.Delay` 0.5)
      (set `/Game/Blueprints/BaseCharacterClass.CanAttack` true (`self.NewVar_0_0`)))
    (:`Is Not Valid`
      (`self.K2_DestroyActor`))))

(event `EventBaseAttack`
  (bind _newvar_0_0 (`self.NewVar_0_0`))
  (bind _newvar_0_0_2 (`self.NewVar_0_0`))
  (bind _newvar_0_0_3 (`self.NewVar_0_0`))
  ;[1 1 1] BaseAttack
  (if (`/Game/Blueprints/BaseCharacterClass.Dead` (`self.NewVar_0_0`))
    _
    (elif (`self.ResetAttack`)
      (set `self.ResetAttack` false)
      (bind _returnvalue (`Character.GetCurrentMontage` _newvar_0_0_3))
      (`Character.StopAnimMontage` _newvar_0_0_3 _returnvalue)
      (`self.TraceForShield`)
      (`self.FindTarget`)
      (`self.ToggleGlobalTimeDilation` false)
      (`self.Trace` 250.0 "NewEnumerator1")
      (`/Engine/EditorBlueprintResources/StandardMacros.IsValid` (`self.TracedActor`)
        (:`Is Valid`
          _)
        (:`Is Not Valid`
          _))
      (set `self.FootAttack` false)
      (switch `int` (`self.AttackCounter`)
        (:`0`
          (set `self.LeftHandAttack` false)
          (`Character.PlayAnimMontage` _newvar_0_0 "/Game/Assets/FightingAnimsetPro/AM_KB_p_MidHook_R.AM_KB_p_MidHook_R" 1.3 "spine_02")
          (`/Engine/EditorBlueprintResources/StandardMacros.IncrementInt` (`self.AttackCounter`)
            (:`  `
              _)))
        (:`1`
          (set `self.LeftHandAttack` true)
          (`Character.PlayAnimMontage` _newvar_0_0 "/Game/Assets/FightingAnimsetPro/AM_KB_p_MidHook_L.AM_KB_p_MidHook_L" 1.3 "spine_02")
          (`/Engine/EditorBlueprintResources/StandardMacros.IncrementInt` (`self.AttackCounter`)
            (:`  `
              _)))
        (:`2`
          (set `self.LeftHandAttack` false)
          (`Character.PlayAnimMontage` _newvar_0_0_2 "/Game/Assets/FightingAnimsetPro/AM_KB_p_MidHook_R.AM_KB_p_MidHook_R" 1.3 "spine_02")
          (`/Engine/EditorBlueprintResources/StandardMacros.IncrementInt` (`self.AttackCounter`)
            (:`  `
              _)))
        (:`3`
          (set `self.LeftHandAttack` true)
          (`Character.PlayAnimMontage` _newvar_0_0_2 "/Game/Assets/FightingAnimsetPro/AM_KB_p_MidHook_L.AM_KB_p_MidHook_L" 1.3 "spine_02")
          (set `self.AttackCounter` 0)))
      (set `self.TracedActor` null))))

(event `self.ReceiveTick`
  (params (DeltaSeconds :type "Float (single-precision)"))
  (`parent.ReceiveTick` DeltaSeconds)
  (`/Engine/EditorBlueprintResources/StandardMacros.IsValid` (`self.GetParentActor`)
    (:`Is Valid`
      (if (not (`/Game/Blueprints/BaseCharacterClass.CanAttack` (`self.NewVar_0_0`)))
        (`PrimitiveComponent.SetCollisionEnabled` (`self.Sphere`) "NoCollision")))))

(fn `FindTarget`
  (bind _newvar_0_0 (`self.NewVar_0_0`))
  (bind _returnvalue (`SceneComponent.GetRightVector` (`Character.Mesh` _newvar_0_0)))
  (bind _returnvalue_2 (+ (`self.K2_GetActorLocation` _newvar_0_0) (* _returnvalue 50.0)))
  (bind _outhit (`KismetSystemLibrary.BoxTraceSingleForObjects` _returnvalue_2 (+ _returnvalue_2 (* _returnvalue 150.0)) (20.0 20.0 20.0) (struct) (`|MakeArray` "ObjectTypeQuery13" :!type "EObjectTypeQuery Enum") false (`|MakeArray` (`self.NewVar_0_0`) :!type "Actor Object Reference")))
  (`/Engine/EditorBlueprintResources/StandardMacros.IsValid` (`.HitActor` (`GameplayStatics.BreakHitResult` _outhit))
    (:`Is Valid`
      (if (!= (`.HitActor` (`GameplayStatics.BreakHitResult` _outhit)) (`self.TracedActor`))
        (set `self.TracedActor` (`.HitActor` (`GameplayStatics.BreakHitResult` _outhit)))))
    (:`Is Not Valid`
      (set `self.HitEnemy` false)))
  (return))

(fn `KneeAttack`
  (returns (Kick :type Boolean)))

(fn `TargetDetection`
  (params (Object :type "Object Object Reference"))
  (returns (Detected :type Boolean))
  (for _array_element (`/Game/Blueprints/Ai/Enemies/BaseActionNPC.EnemiesArray` (`self.NewVar_0_0`))
    (if (and (== _array_element (`GameplayStatics.GetObjectClass` Object)) (!= (`self.NewVar_0_0`) Object))
      (`|ExecutionSequence`
        (:`then_0`
          (break))
        (:`then_1`
          (return true)))))
  (bind _asbase_character_class (cast `/Game/Blueprints/BaseCharacterClass` Object)
    (:`then`
      (for _array_element_2 (`/Game/Blueprints/Ai/Enemies/BaseActionNPC.EnemiesArray` _asbase_character_class)
        (if (and (== _array_element_2 (`GameplayStatics.GetObjectClass` (`self.NewVar_0_0`))) (!= (`self.NewVar_0_0`) Object))
          (`|ExecutionSequence`
            (:`then_0`
              (break))
            (:`then_1`
              (return true)))))
      (return false))
    (:`CastFailed`
      (return true))))

(fn `UserConstructionScript`
  (bind _staticmesh (`self.StaticMesh`))
  (`parent.UserConstructionScript`)
  (set `self.HitEnemy` true)
  (`PrimitiveComponent.SetCollisionProfileName` _staticmesh "NoCollision")
  (`PrimitiveComponent.SetCollisionEnabled` _staticmesh "NoCollision")
  (`PrimitiveComponent.SetSimulatePhysics` _staticmesh false)
  (`PrimitiveComponent.SetCollisionResponseToAllChannels` _staticmesh "ECR_Ignore")
  (set `self.ImageWeapon` "/Game/Assets/Images/Fist.Fist")
  (`/Engine/EditorBlueprintResources/StandardMacros.IsValid` (`self.GetParentActor`)
    (:`Is Not Valid`
      (`self.K2_DestroyActor`))))