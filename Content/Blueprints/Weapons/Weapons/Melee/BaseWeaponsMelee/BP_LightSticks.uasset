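; BP_LightSticks is a melee weapon that acts as a glow stick, lighting up when punched with and then fading out.
; Light, bound to the inherited Punch event and also run on BeginPlay if WeaponHealth is below 100, brightens the point light and applies a purple glow material.
; Tick dims the light by a fixed, frame-rate-dependent step unless lit and paused, then clears the glow material at zero.
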(event `self.ReceiveBeginPlay`
  (`parent.ReceiveBeginPlay`)
  (add `self.Punch` (delegate `Light`))
  (if (< (`self.WeaponHealth`) 100.0)
    (`self.Light`)))

(event `Light`
  (`LightComponent.SetIntensity` (`self.PointLight`) 5000.0)
  (`PrimitiveComponent.SetMaterial` (`self.StaticMesh`) 0 "/Game/Assets/Env/Infil1_Background/Material/PupleGlow_Inst.PupleGlow_Inst")
  (set `self.Lighted` true))

(event `self.ReceiveTick`
  (params (DeltaSeconds :type "Float (single-precision)"))
  (bind _intensity (`LightComponentBase.Intensity` (`self.PointLight`)))
  (`parent.ReceiveTick` DeltaSeconds)
  (if (`KismetMathLibrary.BooleanNAND` (`self.Lighted`) (`GameplayStatics.IsGamePaused`))
    (if (> _intensity 0.0)
      (`LightComponent.SetIntensity` (`self.PointLight`) (- _intensity 2.0))
      (else
        (`PrimitiveComponent.SetMaterial` (`self.StaticMesh`) 0 null)))))

(fn `UserConstructionScript`
  (`parent.UserConstructionScript`))