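; Melee knuckles weapon, attached as a child actor to a character, that deals close-range hits.
; Each attack makes noise, runs traces and cycles three reused sword montages, setting a damage direction for each.
; A capsule overlap damages valid targets once per swing and shakes the camera.
; Human hits add blood, impulse and hit or kill sounds, and the weapon damages itself.
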(event `self.ReceiveBeginPlay`
  (`parent.ReceiveBeginPlay`)
  (`self.EventSpawned` 0.62 -1 "NewEnumerator0")
  (bind _asbase_character_class (cast `/Game/Blueprints/BaseCharacterClass` (`self.GetParentActor`)))
  (bind _output_get (set `self.OwnerCharacter` _asbase_character_class))
  (cast `/Game/Blueprints/Ai/Enemies/BaseActionNPC` _output_get)
  (set `self.AttackCounter` 1))

(event `self.Capsule.OnComponentBeginOverlap`
  (params (OverlappedComponent :type "PrimitiveComponent Object Reference") (OtherActor :type "Actor Object Reference") (OtherComp :type "PrimitiveComponent Object Reference") (OtherBodyIndex :type Integer) (bFromSweep :type Boolean) (SweepResult :type "HitResult Structure (by ref)"))
  (bind _ownercharacter (`self.OwnerCharacter`))
  (bind _ownercharacter_2 (`self.OwnerCharacter`))
  (bind _hitactor (`self.HitActor`))
  (bind _hitcomponent (`self.HitComponent`))
  (bind _returnvalue (`self.K2_GetActorLocation` _ownercharacter_2))
  (bind _returnvalue_location (`KismetMathLibrary.BreakTransform` (`SceneComponent.K2_GetComponentToWorld` (`self.HitComponent`))))
  (bind _returnvalue_2 (+ (+ (* (`self.GetActorForwardVector` _hitactor) 8.0) (+ _returnvalue_location (0.0 0.0 145.0))) (* (`self.GetActorRightVector` _hitactor) 2.0)))
  (if (not (or (`/Game/Blueprints/BaseCharacterClass.Dead` _ownercharacter) (`/Game/Blueprints/BaseCharacterClass.Stuned` _ownercharacter)))
    (bind _detected (`self.DetectTarget` OtherActor (`self.GetParentActor`)))
    (if _detected
      (if (not (== (`self.HitActor`) OtherActor))
        (set `self.HitBone` SweepResult_HitBoneName)
        (set `self.HitComponent` OtherComp)
        (set `self.HitActor` OtherActor)
        (bind _asbase_character_class (cast `/Game/Blueprints/BaseCharacterClass` (`self.HitActor`))
          (:`then`
            (set `self.HitComponent` (`Character.Mesh` _asbase_character_class)))
          (:`CastFailed`
            _))
        (`self.ContactDispatcher`)
        (`self.ShakePlayersCamera` null 2.0)
        (`GameplayStatics.ApplyDamage` (`self.HitActor`) (`self.AttackDamage`) null (`self.GetParentActor`))
        (if (`self.ActorHasTag` (`self.HitActor`) "human")
          (bind _asbase_character_class_2 (cast `/Game/Blueprints/BaseCharacterClass` (`self.HitActor`))
            (:`then`
              (if (`/Game/Blueprints/BaseCharacterClass.Dead` _asbase_character_class_2)
                (`GameplayStatics.PlaySoundAtLocation` "/Game/Assets/Sounds/Effects/WeaponsSounds/Bbate__knocked__Wav_.Bbate__knocked__Wav_" _returnvalue (struct) 1.0 1.0 0.0 "/Game/Blueprints/SoundBlueprints/SoundAttenuationSettings.SoundAttenuationSettings")
                (`KismetSystemLibrary.Delay` 0.01)
                (`GameplayStatics.PlaySoundAtLocation` "/Game/Assets/Sounds/Effects/Skull__Final_.Skull__Final_" _returnvalue (struct) 1.0 1.0 0.05 "/Game/Blueprints/SoundBlueprints/SoundAttenuationSettings.SoundAttenuationSettings")
                (`PrimitiveComponent.AddImpulse` (`self.HitComponent`) (* (`self.GetActorForwardVector` (`self.OwnerCharacter`)) 1000.0) "spine_02" true)
                (`GameplayStatics.SpawnEmitterAttached` "/Game/Assets/FXVillesBloodVFXPack/Particles/PS_StyleBlood_Slash_Z_MED.PS_StyleBlood_Slash_Z_MED" _hitcomponent "head" _returnvalue_2 (struct) (1.0 1.0 1.0) "KeepWorldPosition")
                (else
                  (`GameplayStatics.PlaySoundAtLocation` "/Game/Assets/Sounds/Effects/WeaponsSounds/BaseballBateHit__WAV_.BaseballBateHit__WAV_" _returnvalue (struct) 1.0 1.0 0.0 "/Game/Blueprints/SoundBlueprints/SoundAttenuationSettings.SoundAttenuationSettings" :!label _label)
                  (`PrimitiveComponent.AddImpulse` (`self.HitComponent`) (* (`self.GetActorForwardVector` _ownercharacter_2) 10000.0) "spine_02" true)
                  (`GameplayStatics.SpawnEmitterAttached` "/Game/Assets/FXVillesBloodVFXPack/Particles/PS_StyleBlood_Slash_Z_MED.PS_StyleBlood_Slash_Z_MED" _hitcomponent "head" _returnvalue_2 (struct) (1.0 1.0 1.0) "KeepWorldPosition"))))
            (:`CastFailed`
              (goto _label)))
          (`GameplayStatics.ApplyDamage` self (`self.SelfAttackDamage`) null self))))))

(event `EventBaseAttack`
  (bind _ownercharacter (`self.OwnerCharacter`))
  (bind _attackcounter (`self.AttackCounter`))
  (bind _ownercharacter_2 (`self.OwnerCharacter`))
  ;[1 1 1] attack
  (if (`/Game/Blueprints/BaseCharacterClass.Dead` (`self.OwnerCharacter`))
    _
    (elif (`self.ResetAttack`)
      (if (not (`self.StopAttack`))
        (set `self.ResetAttack` false)
        (set `self.HitActor` null)
        (`self.TraceForShield`)
        (`self.ToggleGlobalTimeDilation` false)
        (`self.MakeNoise` _ownercharacter_2 10.0 _ownercharacter_2 (`self.K2_GetActorLocation` _ownercharacter_2) 0.0 "None")
        (`self.Trace` 700.0 "NewEnumerator1")
        (switch `int` (`self.AttackCounter`)
          (:`0`
            (`Character.PlayAnimMontage` _ownercharacter "/Game/Assets/MeleeAnimSet/SnsAnimsetPro/AnimMontages/AM_Sword_Attack_Mid_LR.AM_Sword_Attack_Mid_LR" 1.3 "spine_02")
            (`/Engine/EditorBlueprintResources/StandardMacros.IncrementInt` _attackcounter
              (:`  `
                (set `self.DamageDirection` "NewEnumerator2"))))
          (:`1`
            (`Character.PlayAnimMontage` _ownercharacter "/Game/Assets/MeleeAnimSet/SnsAnimsetPro/AnimMontages/AM_Sword_Attack_Sp_U_fast.AM_Sword_Attack_Sp_U_fast" 1.3 "spine_02")
            (`/Engine/EditorBlueprintResources/StandardMacros.IncrementInt` _attackcounter
              (:`  `
                (set `self.DamageDirection` "NewEnumerator0"))))
          (:`2`
            (`Character.PlayAnimMontage` _ownercharacter "/Game/Assets/MeleeAnimSet/SnsAnimsetPro/AnimMontages/AM_Sword_Attack_Rd_fast.AM_Sword_Attack_Rd_fast" 1.3 "spine_02")
            (set `self.AttackCounter` 0)
            (set `self.DamageDirection` "NewEnumerator1")))
        (else
          (set `self.ResetAttack` true))))))

(fn `UserConstructionScript`
  (`parent.UserConstructionScript`))