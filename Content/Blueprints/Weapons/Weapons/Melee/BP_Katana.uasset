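; Katana melee weapon that characters swing in a three-montage combo or throw at enemies.
; Attacks trace ahead, then capsule overlaps either trigger a block response or deal heavy damage with camera shake, plus blood, stab sound and impulse on humans.
; Thrown hits deal damage once with similar effects, then stop colliding on the hit channels.
; Hits on humans and thrown hits also damage the katana itself.
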(event `EventHitSmth`
  (bind _capsule (`self.Capsule`))
  (`PrimitiveComponent.SetCollisionResponseToChannel` (`self.StaticMesh`) "ECC_GameTraceChannel5" "ECR_Ignore")
  (`PrimitiveComponent.SetCollisionResponseToChannel` _capsule "ECC_GameTraceChannel5" "ECR_Ignore")
  (`PrimitiveComponent.SetCollisionResponseToChannel` _capsule "ECC_GameTraceChannel4" "ECR_Ignore"))

(event `EventHitThrowedHuman`
  (bind _hitactor (`self.HitActor`))
  (if (not (`self.ActorHasTag` (`self.HitActor`) (`|GetArrayItem` (`self.Tags`) 2)))
    (`/Engine/EditorBlueprintResources/StandardMacros.DoOnce` false
      (:`Completed`
        (`GameplayStatics.ApplyDamage` (`self.HitActor`) 100.0 null (`self.LastOwnerActor`))
        (bind _asbase_character_class (cast `/Game/Blueprints/BaseCharacterClass` (`self.HitActor`)))
        (bind _returnvalue_location (`KismetMathLibrary.BreakTransform` (`SceneComponent.K2_GetComponentToWorld` (`Character.Mesh` _asbase_character_class))))
        (`GameplayStatics.SpawnEmitterAtLocation` "/Game/Assets/FXVillesBloodVFXPack/Particles/PS_StyleBlood_Swipe.PS_StyleBlood_Swipe" (+ (+ (* (`self.GetActorForwardVector` _hitactor) 8.0) (+ _returnvalue_location (0.0 0.0 145.0))) (* (`self.GetActorRightVector` _hitactor) 2.0)) (struct :`Pitch` 40.0))
        (`GameplayStatics.PlaySoundAtLocation` "/Game/Assets/AIBehaviorToolkit/Assets/Sounds/Sword/S_Sword_Stab01.S_Sword_Stab01" (`self.K2_GetActorLocation` (`self.HitActor`)) (struct) (`/Game/Blueprints/Dsm_GameInstance.Volume` (`self.GameInstance`)) 1.0 0.0 "/Game/Blueprints/SoundBlueprints/SoundAttenuationSettings.SoundAttenuationSettings")
        (`PrimitiveComponent.SetCollisionResponseToChannel` (`self.StaticMesh`) "ECC_GameTraceChannel4" "ECR_Ignore")
        (`GameplayStatics.PlaySoundAtLocation` null (`self.K2_GetActorLocation` (`self.HitActor`)) (struct) (`/Game/Blueprints/Dsm_GameInstance.Volume` (`self.GameInstance`)) 1.0 0.0 "/Game/Blueprints/SoundBlueprints/SoundAttenuationSettings.SoundAttenuationSettings")
        (`GameplayStatics.ApplyDamage` self 30.0 null self)
        (`PrimitiveComponent.SetCollisionResponseToChannel` (`self.StaticMesh`) "ECC_GameTraceChannel5" "ECR_Ignore")
        (`GameplayStatics.PlaySoundAtLocation` null (`self.K2_GetActorLocation`) (struct) (`/Game/Blueprints/Dsm_GameInstance.Volume` (`self.GameInstance`)) 1.0 0.0 "/Game/Blueprints/SoundBlueprints/SoundAttenuationSettings.SoundAttenuationSettings")))))

(event `self.Capsule.OnComponentBeginOverlap`
  (params (OverlappedComponent :type "PrimitiveComponent Object Reference") (OtherActor :type "Actor Object Reference") (OtherComp :type "PrimitiveComponent Object Reference") (OtherBodyIndex :type Integer) (bFromSweep :type Boolean) (SweepResult :type "HitResult Structure (by ref)"))
  (bind _newvar_0_0 (`self.NewVar_0_0`))
  (bind _hitactor (`self.HitActor`))
  (bind _returnvalue_location (`KismetMathLibrary.BreakTransform` (`SceneComponent.K2_GetComponentToWorld` (`self.HitComponent`))))
  (if (or (`/Game/Blueprints/BaseCharacterClass.Dead` _newvar_0_0) (`/Game/Blueprints/BaseCharacterClass.Stuned` _newvar_0_0) (`/Game/Blueprints/BaseCharacterClass.Kicked` _newvar_0_0))
    _
    (elif (`self.ActorHasTag` OtherActor (`|GetArrayItem` (`Actor.Tags` (`self.GetParentActor`)) 2))
      _
      (elif (not (== (`self.HitActor`) OtherActor))
        (set `self.HitBone` SweepResult_HitBoneName)
        (set `self.HitComponent` OtherComp)
        (bind _output_get (set `self.HitActor` OtherActor))
        (`self.ContactDispatcher`)
        (bind _asbase_character_class (cast `/Game/Blueprints/BaseCharacterClass` (`self.HitActor`))
          (:`then`
            (if (`self.Blocked`)
              (set `self.ResetAttack` true)
              (`GameplayStatics.PlaySoundAtLocation` "/Game/Assets/AIBehaviorToolkit/Assets/Sounds/Sword/S_Sword_Hit02.S_Sword_Hit02" (`self.K2_GetActorLocation` (`self.NewVar_0_0`)) (struct) 1.0 1.0 0.0 "/Game/Blueprints/SoundBlueprints/SoundAttenuationSettings.SoundAttenuationSettings")
              (`/Game/Blueprints/PlayersComponents/BlockOverlapComponent.EventBlockOverlap` (`self.BlockOverlapComponent`))
              (else
                (set `/Game/Blueprints/BaseCharacterClass.Hit_I` 2 _asbase_character_class)
                (set `/Game/Blueprints/BaseCharacterClass.CounterI` 2 _asbase_character_class)
                (`GameplayStatics.ApplyDamage` _output_get 100.0 null (`self.GetParentActor`))
                (`self.ShakePlayersCamera` null 1.0)
                (if (`self.ActorHasTag` (`self.HitActor`) "human")
                  (`GameplayStatics.PlaySoundAtLocation` (`self.HitHumanStab`) (`self.K2_GetActorLocation` (`self.GetParentActor`)) (struct) 1.0 2.0 0.0 "/Game/Blueprints/SoundBlueprints/SoundAttenuationSettings.SoundAttenuationSettings")
                  (`GameplayStatics.SpawnEmitterAtLocation` "/Game/Assets/FXVillesBloodVFXPack/Particles/PS_StyleBlood_Swipe.PS_StyleBlood_Swipe" (+ (+ (* (`self.GetActorForwardVector` _hitactor) 8.0) (+ _returnvalue_location (0.0 0.0 145.0))) (* (`self.GetActorRightVector` _hitactor) 2.0)) (struct :`Pitch` 40.0))
                  (`PrimitiveComponent.AddImpulse` (`self.HitComponent`) (* (`self.GetActorForwardVector` (`self.NewVar_0_0`)) 1000.0) "spine_02" true)
                  (`GameplayStatics.ApplyDamage` self 25.0 null self)))))
          (:`CastFailed`
            (`GameplayStatics.ApplyDamage` (`self.HitActor`) 100.0 null (`self.GetParentActor`))))))))

(event `self.EventBlock`
  (if (`self.ResetAttack`)
    (`self.ToggleGlobalTimeDilation` false)
    (`Character.PlayAnimMontage` (`self.NewVar_0_0`) "/Game/Assets/AIBehaviorToolkit/Assets/Mannequin/Animations/AM_BlockArms.AM_BlockArms" 1.0 "spine_02")))

(event `EventPunched`
  (`PrimitiveComponent.SetCollisionEnabled` (`self.Sphere`) "NoCollision"))

(event `self.ReceiveBeginPlay`
  (bind _returnvalue (`self.GetParentActor`))
  (bind _sphere (`/Game/Blueprints/BaseCharacterClass.Sphere` (`self.LastOwnerActor`)))
  (`parent.ReceiveBeginPlay`)
  (`self.EventSpawned` 0.62 -1)
  (bind _asdsm_game_instance (cast `/Game/Blueprints/Dsm_GameInstance` (`GameplayStatics.GetGameInstance`)))
  (set `self.GameInstance` _asdsm_game_instance)
  (`/Engine/EditorBlueprintResources/StandardMacros.IsValid` _returnvalue
    (:`Is Valid`
      (bind _asbase_character_class (cast `/Game/Blueprints/BaseCharacterClass` _returnvalue))
      (set `self.NewVar_0_0` _asbase_character_class)
      (if (`self.Throw`)
        (`SceneComponent.K2_SetWorldLocationAndRotation` (`self.StaticMesh`) (`SceneComponent.K2_GetComponentLocation` _sphere) (`KismetMathLibrary.Conv_VectorToRotator` (`SceneComponent.GetForwardVector` _sphere)) false false))
      (if (`self.ActorHasTag` (`self.GetParentActor`) "player")
        (bind _asplayers_character (cast `/Game/Blueprints/PlayersCharacter` (`self.NewVar_0_0`)))
        (bind _output_get (set `self.Player` _asplayers_character)))
      (`KismetSystemLibrary.Delay` 0.02)
      (set `self.LeftHandAttack` false))
    (:`Is Not Valid`
      (`SceneComponent.K2_SetRelativeRotation` (`self.StaticMesh`) (struct :`Pitch` -90.0 :`Yaw` 160.0 :`Roll` -30.0) false false))))

(event `self.ReceiveTick`
  (params (DeltaSeconds :type "Float (single-precision)"))
  (bind _bloodemitter (`self.BloodEmitter`))
  (bind _newvar_0_0 (`self.NewVar_0_0`))
  (`parent.ReceiveTick` DeltaSeconds)
  (`self.EventTogglePhysics`)
  (`/Engine/EditorBlueprintResources/StandardMacros.IsValid` _newvar_0_0
    (:`Is Valid`
      (if (not (`/Game/Blueprints/BaseCharacterClass.CanAttack` (`self.NewVar_0_0`)))
        (`PrimitiveComponent.SetCollisionEnabled` (`self.Sphere`) "NoCollision"))
      (`SceneComponent.K2_SetWorldRotation` (`self.Arrow`) (`KismetMathLibrary.Conv_VectorToRotator` (`KismetMathLibrary.GetRightVector` (`SceneComponent.K2_GetComponentRotation` (`Character.Mesh` _newvar_0_0)))) false false)
      (`/Engine/EditorBlueprintResources/StandardMacros.IsValid` _bloodemitter
        (:`Is Valid`
          (set `ParticleSystemComponent.CustomTimeDilation` (`Actor.CustomTimeDilation` (`self.GetParentActor`)) _bloodemitter))))))

(event `EventToggleHitCollisions`
  (params (EnableCollision :type Boolean))
  (`self.ToggleHitCollisions` (`|MakeArray` (`self.Capsule`) :!type "PrimitiveComponent Object Reference") EnableCollision))

(event `EventBaseAttack`
  (bind _newvar_0_0 (`self.NewVar_0_0`))
  (bind _newvar_0_0_2 (`self.NewVar_0_0`))
  ;[1 1 1] attack
  (if (not (`/Game/Blueprints/BaseCharacterClass.Dead` _newvar_0_0_2))
    (if (`/Game/Blueprints/BaseCharacterClass.Blocked` _newvar_0_0_2)
      (set `self.ResetAttack` true))
    (if (`self.ResetAttack`)
      (if (not (`self.StopAttack`))
        (set `self.ResetAttack` false)
        (`self.TraceForShield`)
        (`self.ToggleGlobalTimeDilation` false)
        (`self.Trace` 700.0 "NewEnumerator1")
        (set `self.HitActor` null)
        (switch `int` (`self.I`)
          (:`0`
            (`Character.PlayAnimMontage` _newvar_0_0 "/Game/Assets/MeleeAnimSet/AM_Attack_Move_slow_Lup.AM_Attack_Move_slow_Lup" 1.5 "spine_02")
            (`/Engine/EditorBlueprintResources/StandardMacros.IncrementInt` (`self.I`)
              (:`  `
                (set `self.HitHumanStab` "/Game/Assets/Sounds/Effects/WeaponsSounds/KatanaSounds/KatanaStab.KatanaStab"))))
          (:`1`
            (`Character.PlayAnimMontage` _newvar_0_0 "/Game/Assets/MeleeAnimSet/AM_Attack_Move_slow_whirl_L_2.AM_Attack_Move_slow_whirl_L_2" 1.5 "spine_02")
            (`/Engine/EditorBlueprintResources/StandardMacros.IncrementInt` (`self.I`)
              (:`  `
                (set `self.HitHumanStab` "/Game/Assets/Sounds/Effects/WeaponsSounds/KatanaSounds/KatanaStab1.KatanaStab1"))))
          (:`2`
            (`Character.PlayAnimMontage` _newvar_0_0 "/Game/Assets/MeleeAnimSet/AM_Attack_Run_Jump_T.AM_Attack_Run_Jump_T" 1.5 "spine_02")
            (set `self.I` 0)
            (set `self.HitHumanStab` "/Game/Assets/Sounds/Effects/WeaponsSounds/KatanaSounds/KatanaStab2.KatanaStab2")))
        (else
          (set `self.ResetAttack` true))))))

(fn `UserConstructionScript`
  (`parent.UserConstructionScript`)
  (set `self.HitEnemy` false)
  (set `self.Destructible` null)
  (set `self.ImageWeapon` "/Game/Assets/Images/Katana.Katana")
  (set `self.WeaponHealth` 300.0))