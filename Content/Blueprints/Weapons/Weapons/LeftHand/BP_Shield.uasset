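; Destructible left-hand shield weapon, attached to a parent character, that can bash other characters.
; Its attack plays a montage and sets an overlap response; overlaps damage characters lacking the owner's team-like tag, once per stored hit actor.
; Human hits add sound, blood and impulse, varying on death, and damage the shield itself.
; When the destroyed dispatcher fires, an NPC owner loses its shield flag, doubles walk speed and gets stunned.
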(event `self.ReceiveBeginPlay`
  (bind _returnvalue (`self.GetParentActor`))
  (`parent.ReceiveBeginPlay`)
  (set `self.HitActor` null)
  (`/Engine/EditorBlueprintResources/StandardMacros.IsValid` _returnvalue
    (:`Is Valid`
      (bind _asbase_character_class (cast `/Game/Blueprints/BaseCharacterClass` _returnvalue))
      (set `self.BaseCharacter` _asbase_character_class)
      (set `/Game/Blueprints/BaseCharacterClass.WeaponType` "NewEnumerator4" _asbase_character_class)
      (set `self.LeftHand` true)
      (add `self.DestroyedtDispatcher` (delegate `EventChangeAnim`))
      (`PrimitiveComponent.SetCollisionEnabled` (`self.StaticMesh`) "NoCollision")
      (`KismetSystemLibrary.Delay` 2.0)
      (`PrimitiveComponent.SetCollisionEnabled` (`self.StaticMesh`) "NoCollision"))))

(event `self.StaticMesh.OnComponentBeginOverlap`
  (params (OverlappedComponent :type "PrimitiveComponent Object Reference") (OtherActor :type "Actor Object Reference") (OtherComp :type "PrimitiveComponent Object Reference") (OtherBodyIndex :type Integer) (bFromSweep :type Boolean) (SweepResult :type "HitResult Structure (by ref)"))
  (bind _basecharacter (`self.BaseCharacter`))
  (bind _returnvalue (`self.K2_GetActorLocation` (`self.BaseCharacter`)))
  (bind _returnvalue_location (`KismetMathLibrary.BreakTransform` (`SceneComponent.K2_GetComponentToWorld` (`self.HitComponent`))))
  (bind _returnvalue_2 (+ (+ (* (`self.GetActorForwardVector` (`self.HitActor`)) 8.0) (+ _returnvalue_location (0.0 0.0 145.0))) (0.0 0.0 0.0)))
  (if (or (`/Game/Blueprints/BaseCharacterClass.Dead` _basecharacter) (`/Game/Blueprints/BaseCharacterClass.Stuned` _basecharacter) (`/Game/Blueprints/BaseCharacterClass.Kicked` _basecharacter))
    _
    (elif (`self.ActorHasTag` OtherActor (`|GetArrayItem` (`Actor.Tags` (`self.GetParentActor`)) 2))
      _
      (elif (not (== (`self.HitActor`) OtherActor))
        (set `self.HitBone` SweepResult_HitBoneName)
        (set `self.HitComponent` OverlappedComponent)
        (set `self.HitActor` OtherActor)
        (bind _asbase_character_class (cast `/Game/Blueprints/BaseCharacterClass` (`self.HitActor`)))
        (`self.ContactDispatcher`)
        (set `/Game/Blueprints/BaseCharacterClass.DeathEnumVar` "NewEnumerator4" _asbase_character_class)
        (`GameplayStatics.ApplyDamage` (`self.HitActor`) 100.0 null (`self.GetParentActor`))
        (if (`self.ActorHasTag` (`self.HitActor`) "human")
          (bind _asbase_character_class_2 (cast `/Game/Blueprints/BaseCharacterClass` (`self.HitActor`))
            (:`then`
              (if (`/Game/Blueprints/BaseCharacterClass.Dead` _asbase_character_class_2)
                (`GameplayStatics.PlaySoundAtLocation` "/Game/Assets/Sounds/Effects/WeaponsSounds/Bbate__knocked__Wav_.Bbate__knocked__Wav_" _returnvalue (struct) 1.0 1.0 0.0 "/Game/Blueprints/SoundBlueprints/SoundAttenuationSettings.SoundAttenuationSettings")
                (`KismetSystemLibrary.Delay` 0.01)
                (`GameplayStatics.PlaySoundAtLocation` "/Game/Assets/Sounds/Effects/Skull__Final_.Skull__Final_" _returnvalue (struct) 1.0 1.0 0.05 "/Game/Blueprints/SoundBlueprints/SoundAttenuationSettings.SoundAttenuationSettings")
                (`GameplayStatics.SpawnEmitterAtLocation` "/Game/Assets/FXVillesBloodVFXPack/Particles/PS_StyleBlood_Burst_02.PS_StyleBlood_Burst_02" _returnvalue_2 (struct :`Pitch` 40.0))
                (`PrimitiveComponent.AddImpulse` (`self.HitComponent`) (* (`self.GetActorForwardVector` (`self.BaseCharacter`)) 1000.0) "spine_02" true)
                (`KismetSystemLibrary.Delay` 0.09)
                (else
                  (`GameplayStatics.PlaySoundAtLocation` "/Game/Assets/Sounds/Effects/WeaponsSounds/BaseballBateHit__WAV_.BaseballBateHit__WAV_" _returnvalue (struct) 1.0 1.0 0.0 "/Game/Blueprints/SoundBlueprints/SoundAttenuationSettings.SoundAttenuationSettings" :!label _label)
                  (`GameplayStatics.SpawnEmitterAtLocation` "/Game/Assets/FXVillesBloodVFXPack/Particles/PS_StyleBlood_Burst_02.PS_StyleBlood_Burst_02" _returnvalue_2 (struct :`Pitch` 40.0))
                  (`PrimitiveComponent.AddImpulse` (`self.HitComponent`) (* (`KismetMathLibrary.GetRightVector` (`SceneComponent.K2_GetComponentRotation` (`Character.Mesh` (`self.BaseCharacter`)))) 2.0) "spine_02" true))))
            (:`CastFailed`
              (goto _label)))
          (`GameplayStatics.ApplyDamage` self 25.0 null self))))))

(event `EventChangeAnim`
  (bind _returnvalue (`self.GetParentActor`))
  (`/Engine/EditorBlueprintResources/StandardMacros.IsValid` _returnvalue
    (:`Is Valid`
      (bind _asbase_action_npc (cast `/Game/Blueprints/Ai/Enemies/BaseActionNPC` _returnvalue))
      (set `/Game/Blueprints/Ai/Enemies/BaseActionNPC.HaveShield` false _asbase_action_npc)
      (set `/Game/Blueprints/BaseCharacterClass.WeaponType` "NewEnumerator4" _asbase_action_npc)
      (bind _charactermovement (`Character.CharacterMovement` _asbase_action_npc))
      (set `CharacterMovementComponent.MaxWalkSpeed` (* (`CharacterMovementComponent.MaxWalkSpeed` _charactermovement) 2.0) _charactermovement)
      (`/Game/Blueprints/BaseCharacterClass.EventStun` _asbase_action_npc))))

(event `EventToggleHitCollisions`
  (params (EnableCollision :type Boolean))
  (`self.ToggleHitCollisions` (`|MakeArray` (`self.StaticMesh`) :!type "PrimitiveComponent Object Reference") EnableCollision))

(event `self.ReceiveTick`
  (params (DeltaSeconds :type "Float (single-precision)"))
  (`parent.ReceiveTick` DeltaSeconds))

(event `EventBaseAttack`
  (if (`/Game/Blueprints/BaseCharacterClass.Dead` (`self.BaseCharacter`))
    _
    (elif (`self.ResetAttack`)
      (if (not (`self.StopAttack`))
        (set `self.ResetAttack` false)
        (set `self.HitActor` null)
        (`PrimitiveComponent.SetCollisionResponseToChannel` (`self.StaticMesh`) "ECC_GameTraceChannel2" "ECR_Overlap")
        (`Character.PlayAnimMontage` (`self.BaseCharacter`) "/Game/Assets/MeleeAnimSet/AM_Attack_Run_Jump_T1.AM_Attack_Run_Jump_T1" 1.0 "spine_02")
        (else
          (set `self.ResetAttack` true))))))

(fn `UserConstructionScript`
  (`parent.UserConstructionScript`)
  (`MeshComponent.SetVectorParameterValueOnMaterials` (`self.StaticMesh`) "Color" (0.1 0.1 0.1))
  (set `self.Destructible` "/Game/Assets/MeleeAnimSet/Models/Shield/Shield_DM.Shield_DM")
  (set `self.WeaponHealth` 1200.0))