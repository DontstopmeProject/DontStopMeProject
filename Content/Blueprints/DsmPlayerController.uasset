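; Player controller that sets game-only input on start and tracks whether the player uses gamepad or another input device.
; BeginPlay caches the controlled PlayersCharacter, hides the cursor and enables the character's input.
; The ToggleInputMode action stores the device type in Dsm_GameInstance, while EventToggleInput disables or enables character input with debug prints.
; Tick's pause check has no effect, and leftover Game-and-UI input-mode logic is unwired.
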(event `InputAction|ToggleInputMode` :consume false :paused true :overrideparent false
  (params (Key :type "Key Structure"))
  (:`Pressed`
    (bind _asdsm_game_instance (cast `/Game/Blueprints/Dsm_GameInstance` (`GameplayStatics.GetGameInstance`)))
    (if (`KismetInputLibrary.Key_IsGamepadKey` Key)
      (set `/Game/Blueprints/Dsm_GameInstance.InputType` "NewEnumerator1" _asdsm_game_instance)
      (else
        (set `/Game/Blueprints/Dsm_GameInstance.InputType` "NewEnumerator0" _asdsm_game_instance)))))

(event `EventToggleInput`
  (params (Disable :type Boolean))
  (bind _returnvalue (`GameplayStatics.GetPlayerController` 0))
  (bind _returnvalue_2 (`GameplayStatics.GetPlayerCharacter` 0))
  (if Disable
    (`self.DisableInput` _returnvalue_2 _returnvalue)
    (`KismetSystemLibrary.PrintString` "1")
    (else
      (`self.EnableInput` _returnvalue_2 _returnvalue)
      (`KismetSystemLibrary.PrintString` "2"))))

(event `self.ReceiveBeginPlay`
  (bind _asplayers_character (cast `/Game/Blueprints/PlayersCharacter` (`self.K2_GetPawn`)))
  (set `self.PlayersCharacter` _asplayers_character)
  (`WidgetBlueprintLibrary.SetInputMode_GameOnly` self)
  (set `self.bShowMouseCursor` false)
  (bind _asplayers_character_2 (cast `/Game/Blueprints/PlayersCharacter` (`GameplayStatics.GetPlayerCharacter` 0)))
  (`self.EnableInput` _asplayers_character_2 self))

(event `self.ReceiveTick`
  (params (DeltaSeconds :type "Float (single-precision)"))
  (bind _playerscharacter (`self.PlayersCharacter`))
  (`/Engine/EditorBlueprintResources/StandardMacros.IsValid` _playerscharacter
    (:`Is Valid`
      (if (`/Game/Blueprints/PlayersCharacter.GamePaused` _playerscharacter)
        _))))

(fn `UserConstructionScript`)