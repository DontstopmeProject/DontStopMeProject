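; One-shot bot spawner that creates one armed AI pawn at its location.
; While enabled, Tick spawns when a timer since BeginPlay elapses, gamemode kills reach a threshold, or SpawnFromBlueprint has configured and forced it.
; The bot gets enemy sight/follow flags and optionally moves to a target actor or location; spawning fires a dispatcher.
; When that move succeeds or fails, sight turns on, following too unless staying, and the spawner destroys itself.
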(event `self.ReceiveBeginPlay`
  (bind _asdsm_gamemode (cast `/Game/Blueprints/DsmGamemode` (`GameplayStatics.GetGameMode`)))
  (set `self.Gamemode` _asdsm_gamemode)
  (bind _asdsm_game_instance (cast `/Game/Blueprints/Dsm_GameInstance` (`GameplayStatics.GetGameInstance`)))
  (set `self.GameInstance` _asdsm_game_instance)
  (set `self.Time` (`GameplayStatics.GetTimeSeconds`)))

(event `self.ReceiveTick`
  (params (DeltaSeconds :type "Float (single-precision)"))
  (bind _spawnedactor (`self.SpawnedActor`))
  (if (`self.SpawnActor`)
    (if (and (>= (- (`GameplayStatics.GetTimeSeconds`) (`self.Time`)) (`self.SpawnTimer`)) (!= (`self.SpawnTimer`) -1.0))
      (`/Engine/EditorBlueprintResources/StandardMacros.DoOnce` false
        (:`Completed`
          (if (not (`self.Spawned`)) :!label _label
            (bind _array (`/Game/Blueprints/BP_Library.SpawnAiOkay` (`self.PawnClass`) "/Game/Blueprints/Ai/DsmAiController.DsmAiController_C" null (`self.K2_GetActorLocation` self) (`self.K2_GetActorRotation` self) false (`self.WeaponClass`) (`self.GroupIndex`)))
            (bind _output (`|GetArrayItem` _array))
            (set `self.SpawnedActor` _output)
            (set `self.SpawnedPawn` _output)
            (if (`KismetSystemLibrary.IsValid` (`self.MoveToActor`))
              (`|AIMoveTo` (`self.SpawnedPawn`) (0.0 0.0 0.0) (`self.MoveToActor`) 10.0 true
                (:`then`
                  (set `self.Spawned` true :!label _label_2)
                  (`/Engine/EditorBlueprintResources/StandardMacros.IsValid` _spawnedactor
                    (:`Is Valid`
                      (bind _asbase_npc (cast `/Game/Blueprints/Ai/BaseNPC` _spawnedactor))
                      (set `/Game/Blueprints/Ai/BaseNPC.SeesEnemy?` (`self.SeesEnemy`) _asbase_npc)
                      (set `/Game/Blueprints/Ai/BaseNPC.FollowsEnemy?` (`self.FollowEnemy`) _asbase_npc))))
                (:`OnSuccess`
                  (if (`self.StayAtTheTargetPoint`) :!label _label_3
                    (bind _asbase_npc_2 (cast `/Game/Blueprints/Ai/BaseNPC` (`self.SpawnedActor`)))
                    (set `/Game/Blueprints/Ai/BaseNPC.SeesEnemy?` true _asbase_npc_2)
                    (else
                      (bind _asbase_npc_3 (cast `/Game/Blueprints/Ai/BaseNPC` (`self.SpawnedActor`)))
                      (set `/Game/Blueprints/Ai/BaseNPC.SeesEnemy?` true _asbase_npc_3)
                      (set `/Game/Blueprints/Ai/BaseNPC.FollowsEnemy?` true _asbase_npc_3)))
                  (`self.K2_DestroyActor` :!label _label_4))
                (:`OnFail`
                  (goto _label_3)))
              (elif (!= (`self.MoveDistanation`) (0.0 0.0 -1000.0))
                (`|AIMoveTo` (`self.SpawnedPawn`) (`self.MoveDistanation`) null 10.0 true
                  (:`then`
                    (goto _label_2))
                  (:`OnSuccess`
                    _)
                  (:`OnFail`
                    _))
                (if (`self.StayAtTheTargetPoint`)
                  (bind _asbase_npc_4 (cast `/Game/Blueprints/Ai/BaseNPC` (`self.SpawnedActor`)))
                  (set `/Game/Blueprints/Ai/BaseNPC.SeesEnemy?` true _asbase_npc_4)
                  (goto _label_4)
                  (else
                    (bind _asbase_npc_5 (cast `/Game/Blueprints/Ai/BaseNPC` (`self.SpawnedActor`)))
                    (set `/Game/Blueprints/Ai/BaseNPC.SeesEnemy?` true _asbase_npc_5)
                    (set `/Game/Blueprints/Ai/BaseNPC.FollowsEnemy?` true _asbase_npc_5)
                    (goto _label_4)))
                (else
                  (goto _label_2))))
            (`self.SpawnedDispatcher`))))
      (elif (and (>= (`/Game/Blueprints/DsmGamemode.kills` (`self.Gamemode`)) (`self.Kills`)) (!= (`self.Kills`) -1))
        (`/Engine/EditorBlueprintResources/StandardMacros.DoOnce` false :!label _label_5
          (:`Completed`
            (goto _label)))
        (elif (`self.SpawnVar`)
          (goto _label_5))))))

(fn `SpawnFromBlueprint`
  (params (WeaponClass :type "Actor Class Reference") (GroupIndex :type Integer) (MoveToActor :type "Actor Object Reference") (MoveDistanation :type "Vector Structure") (PawnClass :type "Pawn Class Reference") (SeesEnemy :type Boolean) (FollowEnemy :type Boolean))
  (set `self.WeaponClass` WeaponClass)
  (set `self.GroupIndex` GroupIndex)
  (set `self.MoveToActor` MoveToActor)
  (set `self.MoveDistanation` MoveDistanation)
  (set `self.SeesEnemy` SeesEnemy)
  (set `self.FollowEnemy` FollowEnemy)
  (set `self.PawnClass` PawnClass)
  (set `self.SpawnVar` true)
  (set `self.SpawnActor` true))

(fn `UserConstructionScript`)