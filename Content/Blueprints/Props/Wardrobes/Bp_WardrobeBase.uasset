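; Base Blueprint for wardrobe props that react to projectile and weapon impacts with sound and particle effects.
; Actor hits and mesh hits from projectiles, plus box overlaps from weapons, call PlayDestructionSounds with a timed emitter, smaller for weapons.
; Mesh and box impacts pick a random sound from an array, while the actor Hit path passes none.
; SpawnBrokenGlass is empty, and an older wood-impact sound and emitter chain is left disconnected.
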(event `SpawnBrokenGlass`
  (params (Target :type "SceneComponent Object Reference") (RelativeTransform :type "Transform Structure") (Location :type "Vector Structure")))

(event `self.ReceiveHit`
  (params (MyComp :type "PrimitiveComponent Object Reference") (Other :type "Actor Object Reference") (OtherComp :type "PrimitiveComponent Object Reference") (bSelfMoved :type Boolean) (HitLocation :type "Vector Structure") (HitNormal :type "Vector Structure") (NormalImpulse :type "Vector Structure") (Hit :type "HitResult Structure (by ref)"))
  (cast `/Game/Blueprints/Weapons/projectiles/BP_ProjectileBase` Other)
  (`self.PlayDestructionSounds` HitLocation HitLocation (6.0 6.0 6.0) (`self.Emitter`) (`self.StaticMesh`) true 1.0))

(event `self.StaticMesh.OnComponentHit`
  (params (HitComponent :type "PrimitiveComponent Object Reference") (OtherActor :type "Actor Object Reference") (OtherComp :type "PrimitiveComponent Object Reference") (NormalImpulse :type "Vector Structure") (Hit :type "HitResult Structure (by ref)"))
  (bind _soundsarray (`self.SoundsArray`))
  (cast `/Game/Blueprints/Weapons/projectiles/BP_ProjectileBase` OtherActor)
  (`self.PlayDestructionSounds` Hit_Location Hit_Location (6.0 6.0 6.0) (`self.Emitter`) (`self.StaticMesh`) true 1.0 (`|GetArrayItem` _soundsarray (`KismetMathLibrary.RandomIntegerInRange` 0 (`KismetArrayLibrary.Array_LastIndex` _soundsarray)))))

(event `self.Box.OnComponentBeginOverlap`
  (params (OverlappedComponent :type "PrimitiveComponent Object Reference") (OtherActor :type "Actor Object Reference") (OtherComp :type "PrimitiveComponent Object Reference") (OtherBodyIndex :type Integer) (bFromSweep :type Boolean) (SweepResult :type "HitResult Structure (by ref)"))
  (bind _soundsarray (`self.SoundsArray`))
  (cast `/Game/Blueprints/Weapons/Weapons/WeaponBase` OtherActor)
  (`self.PlayDestructionSounds` SweepResult_Location SweepResult_Location (3.0 3.0 3.0) (`self.Emitter`) OverlappedComponent true 1.0 (`|GetArrayItem` _soundsarray (`KismetMathLibrary.RandomIntegerInRange` 0 (`KismetArrayLibrary.Array_LastIndex` _soundsarray)))))

(fn `UserConstructionScript`)