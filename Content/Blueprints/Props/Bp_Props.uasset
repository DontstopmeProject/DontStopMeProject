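; Breakable prop base that swaps its static mesh for a physics-driven destructible when damaged, overlapped, or hit by a stunned, dead or kicked character.
; A DoOnce break sequence shakes the camera, can push debris along the overlapping actor's velocity, fires a radial impulse, removes helper components and later stops physics.
; The construction script sets the mesh and optional invisible trigger box, which also decides whether the destructible blocks pawns.
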(event `self.ReceiveAnyDamage`
  (params (Damage :type "Float (single-precision)") (DamageType :type "DamageType Object Reference") (InstigatedBy :type "Controller Object Reference") (DamageCauser :type "Actor Object Reference"))
  (bind _radialforce (`self.RadialForce`))
  (bind _instigatoractor (`self.InstigatorActor`))
  (`/Engine/EditorBlueprintResources/StandardMacros.DoOnce` false :!label _label
    (:`Completed`
      (`ActorComponent.K2_DestroyComponent` (`self.InvisBox`))
      (`SceneComponent.SetHiddenInGame` (`self.StaticMesh`) true false)
      (`DestructibleComponent.SetDestructibleMesh` (`self.Destructible`) (`self.DestructibleMeshs`))
      (`PrimitiveComponent.SetSimulatePhysics` (`self.Destructible`) true)
      (`PlayerCameraManager.PlayCameraShake` :`self` (`GameplayStatics.GetPlayerCameraManager` 0) :`ShakeClass` "/Game/Blueprints/CameraShakes/HitCameraShake.HitCameraShake_C" :`Scale` 2.0)
      (`/Engine/EditorBlueprintResources/StandardMacros.IsValid` _instigatoractor
        (:`Is Valid`
          (if (not (`self.InvertVelVector`))
            (`PrimitiveComponent.AddImpulse` (`self.Destructible`) (* (`self.GetVelocity` _instigatoractor) 1000.0) "None" false))
          (`KismetSystemLibrary.Delay` 0.01))
        (:`Is Not Valid`
          _))
      (`RadialForceComponent.FireImpulse` (`self.RadialForce`))
      (`/Engine/EditorBlueprintResources/StandardMacros.IsValid` (`self.InvisBox`)
        (:`Is Valid`
          (`ActorComponent.K2_DestroyComponent` _radialforce)
          (`ActorComponent.K2_DestroyComponent` (`self.InvisBox`))
          (`ActorComponent.K2_DestroyComponent` (`self.StaticMesh`)))
        (:`Is Not Valid`
          (`ActorComponent.K2_DestroyComponent` _radialforce)
          (`ActorComponent.K2_DestroyComponent` (`self.StaticMesh`))))
      (`PrimitiveComponent.SetCollisionResponseToChannel` (`self.Destructible`) "ECC_Pawn" "ECR_Ignore")
      (`KismetSystemLibrary.Delay` 5.0)
      (`PrimitiveComponent.SetSimulatePhysics` (`self.Destructible`) false))))

(event `self.InvisBox.OnComponentBeginOverlap`
  (params (OverlappedComponent :type "PrimitiveComponent Object Reference") (OtherActor :type "Actor Object Reference") (OtherComp :type "PrimitiveComponent Object Reference") (OtherBodyIndex :type Integer) (bFromSweep :type Boolean) (SweepResult :type "HitResult Structure (by ref)"))
  (set `self.InstigatorActor` OtherActor)
  (goto _label))

(event `self.StaticMesh.OnComponentBeginOverlap`
  (params (OverlappedComponent :type "PrimitiveComponent Object Reference") (OtherActor :type "Actor Object Reference") (OtherComp :type "PrimitiveComponent Object Reference") (OtherBodyIndex :type Integer) (bFromSweep :type Boolean) (SweepResult :type "HitResult Structure (by ref)"))
  (set `self.InstigatorActor` OtherActor)
  (goto _label))

(event `self.StaticMesh.OnComponentHit`
  (params (HitComponent :type "PrimitiveComponent Object Reference") (OtherActor :type "Actor Object Reference") (OtherComp :type "PrimitiveComponent Object Reference") (NormalImpulse :type "Vector Structure") (Hit :type "HitResult Structure (by ref)"))
  (bind _asbase_character_class (cast `/Game/Blueprints/BaseCharacterClass` OtherActor))
  (if (or (`/Game/Blueprints/BaseCharacterClass.Stuned` _asbase_character_class) (`/Game/Blueprints/BaseCharacterClass.Dead` _asbase_character_class) (`/Game/Blueprints/BaseCharacterClass.Kicked` _asbase_character_class))
    (goto _label)))

(event `self.InvisBox.OnComponentHit`
  (params (HitComponent :type "PrimitiveComponent Object Reference") (OtherActor :type "Actor Object Reference") (OtherComp :type "PrimitiveComponent Object Reference") (NormalImpulse :type "Vector Structure") (Hit :type "HitResult Structure (by ref)"))
  (bind _asbase_character_class (cast `/Game/Blueprints/BaseCharacterClass` OtherActor))
  (if (or (`/Game/Blueprints/BaseCharacterClass.Dead` _asbase_character_class) (`/Game/Blueprints/BaseCharacterClass.Stuned` _asbase_character_class) (`/Game/Blueprints/BaseCharacterClass.Kicked` _asbase_character_class))
    (goto _label)))

(event `self.Destructible.OnComponentFracture`
  (params (HitPoint :type "Vector Structure (by ref)") (HitDirection :type "Vector Structure (by ref)"))
  (bind _invisbox (`self.InvisBox`))
  (`/Engine/EditorBlueprintResources/StandardMacros.IsValid` _invisbox
    (:`Is Valid`
      (`ActorComponent.K2_DestroyComponent` _invisbox)
      (`PrimitiveComponent.SetSimulatePhysics` (`self.Destructible`) true))))

(fn `UserConstructionScript`
  (bind _invisbox (`self.InvisBox`))
  (`StaticMeshComponent.SetStaticMesh` (`self.StaticMesh`) (`self.DefaultMesh`))
  (if (`self.EnableInvisBox`)
    (`PrimitiveComponent.SetCollisionEnabled` _invisbox "QueryOnly")
    (`BoxComponent.SetBoxExtent` (`self.InvisBox`) (`self.InvisBoxExtent`) true)
    (`SceneComponent.K2_SetRelativeLocationAndRotation` (`self.InvisBox`) (`self.InvisBoxLocation`) (`self.InvisBoxRotation`) false false)
    (`PrimitiveComponent.SetCollisionResponseToChannel` (`self.Destructible`) "ECC_Pawn" "ECR_Ignore")
    (else
      (`PrimitiveComponent.SetCollisionEnabled` _invisbox "NoCollision")
      (`PrimitiveComponent.SetCollisionResponseToChannel` (`self.Destructible`) "ECC_Pawn" "ECR_Block")))
  (`SceneComponent.K2_SetRelativeLocationAndRotation` :`self` (`self.RadialForce`) :`NewLocation` (`self.InvisBoxLocation`)))