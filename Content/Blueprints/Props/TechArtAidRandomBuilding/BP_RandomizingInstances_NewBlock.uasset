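; Construction-script prop that builds a procedural wall block for a building from a single wall mesh.
; Nested loops over floor and segment counts add one static mesh component per cell.
; Each piece is offset along X and Z by the wall mesh's bounds, so segments tile edge to edge in a flat grid.
; Despite the asset name, placement uses no randomization, and the event graph is empty.
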(fn `UserConstructionScript`
  (for _index (range (`self.NumberOfFloors`))
    (for _index_2 (range (`self.NumberOfSegments`))
      (bind _returnvalue (`AddComponent|NODE_AddStaticMeshComponent-2` :`RelativeTransform` (`KismetMathLibrary.MakeTransform` (`KismetMathLibrary.MakeVector` (* _index_2 (* (.x (`.BoxExtent` (`KismetMathLibrary.BreakBoxSphereBounds` (`StaticMesh.GetBounds` (`self.MeshWall`))))) 2.0)) 0.0 (* _index (* (.z (`.BoxExtent` (`KismetMathLibrary.BreakBoxSphereBounds` (`StaticMesh.GetBounds` (`self.MeshWall`))))) 2.0))))))
      (`StaticMeshComponent.SetStaticMesh` _returnvalue (`self.MeshWall`)))))