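; Elevator prop with two sliding doors driven by a child button actor's dispatcher, optionally opened at construction.
; Open and close events ease the doors with MoveComponentTo and fire an arrival dispatcher, and opening also plays a sound.
; Overlap triggers slow characters and block their actions, restore them, disable camera-arm collision, and auto-close open doors after exit.
; An older counter-and-gate door animation remains as unconnected logic.
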(event `self.ReceiveBeginPlay`
  (`parent.ReceiveBeginPlay`)
  (bind _asbp_button_base (cast `/Game/Blueprints/Props/Buttons/BP_ButtonBase` (`ChildActorComponent.ChildActor` (`self.ButtonActor_0`))))
  (add `/Game/Blueprints/Props/Buttons/BP_ButtonBase.PushedDispatcher` _asbp_button_base (delegate `PushedDispatcher_Event_0`)))

(event `PushedDispatcher_Event_0`
  (if (`self.Opened_0_0`)
    (`self.EventOpen`)
    (else
      (`self.EventClose`)))
  (`self.ButtonPushedEventDispatcher`)
  (bind _asplayers_character (cast `/Game/Blueprints/PlayersCharacter` (`self.Character`)))
  (`KismetSystemLibrary.Delay` 1.0)
  (set `/Game/Blueprints/PlayersCharacter.MasterEnableTimeDilation` true _asplayers_character))

(event `self.ReceiveTick`
  (params (DeltaSeconds :type "Float (single-precision)"))
  (`parent.ReceiveTick` DeltaSeconds)
  (if (`self.Visibilty`)
    (`/Engine/EditorBlueprintResources/StandardMacros.DoOnce` false
      (:`Completed`
        (`SceneComponent.SetVisibility` (`self.Roof_0`) (`self.Visibilty`) false)))))

(event `EventOpen`
  (bind _doorl_0 (`self.DoorL_0`))
  (bind _doorr_0 (`self.DoorR_0`))
  (bind _returnvalue (`SceneComponent.GetRelativeTransform` _doorl_0))
  (bind _returnvalue_2 (`SceneComponent.GetRelativeTransform` _doorr_0))
  (set `self.Opened_0_0` true)
  (`|ExecutionSequence`
    (:`then_0`
      (`KismetSystemLibrary.MoveComponentTo` _doorl_0 (`KismetMathLibrary.MakeVector` (+ (.x (.location _returnvalue)) 150.0) (.y (.location _returnvalue)) (.z (.location _returnvalue))) (.rotation _returnvalue) true true 1.0))
    (:`then_1`
      (`GameplayStatics.PlaySoundAtLocation` "/Game/Assets/Sounds/Effects/ElevatorSound__wav_.ElevatorSound__wav_" (`self.K2_GetActorLocation`) (struct) (`self.SoundVolume`) 1.0 0.0 "/Game/Blueprints/SoundBlueprints/SoundAttenuationSettings.SoundAttenuationSettings")
      (`self.ArrivedDispatcher_0`)
      (`KismetSystemLibrary.MoveComponentTo` _doorr_0 (`KismetMathLibrary.MakeVector` (+ (.x (.location _returnvalue_2)) -150.0) (.y (.location _returnvalue_2)) (.z (.location _returnvalue_2))) (.rotation _returnvalue_2) true true 1.0))))

(event `self.Trigger.OnComponentBeginOverlap`
  (params (OverlappedComponent :type "PrimitiveComponent Object Reference") (OtherActor :type "Actor Object Reference") (OtherComp :type "PrimitiveComponent Object Reference") (OtherBodyIndex :type Integer) (bFromSweep :type Boolean) (SweepResult :type "HitResult Structure (by ref)"))
  (if (and (or (`self.ActorHasTag` OtherActor "player") (`self.ActorHasTag` OtherActor "human")) (`self.CanPassTrigger`))
    (bind _asplayers_character (cast `/Game/Blueprints/PlayersCharacter` OtherActor))
    (set `CharacterMovementComponent.MaxWalkSpeed` 450.0 (`Character.CharacterMovement` _asplayers_character))
    (`/Game/Blueprints/PlayersCharacter.EventSetInput` _asplayers_character false false false false false false false false false)))

(event `EventClose`
  (bind _doorl_0 (`self.DoorL_0`))
  (bind _doorr_0 (`self.DoorR_0`))
  (bind _returnvalue (`SceneComponent.GetRelativeTransform` _doorl_0))
  (bind _returnvalue_2 (`SceneComponent.GetRelativeTransform` _doorr_0))
  (set `self.Opened_0_0` false)
  (`|ExecutionSequence`
    (:`then_0`
      (`KismetSystemLibrary.MoveComponentTo` _doorl_0 (`KismetMathLibrary.MakeVector` (+ (.x (.location _returnvalue)) -150.0) (.y (.location _returnvalue)) (.z (.location _returnvalue))) (.rotation _returnvalue) true true 1.0))
    (:`then_1`
      (`KismetSystemLibrary.MoveComponentTo` _doorr_0 (`KismetMathLibrary.MakeVector` (+ (.x (.location _returnvalue_2)) 150.0) (.y (.location _returnvalue_2)) (.z (.location _returnvalue_2))) (.rotation _returnvalue_2) true true 1.0)
      (`self.ArrivedDispatcher_0`))))

(event `self.Trigger1.OnComponentBeginOverlap`
  (params (OverlappedComponent :type "PrimitiveComponent Object Reference") (OtherActor :type "Actor Object Reference") (OtherComp :type "PrimitiveComponent Object Reference") (OtherBodyIndex :type Integer) (bFromSweep :type Boolean) (SweepResult :type "HitResult Structure (by ref)"))
  (if (or (`self.ActorHasTag` OtherActor "player") (`self.ActorHasTag` OtherActor "human"))
    (bind _asplayers_character (cast `/Game/Blueprints/PlayersCharacter` OtherActor))
    (set `CharacterMovementComponent.MaxWalkSpeed` 200.0 (`Character.CharacterMovement` _asplayers_character))
    (`/Game/Blueprints/PlayersCharacter.EventSetInput` _asplayers_character false false true true false false false false false)
    (set `self.CanPassTrigger` false)))

(event `self.Trigger.OnComponentEndOverlap`
  (params (OverlappedComponent :type "PrimitiveComponent Object Reference") (OtherActor :type "Actor Object Reference") (OtherComp :type "PrimitiveComponent Object Reference") (OtherBodyIndex :type Integer))
  (set `self.CanPassTrigger` true))

(event `self.Box_0.OnComponentBeginOverlap`
  (params (OverlappedComponent :type "PrimitiveComponent Object Reference") (OtherActor :type "Actor Object Reference") (OtherComp :type "PrimitiveComponent Object Reference") (OtherBodyIndex :type Integer) (bFromSweep :type Boolean) (SweepResult :type "HitResult Structure (by ref)"))
  (bind _asplayers_character (cast `/Game/Blueprints/PlayersCharacter` OtherActor))
  (bind _springarm (`/Game/Blueprints/PlayersCharacter.SpringArm` _asplayers_character))
  (if (`SpringArmComponent.bDoCollisionTest` _springarm)
    (set `SpringArmComponent.bDoCollisionTest` false _springarm)
    (else
      (set `SpringArmComponent.bDoCollisionTest` false _springarm))))

(event `self.PlayerControlTrigger.OnComponentEndOverlap`
  (params (OverlappedComponent :type "PrimitiveComponent Object Reference") (OtherActor :type "Actor Object Reference") (OtherComp :type "PrimitiveComponent Object Reference") (OtherBodyIndex :type Integer))
  (if (`self.Opened_0_0`)
    (cast `/Game/Blueprints/PlayersCharacter` OtherActor)
    (set `self.Character` null)
    (set `self.PlayerInLift` false)
    (`KismetSystemLibrary.Delay` 1.0)
    (if (not (`self.PlayerInLift`))
      (`self.EventClose`))))

(event `self.PlayerControlTrigger.OnComponentBeginOverlap`
  (params (OverlappedComponent :type "PrimitiveComponent Object Reference") (OtherActor :type "Actor Object Reference") (OtherComp :type "PrimitiveComponent Object Reference") (OtherBodyIndex :type Integer) (bFromSweep :type Boolean) (SweepResult :type "HitResult Structure (by ref)"))
  (if (not (`self.Opened_0_0`))
    (bind _asplayers_character (cast `/Game/Blueprints/PlayersCharacter` OtherActor))
    (set `self.Character` _asplayers_character)
    (set `self.PlayerInLift` true)))

(fn `UserConstructionScript`
  (`parent.UserConstructionScript`)
  (`SceneComponent.SetVisibility` (`self.Roof_0`) (`self.Visibilty`) false)
  (if (`self.OpenDoors`)
    (if (not (`self.Opened_0_0`))
      (`self.EventOpen`)
      (set `self.Opened_0_0` true))))