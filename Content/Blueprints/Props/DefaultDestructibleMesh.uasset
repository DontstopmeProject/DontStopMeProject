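; Configurable destructible prop that breaks apart when first overlapped or when fractured.
; The construction script assigns the mesh and either enables a sized, positioned invisible box with the mesh ignoring Pawns, or lets the mesh block them.
; Overlap adds an impulse from the other actor's velocity; fracture skips this while the box remains valid.
; Both paths remove the box, enable physics, fire a radial impulse, ignore Pawns, then stop physics after a delay.
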(event `self.Destructible.OnComponentBeginOverlap`
  (params (OverlappedComponent :type "PrimitiveComponent Object Reference") (OtherActor :type "Actor Object Reference") (OtherComp :type "PrimitiveComponent Object Reference") (OtherBodyIndex :type Integer) (bFromSweep :type Boolean) (SweepResult :type "HitResult Structure (by ref)"))
  (set `self.instigatorActor` OtherActor)
  (`/Engine/EditorBlueprintResources/StandardMacros.DoOnce` false
    (:`Completed`
      (`ActorComponent.K2_DestroyComponent` (`self.InvisBox`))
      (`PrimitiveComponent.SetSimulatePhysics` (`self.Destructible`) true)
      (`PrimitiveComponent.AddImpulse` (`self.Destructible`) (* (`self.GetVelocity` (`self.instigatorActor`)) 1000.0) "None" false)
      (`RadialForceComponent.FireImpulse` (`self.RadialForce`) :!label _label)
      (`ActorComponent.K2_DestroyComponent` (`self.RadialForce`))
      (`PrimitiveComponent.SetCollisionResponseToChannel` (`self.Destructible`) "ECC_Pawn" "ECR_Ignore")
      (`KismetSystemLibrary.Delay` 5.0)
      (`PrimitiveComponent.SetSimulatePhysics` (`self.Destructible`) false))))

(event `self.Destructible.OnComponentFracture`
  (params (HitPoint :type "Vector Structure (by ref)") (HitDirection :type "Vector Structure (by ref)"))
  (bind _invisbox (`self.InvisBox`))
  (`/Engine/EditorBlueprintResources/StandardMacros.IsValid` _invisbox
    (:`Is Valid`
      (`ActorComponent.K2_DestroyComponent` _invisbox)
      (`PrimitiveComponent.SetSimulatePhysics` (`self.Destructible`) true)
      (goto _label))))

(fn `UserConstructionScript`
  (bind _invisbox (`self.InvisBox`))
  (`DestructibleComponent.SetDestructibleMesh` (`self.Destructible`) (`self.DestructibleMeshs`))
  (if (`self.EnableInvisBox`)
    (`PrimitiveComponent.SetCollisionEnabled` _invisbox "QueryOnly")
    (`BoxComponent.SetBoxExtent` (`self.InvisBox`) (`self.InvisBoxExtent`) true)
    (`SceneComponent.K2_SetRelativeLocationAndRotation` (`self.InvisBox`) (`self.InvisBoxLocation`) (`self.InvisBoxRotation`) false false)
    (`PrimitiveComponent.SetCollisionResponseToChannel` (`self.Destructible`) "ECC_Pawn" "ECR_Ignore")
    (else
      (`PrimitiveComponent.SetCollisionEnabled` _invisbox "NoCollision")
      (`PrimitiveComponent.SetCollisionResponseToChannel` (`self.Destructible`) "ECC_Pawn" "ECR_Block"))))