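; Breakable computer prop that swaps its static mesh for a simulated destructible component when hit by a projectile or overlapped by anything.
; The swap runs once through a shared DoOnce, and only projectile hits set the flag that adds a backward impulse to the destructible.
; Other hits turn on mesh physics, with weapon hits also pushing it backward and incrementing a Counter that this graph never reads.
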(event `self.StaticMesh.OnComponentHit`
  (params (HitComponent :type "PrimitiveComponent Object Reference") (OtherActor :type "Actor Object Reference") (OtherComp :type "PrimitiveComponent Object Reference") (NormalImpulse :type "Vector Structure") (Hit :type "HitResult Structure (by ref)"))
  (bind _staticmesh (`self.StaticMesh`))
  (bind _staticmesh_2 (`self.StaticMesh`))
  (bind _staticmesh_3 (`self.StaticMesh`))
  (cast `/Game/Blueprints/Weapons/projectiles/BP_ProjectileBase` OtherActor
    (:`then`
      (set `self.GiveImpulse` true)
      (`/Engine/EditorBlueprintResources/StandardMacros.DoOnce` false :!label _label
        (:`Completed`
          (`SceneComponent.SetHiddenInGame` _staticmesh_2 true false)
          (bind _returnvalue (`AddComponent|NODE_AddDestructibleComponent-2` :`bManualAttachment` true :`RelativeTransform` (`SceneComponent.GetRelativeTransform` _staticmesh_2)))
          (`PrimitiveComponent.SetSimulatePhysics` _returnvalue true)
          (`ActorComponent.K2_DestroyComponent` _staticmesh_2)
          (set `self.Counter` 20)
          (if (`self.GiveImpulse`)
            (`PrimitiveComponent.AddImpulse` _returnvalue (* (`SceneComponent.GetForwardVector` _returnvalue) -1000.0) "None" true)))))
    (:`CastFailed`
      (`PrimitiveComponent.SetCollisionEnabled` _staticmesh_3 "QueryAndPhysics")
      (`PrimitiveComponent.SetSimulatePhysics` _staticmesh_3 true)
      (cast `/Game/Blueprints/Weapons/Weapons/WeaponBase` OtherActor)
      (`/Engine/EditorBlueprintResources/StandardMacros.IncrementInt` (`self.Counter`)
        (:`  `
          (`PrimitiveComponent.AddImpulse` _staticmesh (* (`SceneComponent.GetForwardVector` _staticmesh) -1000.0) "None" true))))))

(event `self.StaticMesh.OnComponentBeginOverlap`
  (params (OverlappedComponent :type "PrimitiveComponent Object Reference") (OtherActor :type "Actor Object Reference") (OtherComp :type "PrimitiveComponent Object Reference") (OtherBodyIndex :type Integer) (bFromSweep :type Boolean) (SweepResult :type "HitResult Structure (by ref)"))
  (goto _label))

(fn `UserConstructionScript`)