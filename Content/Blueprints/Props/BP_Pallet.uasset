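; BP_Pallet is a prop that procedurally builds a row or stack of pallet instances.
; Its construction script adds Instanced Static Mesh instances in a loop driven by Quantity, stepping location by a relative offset and applying a set rotation and fixed scale.
; An optional final instance gets an additional offset and its own rotation when DifferentLastItem is set.
; The event graph has no active logic.
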(fn `UserConstructionScript`
  (bind _palletetransform_location (`KismetMathLibrary.BreakTransform` (`self.PalleteTransform`)))
  (bind _palletetransform_location_2 (`KismetMathLibrary.BreakTransform` (`self.PalleteTransform`)))
  (for _ (range (+ (`self.Quantity`) 1))
    (`InstancedStaticMeshComponent.AddInstance` (`self.InstancedStaticMesh`) (`self.PalleteTransform`))
    (set `self.PalleteTransform` (`KismetMathLibrary.MakeTransform` (+ _palletetransform_location_2 (`self.PalleteRelLocation`)) (`self.PalleteRelRotation`) (4.0 4.0 4.0))))
  (if (`self.DifferentLastItem?`)
    (set `self.PalleteTransform` (`KismetMathLibrary.MakeTransform` (+ _palletetransform_location (`self.LastPalleteRelLocation`)) (`self.LastPalleteRelRotation`) (4.0 4.0 4.0)))
    (`InstancedStaticMeshComponent.AddInstance` (`self.InstancedStaticMesh`) (`self.PalleteTransform`))))