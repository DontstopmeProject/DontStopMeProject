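; Base Blueprint for interactable props, providing shared functions to prepare the player for an interaction.
; BeginInteract flags the player as in action, cancels active master time dilation by unpausing at normal speed, disables camera, cursor and target lock, then moves camera and cursor back.
; SetPosition snaps a character to the Arrow component's horizontal position, keeping its height, and matches control rotation to the arrow.
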(fn `BeginInteract`
  (bind _player (`self.Player`))
  (bind _player_2 (`self.Player`))
  (bind _cameracontrolcomponent (`/Game/Blueprints/PlayersCharacter.CameraControlComponent` _player))
  (`/Engine/EditorBlueprintResources/StandardMacros.IsValid` _player_2
    (:`Is Valid`
      (set `/Game/Blueprints/PlayersCharacter.Action` true _player_2)
      (bind _output_get (set `self.PlayerEnabledTimeDilation` (`/Game/Blueprints/PlayersCharacter.MasterEnableTimeDilation` _player_2)))
      (if _output_get
        (set `/Game/Blueprints/PlayersCharacter.MasterEnableTimeDilation` false _player_2)
        (`GameplayStatics.SetGamePaused` false)
        (`GameplayStatics.SetGlobalTimeDilation` 1.0))
      (set `/Game/Blueprints/PlayersComponents/CameraControlComponent.CanMoveCamera` false _cameracontrolcomponent)
      (set `/Game/Blueprints/PlayersComponents/CameraControlComponent.CanMoveCursor` false _cameracontrolcomponent)
      (set `/Game/Blueprints/PlayersComponents/LockTargetComponent.Lock` false (`/Game/Blueprints/PlayersCharacter.LockTargetComponent` _player))
      (`/Game/Blueprints/PlayersComponents/CameraControlComponent.MoveCameraBack` _cameracontrolcomponent (`/Game/Blueprints/PlayersCharacter.CameraMove` (`self.Player`)))
      (`/Game/Blueprints/PlayersComponents/CameraControlComponent.MoveCameraBack` _cameracontrolcomponent (`/Game/Blueprints/PlayersCharacter.Cursor` (`self.Player`)))
      (return))
    (:`Is Not Valid`
      (return))))

(fn `SetPosition`
  (params (Object :type "Actor Object Reference"))
  (bind _arrow (`self.Arrow`))
  (bind (_returnvalue_x _returnvalue_y) (`KismetMathLibrary.BreakVector` (`SceneComponent.K2_GetComponentLocation` _arrow)))
  (bind _asbase_character_class (cast `/Game/Blueprints/BaseCharacterClass` Object))
  (bind (_returnvalue_x_2 _returnvalue_y_2 _returnvalue_z) (`KismetMathLibrary.BreakVector` (`self.K2_GetActorLocation` _asbase_character_class)))
  (`self.K2_SetActorLocation` _asbase_character_class (`KismetMathLibrary.MakeVector` _returnvalue_x _returnvalue_y _returnvalue_z) false false)
  (`Controller.SetControlRotation` (`Pawn.GetController` _asbase_character_class) (`SceneComponent.K2_GetComponentRotation` _arrow)))

(fn `UserConstructionScript`)