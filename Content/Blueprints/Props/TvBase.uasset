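; TvBase is a TV prop actor that plays a looping video on its screen panel, with a configurable mesh, scale and light.
; The construction script applies appearance settings; at play, a media player feeds the panel and restarts on reaching the end.
; Tick copies the player character's time dilation, using paired DoOnce gates to pause playback during slow motion and resume it afterwards.
; An older text-and-picture slideshow with changing light color remains disconnected.
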(event `self.ReceiveBeginPlay`
  (`self.EventPlay`))

(event `EventPlay`
  (bind (_video_video _video_audio _video_mediaplayer) (break `/Game/Assets/Movies/VideoStructure` (`self.Video`)))
  (`MediaPlayer.OpenSource` _video_mediaplayer (`self.MediaSource`))
  (`MediaPlayer.Rewind` _video_mediaplayer)
  (`KismetSystemLibrary.Delay` 0.1)
  (`MediaPlayer.Play` _video_mediaplayer)
  (`PrimitiveComponent.SetMaterial` (`self.Panel`) 0 _video_video)
  (add `MediaPlayer.OnEndReached` _video_mediaplayer (delegate `OnEndReached_Event`)))

(event `OnEndReached_Event`
  (bind (_video_video _video_audio _video_mediaplayer) (break `/Game/Assets/Movies/VideoStructure` (`self.Video`)))
  (`MediaPlayer.Pause` _video_mediaplayer)
  (`self.EventPlay`))

(event `self.ReceiveTick`
  (params (DeltaSeconds :type "Float (single-precision)"))
  (bind _returnvalue (`GameplayStatics.GetPlayerCharacter` 0))
  (bind (_video_video _video_audio _video_mediaplayer) (break `/Game/Assets/Movies/VideoStructure` (`self.Video`)))
  (`/Engine/EditorBlueprintResources/StandardMacros.IsValid` _returnvalue
    (:`Is Valid`
      (bind _output_get (set `self.CustomTimeDilation` (`Actor.CustomTimeDilation` _returnvalue)))
      (if (< _output_get 1.0)
        (`/Engine/EditorBlueprintResources/StandardMacros.DoOnce` false :!label _label
          (:`Completed`
            (`MediaPlayer.Pause` _video_mediaplayer)
            (goto _label_2 :!via `Reset`)))
        (else
          (`/Engine/EditorBlueprintResources/StandardMacros.DoOnce` false :!label _label_2
            (:`Completed`
              (`MediaPlayer.Play` _video_mediaplayer)
              (goto _label :!via `Reset`))))))))

(event `EventChangeInfo`)

(fn `UserConstructionScript`
  (locals (NewLocalVar_0 :type "MaterialInterface Object Reference"))
  (bind _panel (`self.Panel`))
  (`LightComponent.SetIntensity` (`self.Light`) (`self.Intentsity`))
  (`StaticMeshComponent.SetStaticMesh` _panel (`self.TvMesh`))
  (`PrimitiveComponent.SetMaterial` _panel 0 (`self.TV picture`))
  (`SceneComponent.K2_SetRelativeLocationAndRotation` :`self` (`self.TextRender`))
  (`LightComponent.SetLightColor` (`self.Light`) (`self.LightColor`) true)
  (`SpotLightComponent.SetInnerConeAngle` (`self.Light`) (`self.InnerLightAngle`))
  (`TextRenderComponent.SetWorldSize` (`self.TextRender`) 0.0)
  (`SceneComponent.SetWorldScale3D` (`self.Panel`) (`self.MeshScale`)))