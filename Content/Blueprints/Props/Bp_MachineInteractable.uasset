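; One-shot interactable machine prop that plays a hack-style "sending" sequence when the player uses it.
; Interact disables the player's trace and time dilation, restores normal game speed and plays a button-push montage.
; A temporary console widget shows timed status messages, then a cutscene-finish dispatcher fires.
; Box overlap toggles a text prompt until the machine is used, and Tick yaws that text toward the player.
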(event `/Game/Blueprints/BlueprintInterfaces/BPI_Interact.Interact`
  (params (WhoInteracted :type "Actor Object Reference") (InteractedActor :type "Actor Object Reference") (UsedComponent :type "ActorComponent Object Reference"))
  (bind _asplayers_character (cast `/Game/Blueprints/PlayersCharacter` WhoInteracted :!pure true))
  (`/Engine/EditorBlueprintResources/StandardMacros.DoOnce` false
    (:`Completed`
      (set `self.Used` true)
      (set `/Game/Blueprints/BaseCharacterClass.Trace` false _asplayers_character)
      (set `/Game/Blueprints/PlayersCharacter.MasterEnableTimeDilation` false _asplayers_character)
      (`GameplayStatics.SetGlobalTimeDilation` 1.0)
      (`|PlayMontage` (`Character.Mesh` _asplayers_character) "/Game/Assets/AIBehaviorToolkit/Assets/Mannequin/Animations/AM_ButtonPush.AM_ButtonPush" 1.0 0.0 "spine_01"
        (:`then`
          (bind _returnvalue (`|CreateWidget` "/Game/Blueprints/Widgets/W_TestHackLine.W_TestHackLine_C"))
          (`UserWidget.AddToViewport` _returnvalue 0)
          (`/Game/Blueprints/Widgets/W_TestHackLine.event Console` _returnvalue "Sending...")
          (`KismetSystemLibrary.Delay` 5.0)
          (`/Game/Blueprints/Widgets/W_TestHackLine.event Console` _returnvalue "Sending complete!")
          (`KismetSystemLibrary.Delay` 2.0)
          (`Widget.RemoveFromParent` _returnvalue)
          (`self.FnishCutsceneDispatcher`)
          (`SceneComponent.SetVisibility` (`self.TextRender`) false false))))))

(event `self.ReceiveTick`
  (params (DeltaSeconds :type "Float (single-precision)"))
  (bind _textrender (`self.TextRender`))
  (bind (_returnvalue_roll _returnvalue_pitch _returnvalue_yaw) (`KismetMathLibrary.BreakRotator` (`KismetMathLibrary.FindLookAtRotation` (`SceneComponent.K2_GetComponentLocation` _textrender) (`self.K2_GetActorLocation` (`GameplayStatics.GetPlayerCharacter` 0)))))
  (`parent.ReceiveTick` DeltaSeconds)
  (`SceneComponent.K2_SetWorldRotation` _textrender (`KismetMathLibrary.MakeRotator` 0.0 35.0 _returnvalue_yaw) false false))

(event `self.Box.OnComponentBeginOverlap`
  (params (OverlappedComponent :type "PrimitiveComponent Object Reference") (OtherActor :type "Actor Object Reference") (OtherComp :type "PrimitiveComponent Object Reference") (OtherBodyIndex :type Integer) (bFromSweep :type Boolean) (SweepResult :type "HitResult Structure (by ref)"))
  (set `self.Actor` OtherActor)
  (if (not (`self.Used`))
    (`SceneComponent.SetVisibility` (`self.TextRender`) true false)))

(event `self.Box.OnComponentEndOverlap`
  (params (OverlappedComponent :type "PrimitiveComponent Object Reference") (OtherActor :type "Actor Object Reference") (OtherComp :type "PrimitiveComponent Object Reference") (OtherBodyIndex :type Integer))
  (set `self.Actor` null)
  (`SceneComponent.SetVisibility` (`self.TextRender`) false false))

(fn `UserConstructionScript`
  (`parent.UserConstructionScript`))