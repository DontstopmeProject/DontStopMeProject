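; Table prop that the player can vault and that breaks apart when damaged.
; Box hits or overlaps by tagged actors that are dead BaseCharacterClass characters apply damage; AnyDamage once swaps in a destructible component, enables physics on the part meshes and fires a radial impulse.
; Overlapping Box1 resets time dilation, blocks player input, starts the vault and disables collision; Tick waits for Vault to clear, then teleports the player to the Arrow's XY and restores collision.
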(event `self.ReceiveAnyDamage`
  (params (Damage :type "Float (single-precision)") (DamageType :type "DamageType Object Reference") (InstigatedBy :type "Controller Object Reference") (DamageCauser :type "Actor Object Reference"))
  (bind _staticmesh2 (`self.StaticMesh2`))
  (bind _platte (`self.Platte`))
  (`/Engine/EditorBlueprintResources/StandardMacros.DoOnce` false
    (:`Completed`
      (`ActorComponent.K2_DestroyComponent` (`self.Box`))
      (`StaticMeshComponent.SetStaticMesh` _platte null)
      (`AddComponent|NODE_AddDestructibleComponent-0` :`bManualAttachment` true :`RelativeTransform` (`SceneComponent.K2_GetComponentToWorld` _platte))
      (`PrimitiveComponent.SetSimulatePhysics` _staticmesh2 true)
      (`PrimitiveComponent.SetSimulatePhysics` (`self.StaticMesh3`) true)
      (`PrimitiveComponent.SetSimulatePhysics` (`self.StaticMesh4`) true)
      (`PrimitiveComponent.SetSimulatePhysics` (`self.StaticMesh5`) true)
      (`PrimitiveComponent.SetSimulatePhysics` (`self.StaticMesh6`) true)
      (`PrimitiveComponent.SetSimulatePhysics` (`self.ew`) true)
      (`PrimitiveComponent.SetSimulatePhysics` (`self.StaticMesh`) true)
      (`PrimitiveComponent.SetSimulatePhysics` (`self.StaticMesh4`) true)
      (`PrimitiveComponent.SetCollisionEnabled` _staticmesh2 "QueryAndPhysics")
      (`PrimitiveComponent.SetCollisionEnabled` (`self.StaticMesh3`) "QueryAndPhysics")
      (`PrimitiveComponent.SetCollisionEnabled` (`self.StaticMesh4`) "QueryAndPhysics")
      (`PrimitiveComponent.SetCollisionEnabled` (`self.StaticMesh5`) "QueryAndPhysics")
      (`PrimitiveComponent.SetCollisionEnabled` (`self.StaticMesh6`) "QueryAndPhysics")
      (`PrimitiveComponent.SetCollisionEnabled` (`self.ew`) "QueryAndPhysics")
      (`PrimitiveComponent.SetCollisionEnabled` (`self.StaticMesh`) "QueryAndPhysics")
      (`PrimitiveComponent.SetCollisionEnabled` (`self.StaticMesh4`) "QueryAndPhysics")
      (`ActorComponent.SetActive` (`self.RadialForce`) true false)
      (`RadialForceComponent.FireImpulse` (`self.RadialForce`)))))

(event `self.Box.OnComponentHit`
  (params (HitComponent :type "PrimitiveComponent Object Reference") (OtherActor :type "Actor Object Reference") (OtherComp :type "PrimitiveComponent Object Reference") (NormalImpulse :type "Vector Structure") (Hit :type "HitResult Structure (by ref)"))
  (if (or (`self.ActorHasTag` OtherActor "projectile") (and (`self.ActorHasTag` OtherActor "human") (or (`self.ActorHasTag` OtherActor "ai") (`self.ActorHasTag` OtherActor "player")))) :!label _label
    (bind _asbase_character_class (cast `/Game/Blueprints/BaseCharacterClass` OtherActor))
    (if (`/Game/Blueprints/BaseCharacterClass.Dead` _asbase_character_class)
      (`GameplayStatics.ApplyDamage` self 100.0 null OtherActor))))

(event `self.Box.OnComponentBeginOverlap`
  (params (OverlappedComponent :type "PrimitiveComponent Object Reference") (OtherActor :type "Actor Object Reference") (OtherComp :type "PrimitiveComponent Object Reference") (OtherBodyIndex :type Integer) (bFromSweep :type Boolean) (SweepResult :type "HitResult Structure (by ref)"))
  (goto _label))

(event `self.Box1.OnComponentBeginOverlap`
  (params (OverlappedComponent :type "PrimitiveComponent Object Reference") (OtherActor :type "Actor Object Reference") (OtherComp :type "PrimitiveComponent Object Reference") (OtherBodyIndex :type Integer) (bFromSweep :type Boolean) (SweepResult :type "HitResult Structure (by ref)"))
  (bind (_returnvalue_x _returnvalue_y) (`KismetMathLibrary.BreakVector` (`SceneComponent.K2_GetComponentLocation` (`self.Arrow`))))
  (bind _output_get (set `self.Actor` OtherActor))
  (bind _asplayers_character (cast `/Game/Blueprints/PlayersCharacter` _output_get))
  (set `self.action` true)
  (set `/Game/Blueprints/PlayersCharacter.MasterEnableTimeDilation` false _asplayers_character)
  (`GameplayStatics.SetGlobalTimeDilation` 1.0)
  (`/Game/Blueprints/PlayersCharacter.EventSetInput` _asplayers_character true true true true true true true true true)
  (set `/Game/Blueprints/PlayersCharacter.Vault` true _asplayers_character)
  (`PrimitiveComponent.SetCollisionEnabled` (`self.Box1`) "NoCollision")
  (`PrimitiveComponent.SetCollisionEnabled` (`self.Box`) "NoCollision")
  (goto _label_2 :!via `Reset`))

(event `self.ReceiveTick`
  (params (DeltaSeconds :type "Float (single-precision)"))
  (bind (_returnvalue_x _returnvalue_y) (`KismetMathLibrary.BreakVector` (`SceneComponent.K2_GetComponentLocation` (`self.Arrow`))))
  (bind _asplayers_character (cast `/Game/Blueprints/PlayersCharacter` (`self.Actor`)))
  (if (not (`/Game/Blueprints/PlayersCharacter.Vault` _asplayers_character))
    (`/Engine/EditorBlueprintResources/StandardMacros.DoOnce` false :!label _label_2
      (:`Completed`
        (bind (_returnvalue_x_2 _returnvalue_y_2 _returnvalue_z) (`KismetMathLibrary.BreakVector` (`self.K2_GetActorLocation` _asplayers_character)))
        (`self.K2_SetActorLocation` _asplayers_character (`KismetMathLibrary.MakeVector` _returnvalue_x _returnvalue_y _returnvalue_z) false true)
        (`PrimitiveComponent.SetCollisionEnabled` (`self.Box1`) "QueryAndPhysics")
        (`PrimitiveComponent.SetCollisionEnabled` (`self.Box`) "QueryAndPhysics")))))

(event `self.Box2.OnComponentBeginOverlap`
  (params (OverlappedComponent :type "PrimitiveComponent Object Reference") (OtherActor :type "Actor Object Reference") (OtherComp :type "PrimitiveComponent Object Reference") (OtherBodyIndex :type Integer) (bFromSweep :type Boolean) (SweepResult :type "HitResult Structure (by ref)"))
  (set `self.NewVar_0` SweepResult_Location))

(fn `UserConstructionScript`)