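; Prop Blueprint that scatters randomly placed document meshes, built in the construction script with no active event logic.
; It adds hierarchical instanced static mesh instances in a loop over NumberOfDocs, keeping the first at the origin and randomly offsetting and rotating the rest.
; A second loop creates dynamic material instances from Material, passing the loop index as the material element index, which addresses slots rather than individual instances.
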(fn `UserConstructionScript`
  (for _index (range (+ (`self.Number of docs`) 1))
    (if (> _index 0)
      (set `self.Transform` (`KismetMathLibrary.MakeTransform` (`KismetMathLibrary.MakeVector` (`KismetMathLibrary.RandomFloatInRange` -150.0 150.0) (`KismetMathLibrary.RandomFloatInRange` -150.0 150.0) (`KismetMathLibrary.RandomFloatInRange` 0.0 10.0)) (`KismetMathLibrary.MakeRotator` 0.0 0.0 (`KismetMathLibrary.RandomFloatInRange` -15.0 15.0))))
      (else
        (set `self.Transform` (`KismetMathLibrary.MakeTransform` (0.0 0.0 0.0)))))
    (`InstancedStaticMeshComponent.AddInstance` (`self.HierarchicalInstancedStaticMesh`) (`self.Transform`))
    (set `self.Transform` (`KismetMathLibrary.MakeTransform` (0.0 0.0 0.0))))
  (for _index_2 (range (+ (`self.Number of docs`) 1))
    (`PrimitiveComponent.CreateDynamicMaterialInstance` (`self.HierarchicalInstancedStaticMesh`) _index_2 (`self.Material`))))