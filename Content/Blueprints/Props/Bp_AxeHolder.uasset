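; Wall or prop axe holder with a glass pane that shatters when the actor takes damage or its axe child actor is no longer valid.
; Tick watches the axe through a DoOnce, and AnyDamage calls the same SpawnGlassBroken function, guarded by a Broken flag.
; That function adds destructible and radial force components at the glass's relative transform, fires an impulse, then destroys the intact glass component.
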(event `self.ReceiveTick`
  (params (DeltaSeconds :type "Float (single-precision)"))
  (`/Engine/EditorBlueprintResources/StandardMacros.IsValid` (`ChildActorComponent.ChildActor` (`self.Axe`))
    (:`Is Not Valid`
      (`/Engine/EditorBlueprintResources/StandardMacros.DoOnce` false
        (:`Completed`
          (`self.SpawnGlassBroken`))))))

(event `self.ReceiveAnyDamage`
  (params (Damage :type "Float (single-precision)") (DamageType :type "DamageType Object Reference") (InstigatedBy :type "Controller Object Reference") (DamageCauser :type "Actor Object Reference"))
  (`self.SpawnGlassBroken`))

(fn `SpawnGlassBroken`
  (bind _returnvalue (`SceneComponent.GetRelativeTransform` (`self.Glass`)))
  (if (not (`self.Broken`))
    (set `self.Broken` true)
    (`AddComponent|NODE_AddDestructibleComponent-1` :`RelativeTransform` _returnvalue)
    (bind _returnvalue_2 (`AddComponent|NODE_AddRadialForceComponent-1` :`RelativeTransform` _returnvalue))
    (`RadialForceComponent.FireImpulse` _returnvalue_2)
    (`ActorComponent.K2_DestroyComponent` (`self.Glass`))))

(fn `UserConstructionScript`)