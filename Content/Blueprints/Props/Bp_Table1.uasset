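; Breakable table prop that shatters the first time it takes any damage.
; Box hit and overlap events share a check on projectile or human AI/player tags, then apply damage to the table only if the other actor casts to BaseCharacterClass and is dead.
; A DoOnce on damage destroys the box, clears the static mesh, spawns a destructible component at its transform and fires a radial force impulse.
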(event `self.ReceiveTick`
  (params (DeltaSeconds :type "Float (single-precision)")))

(event `self.ReceiveAnyDamage`
  (params (Damage :type "Float (single-precision)") (DamageType :type "DamageType Object Reference") (InstigatedBy :type "Controller Object Reference") (DamageCauser :type "Actor Object Reference"))
  (bind _staticmesh (`self.StaticMesh`))
  (`/Engine/EditorBlueprintResources/StandardMacros.DoOnce` false
    (:`Completed`
      (`ActorComponent.K2_DestroyComponent` (`self.Box`))
      (`StaticMeshComponent.SetStaticMesh` _staticmesh null)
      (`AddComponent|NODE_AddDestructibleComponent-0` :`bManualAttachment` true :`RelativeTransform` (`SceneComponent.K2_GetComponentToWorld` _staticmesh))
      (`ActorComponent.SetActive` (`self.RadialForce`) true false)
      (`RadialForceComponent.FireImpulse` (`self.RadialForce`)))))

(event `self.Box.OnComponentHit`
  (params (HitComponent :type "PrimitiveComponent Object Reference") (OtherActor :type "Actor Object Reference") (OtherComp :type "PrimitiveComponent Object Reference") (NormalImpulse :type "Vector Structure") (Hit :type "HitResult Structure (by ref)"))
  (if (or (`self.ActorHasTag` OtherActor "projectile") (and (`self.ActorHasTag` OtherActor "human") (or (`self.ActorHasTag` OtherActor "ai") (`self.ActorHasTag` OtherActor "player")))) :!label _label
    (bind _asbase_character_class (cast `/Game/Blueprints/BaseCharacterClass` OtherActor))
    (if (`/Game/Blueprints/BaseCharacterClass.Dead` _asbase_character_class)
      (`GameplayStatics.ApplyDamage` self 100.0 null OtherActor))))

(event `self.Box.OnComponentBeginOverlap`
  (params (OverlappedComponent :type "PrimitiveComponent Object Reference") (OtherActor :type "Actor Object Reference") (OtherComp :type "PrimitiveComponent Object Reference") (OtherBodyIndex :type Integer) (bFromSweep :type Boolean) (SweepResult :type "HitResult Structure (by ref)"))
  (goto _label))

(fn `UserConstructionScript`)