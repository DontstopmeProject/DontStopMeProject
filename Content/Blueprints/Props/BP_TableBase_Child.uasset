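; BP_TableBase_Child is a table prop Blueprint, apparently prototyping matching of hit components to destructible meshes.
; The construction script runs the parent's, then fills MeshesArray with the chair, phone, calculator and other entries.
; On Hit, components other than StaticMesh have the first underscore-delimited name token compared against every token in DestructableMeshes names.
; A match only prints a debug "Hello", with no destruction logic here.
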(event `self.ReceiveBeginPlay`
  (`parent.ReceiveBeginPlay`))

(event `self.ReceiveHit`
  (params (MyComp :type "PrimitiveComponent Object Reference") (Other :type "Actor Object Reference") (OtherComp :type "PrimitiveComponent Object Reference") (bSelfMoved :type Boolean) (HitLocation :type "Vector Structure") (HitNormal :type "Vector Structure") (NormalImpulse :type "Vector Structure") (Hit :type "HitResult Structure (by ref)"))
  (if (!= MyComp (`self.StaticMesh`))
    (set `self.StaticNameArray` (`KismetStringLibrary.ParseIntoArray` (`KismetSystemLibrary.GetObjectName` MyComp) "_"))
    (for _array_element (`self.DestructableMeshes`)
      (bind _output_get (set `self.DestructableNameArray` (`KismetStringLibrary.ParseIntoArray` (`KismetSystemLibrary.GetObjectName` _array_element) "_")))
      (for _array_element_2 _output_get
        (if (`KismetStringLibrary.EqualEqual_StrStr` (`|GetArrayItem` (`self.StaticNameArray`)) _array_element_2)
          (`KismetSystemLibrary.PrintString` "Hello"))))))

(fn `UserConstructionScript`
  (`parent.UserConstructionScript`)
  (set `self.MeshesArray` (`|MakeArray` (`self.ChairMesh`) (`self.Phone`) (`self.Calculator`) null :!type "SceneComponent Object Reference")))