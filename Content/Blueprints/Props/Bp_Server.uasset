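; Server rack prop that gives destruction feedback when struck or touched.
; The construction script stacks server meshes vertically according to OverallServers, each with a random material from MaterialsArray.
; Weapon or projectile hits and any Box1 overlap share one effect path: a random destruction sound plus briefly attached sparks at the contact position.
; A separate Destroy function only removes the first PartAArray entry and is not called in this graph.
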(event `self.ReceiveHit`
  (params (MyComp :type "PrimitiveComponent Object Reference") (Other :type "Actor Object Reference") (OtherComp :type "PrimitiveComponent Object Reference") (bSelfMoved :type Boolean) (HitLocation :type "Vector Structure") (HitNormal :type "Vector Structure") (NormalImpulse :type "Vector Structure") (Hit :type "HitResult Structure (by ref)"))
  (bind _hitlocation_0 (`self.HitLocation_0`))
  (cast `/Game/Blueprints/Weapons/Weapons/WeaponBase` Other
    (:`then`
      _)
    (:`CastFailed`
      (cast `/Game/Blueprints/Weapons/projectiles/BP_ProjectileBase` Other)))
  (set `self.HitLocation_0` HitLocation)
  (`GameplayStatics.PlaySoundAtLocation` (select `bool` (`KismetMathLibrary.RandomBool`) :`false` "/Game/Assets/Sounds/Effects/DestructionSounds/Technics/destraction_technics_v3__mp3cut_net_.destraction_technics_v3__mp3cut_net_" :`true` "/Game/Assets/Sounds/Effects/DestructionSounds/Technics/destruct_technic__v2_.destruct_technic__v2_" :!type "SoundBase Object Reference") _hitlocation_0 (struct) 10.0 1.0 0.0 "/Game/Blueprints/SoundBlueprints/SoundAttenuationSettings.SoundAttenuationSettings" :!label _label)
  (bind _returnvalue (`GameplayStatics.SpawnEmitterAttached` "/Game/Assets/StarterContent/Particles/P_Sparks.P_Sparks" (`self.Box_0`) "None" _hitlocation_0 (struct) (1.0 1.0 1.0) "KeepWorldPosition"))
  (`KismetSystemLibrary.Delay` 0.2)
  (`ActorComponent.K2_DestroyComponent` _returnvalue))

(event `self.Box1.OnComponentBeginOverlap`
  (params (OverlappedComponent :type "PrimitiveComponent Object Reference") (OtherActor :type "Actor Object Reference") (OtherComp :type "PrimitiveComponent Object Reference") (OtherBodyIndex :type Integer) (bFromSweep :type Boolean) (SweepResult :type "HitResult Structure (by ref)"))
  (`/Engine/EditorBlueprintResources/StandardMacros.IsValid` OtherComp
    (:`Is Valid`
      (set `self.Hit` false)
      (set `self.HitLocation_0` (`SceneComponent.K2_GetComponentLocation` OtherComp))
      (goto _label))))

(fn `Destroy`
  (`KismetArrayLibrary.Array_Remove` (`self.PartAArray`)))

(fn `UserConstructionScript`
  (for _ (range (+ (`self.OverallServers`) 1))
    (set `self.transform` (`KismetMathLibrary.MakeTransform` (`KismetMathLibrary.MakeVector` 0.0 -100.0 (`self.ZValue`)) (struct) (1.3 1.0 1.0)))
    (bind _returnvalue (`AddComponent|NODE_AddStaticMeshComponent-0` :`RelativeTransform` (`self.transform`)))
    (`PrimitiveComponent.SetMaterial` _returnvalue 0 (`|GetArrayItem` (`self.MaterialsArray`) (`KismetMathLibrary.RandomIntegerInRange` 0 4)))
    (set `self.ZValue` (+ (`self.ZValue`) 50.0))))