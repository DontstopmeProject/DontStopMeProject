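; BP_PropsDestructable is a prop that reacts destructively when its detection box is overlapped or a projectile hits it.
; Either trigger enables mesh physics and calls PlayDestructionSounds with a random sound and an emitter.
; Weapons and projectiles also apply a radial impulse plus their own impulse along the owning player mesh's right vector.
; The Broken flag is never set, so nothing here blocks retriggering.
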(event `EventDestroy`
  (params (HiActor :type "Actor Object Reference") (Hit :type "HitResult Structure"))
  (bind _hit_actor (`self.Hit Actor`))
  (bind _emmiterspawnlocation (`self.EmmiterSpawnLocation`))
  (bind _hitlocation (`self.HitLocation`))
  (bind _staticmesh (`self.StaticMesh`))
  (bind _destructionsounds (`self.DestructionSounds`))
  (bind _returnvalue (`self.GetParentActor` _hit_actor))
  (bind (_asweapon_base _bsuccess) (cast `/Game/Blueprints/Weapons/Weapons/WeaponBase` (`self.Hit Actor`) :!pure true))
  (set `self.Hit Actor` HiActor)
  (set `self.HitLocation` Hit_Location)
  (set `self.NormalImpulse` Hit_Normal)
  (`PrimitiveComponent.SetSimulatePhysics` (`self.StaticMesh`) true)
  (if (or (`.bSuccess` (cast `/Game/Blueprints/Weapons/projectiles/BP_ProjectileBase` (`self.Hit Actor`) :!pure true)) (`.bSuccess` (cast `/Game/Blueprints/Weapons/Weapons/WeaponBase` (`self.Hit Actor`) :!pure true)))
    (`PrimitiveComponent.AddImpulse` (`self.StaticMesh`) (* (`SceneComponent.GetRightVector` (`Character.Mesh` (cast `/Game/Blueprints/PlayersCharacter` (`KismetMathLibrary.SelectObject` _returnvalue (`self.GetOwner` _hit_actor) (`KismetSystemLibrary.IsValid` _returnvalue)) :!pure true))) (select `bool` _bsuccess :`false` (`/Game/Blueprints/Weapons/projectiles/BP_ProjectileBase.HitPropsImpulseProjectiles` (cast `/Game/Blueprints/Weapons/projectiles/BP_ProjectileBase` (`self.Hit Actor`) :!pure true)) :`true` (`/Game/Blueprints/Weapons/Weapons/WeaponBase.HitPropsImpulse` _asweapon_base))) "None" true)
    (`PrimitiveComponent.AddRadialImpulse` _staticmesh (`SceneComponent.K2_GetComponentLocation` _staticmesh) 10.0 500.0 "RIF_Constant" true))
  (`self.PlayDestructionSounds` _hitlocation (select `bool` (!= _emmiterspawnlocation (-1.0 -1.0 -1.0) :`ErrorTolerance` 1.0) :`false` _hitlocation :`true` _emmiterspawnlocation) (`self.EmmiterScale`) (`self.Emmiter`) (`self.ComponentAttachTo`) (`self.DestroyEmmiterOnTimer`) 0.0 (`|GetArrayItem` _destructionsounds (`KismetMathLibrary.RandomIntegerInRange` 0 (`KismetArrayLibrary.Array_LastIndex` _destructionsounds)))))

(event `self.DamageDetectionBox.OnComponentBeginOverlap`
  (params (OverlappedComponent :type "PrimitiveComponent Object Reference") (OtherActor :type "Actor Object Reference") (OtherComp :type "PrimitiveComponent Object Reference") (OtherBodyIndex :type Integer) (bFromSweep :type Boolean) (SweepResult :type "HitResult Structure (by ref)"))
  (`self.EventDestroy` OtherActor SweepResult))

(event `self.ReceiveHit`
  (params (MyComp :type "PrimitiveComponent Object Reference") (Other :type "Actor Object Reference") (OtherComp :type "PrimitiveComponent Object Reference") (bSelfMoved :type Boolean) (HitLocation :type "Vector Structure") (HitNormal :type "Vector Structure") (NormalImpulse :type "Vector Structure") (Hit :type "HitResult Structure (by ref)"))
  (cast `/Game/Blueprints/Weapons/projectiles/BP_ProjectileBase` Other)
  (`self.EventDestroy` Other (`GameplayStatics.MakeHitResult` Hit_bBlockingHit Hit_bInitialOverlap Hit_Time Hit_Distance Hit_Location Hit_ImpactPoint Hit_Normal Hit_ImpactNormal Hit_PhysMat Hit_HitActor Hit_HitComponent Hit_HitBoneName Hit_HitItem Hit_FaceIndex Hit_TraceStart Hit_TraceEnd)))

(fn `UserConstructionScript`
  (set `self.ComponentAttachTo` (`self.StaticMesh`)))