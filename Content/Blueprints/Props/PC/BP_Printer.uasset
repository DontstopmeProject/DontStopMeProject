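; BP_Printer is a PC prop that carries a WeaponBase child actor and reacts to damage and destruction.
; On BeginPlay it hands that weapon a backup pickup actor and binds a Destructed event, which swaps the Comput2erIkranLow mesh to a shattered-glass material.
; Any damage received is forwarded to the child actor as a fixed amount, regardless of the incoming value.
; The construction script snaps the Comput2erSystemLow component onto its attach parent.
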(event `self.ReceiveBeginPlay`
  (set `/Game/Blueprints/Weapons/Weapons/WeaponBase.BackUpWeaponPickupActor` (`self.BackupActorToPickUpWeapons`) (cast `/Game/Blueprints/Weapons/Weapons/WeaponBase` (`ChildActorComponent.ChildActor` (`self.ChildActor`)) :!pure true))
  (add `self.Destructed` (delegate `Destructed_Event`)))

(event `Destructed_Event`
  (`PrimitiveComponent.SetMaterial` (`self.comput2er_Ikran_low`) 0 "/Game/Assets/M_Orzelek_Assets/Materials/Free/Glass/M_GlassShattered_Master.M_GlassShattered_Master"))

(event `self.ReceiveAnyDamage`
  (params (Damage :type "Float (single-precision)") (DamageType :type "DamageType Object Reference") (InstigatedBy :type "Controller Object Reference") (DamageCauser :type "Actor Object Reference"))
  (`GameplayStatics.ApplyDamage` (`ChildActorComponent.ChildActor` (`self.ChildActor`)) 100.0 InstigatedBy DamageCauser))

(fn `UserConstructionScript`
  (`SceneComponent.K2_AttachToComponent` (`self.comput2er_system_low`) null "None" "SnapToTarget" "KeepWorld" "KeepWorld" true)
  (`SceneComponent.K2_AttachToComponent` (`self.comput2er_system_low`) null "None" "SnapToTarget" "KeepWorld" "KeepWorld" true)
  (set `self.ComponentAttachTo` (`self.StaticMesh`)))