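; Computer prop with a breakable monitor and an attached keyboard that is also a weapon.
; On BeginPlay it spawns BP_Keyboard, attaches it at a fixed offset and passes it a backup weapon pickup actor.
; A bound Destructed event swaps the monitor material to shattered glass.
; Damage to the computer is forwarded to the keyboard only when the keyboard has a valid owner that is not a BaseCharacterClass.
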(event `self.ReceiveBeginPlay`
  (`|ExecutionSequence`
    (:`then_0`
      (bind _returnvalue (`|SpawnActorFromClass` "/Game/Blueprints/Weapons/Weapons/Melee/BP_Keyboard.BP_Keyboard_C" (`KismetMathLibrary.MakeTransform` (0.0 10000.0 10000.0)) "Undefined" "OverrideRootScale" null null))
      (bind _output_get (set `self.Keyboard` _returnvalue))
      (`self.K2_AttachToActor` _output_get self "None" "KeepRelative" "KeepRelative" "KeepRelative" true)
      (`self.K2_SetActorRelativeTransform` (`self.Keyboard`) (`KismetMathLibrary.MakeTransform` (14.139326 38.137573 27.671717) (struct :`Yaw` 66.140045 :`Roll` 125.105316) (2.0 2.0 2.0)) false true))
    (:`then_1`
      (set `/Game/Blueprints/Weapons/Weapons/WeaponBase.BackUpWeaponPickupActor` (`self.BackupActorToPickUpWeapons`) (cast `/Game/Blueprints/Weapons/Weapons/WeaponBase` (`self.Keyboard`) :!pure true))
      (add `self.Destructed` (delegate `Destructed_Event`)))))

(event `Destructed_Event`
  (`PrimitiveComponent.SetMaterial` (`self.comput2er_Ikran_low`) 0 "/Game/Assets/M_Orzelek_Assets/Materials/Free/Glass/M_GlassShattered_Master.M_GlassShattered_Master"))

(event `self.ReceiveAnyDamage`
  (params (Damage :type "Float (single-precision)") (DamageType :type "DamageType Object Reference") (InstigatedBy :type "Controller Object Reference") (DamageCauser :type "Actor Object Reference"))
  (bind _keyboard (`self.Keyboard`))
  (bind _returnvalue (`self.GetOwner` _keyboard))
  (`/Engine/EditorBlueprintResources/StandardMacros.IsValid` _returnvalue
    (:`Is Valid`
      (cast `/Game/Blueprints/BaseCharacterClass` _returnvalue
        (:`CastFailed`
          (`GameplayStatics.ApplyDamage` _keyboard 100.0 InstigatedBy DamageCauser))))))

(fn `UserConstructionScript`
  (set `self.ComponentAttachTo` (`self.StaticMesh`)))