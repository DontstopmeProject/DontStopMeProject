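; Destructible-looking server prop that reacts with sparks and sound when struck by projectiles or weapons.
; The construction script stacks OverallServers mesh components vertically, each with a random material.
; BulletBox hits from BP_ProjectileBase and Box overlaps from WeaponBase call PlayDestructionSounds with a random sound and spark emitter at the impact.
; Older inline effect logic is disconnected, and Destroy only removes the first PartAArray entry.
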(event `self.Box1.OnComponentBeginOverlap`
  (params (OverlappedComponent :type "PrimitiveComponent Object Reference") (OtherActor :type "Actor Object Reference") (OtherComp :type "PrimitiveComponent Object Reference") (OtherBodyIndex :type Integer) (bFromSweep :type Boolean) (SweepResult :type "HitResult Structure (by ref)")))

(event `self.ReceiveHit`
  (params (MyComp :type "PrimitiveComponent Object Reference") (Other :type "Actor Object Reference") (OtherComp :type "PrimitiveComponent Object Reference") (bSelfMoved :type Boolean) (HitLocation :type "Vector Structure") (HitNormal :type "Vector Structure") (NormalImpulse :type "Vector Structure") (Hit :type "HitResult Structure (by ref)")))

(event `self.BulletBox.OnComponentHit`
  (params (HitComponent :type "PrimitiveComponent Object Reference") (OtherActor :type "Actor Object Reference") (OtherComp :type "PrimitiveComponent Object Reference") (NormalImpulse :type "Vector Structure") (Hit :type "HitResult Structure (by ref)"))
  (bind _sound (`self.Sound`))
  (cast `/Game/Blueprints/Weapons/projectiles/BP_ProjectileBase` OtherActor)
  (`self.PlayDestructionSounds` Hit_Location Hit_Location (3.0 3.0 3.0) "/Game/Assets/StarterContent/Particles/P_Sparks.P_Sparks" HitComponent true 1.0 (`|GetArrayItem` _sound (`KismetMathLibrary.RandomIntegerInRange` 0 (`KismetArrayLibrary.Array_LastIndex` _sound)))))

(event `self.Box.OnComponentBeginOverlap`
  (params (OverlappedComponent :type "PrimitiveComponent Object Reference") (OtherActor :type "Actor Object Reference") (OtherComp :type "PrimitiveComponent Object Reference") (OtherBodyIndex :type Integer) (bFromSweep :type Boolean) (SweepResult :type "HitResult Structure (by ref)"))
  (bind _sound (`self.Sound`))
  (cast `/Game/Blueprints/Weapons/Weapons/WeaponBase` OtherActor)
  (`self.PlayDestructionSounds` SweepResult_Location SweepResult_Location (3.0 3.0 3.0) "/Game/Assets/StarterContent/Particles/P_Sparks.P_Sparks" OverlappedComponent true 1.0 (`|GetArrayItem` _sound (`KismetMathLibrary.RandomIntegerInRange` 0 (`KismetArrayLibrary.Array_LastIndex` _sound)))))

(fn `Destroy`
  (`KismetArrayLibrary.Array_Remove` (`self.PartAArray`)))

(fn `UserConstructionScript`
  (for _ (range (+ (`self.OverallServers`) 1))
    (set `self.transform` (`KismetMathLibrary.MakeTransform` (`KismetMathLibrary.MakeVector` 0.0 -100.0 (`self.ZValue`)) (struct) (1.3 1.0 1.0)))
    (bind _returnvalue (`AddComponent|NODE_AddStaticMeshComponent-0` :`RelativeTransform` (`self.transform`)))
    (`PrimitiveComponent.SetMaterial` _returnvalue 0 (`|GetArrayItem` (`self.MaterialsArray`) (`KismetMathLibrary.RandomIntegerInRange` 0 4)))
    (set `self.ZValue` (+ (`self.ZValue`) 50.0))))