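; Base push-button prop that the player activates once, firing a Pushed dispatcher for other logic to react to.
; Capsule overlap shows a prompt and binds the push to the character's use dispatcher; leaving hides the prompt without unbinding.
; Pushing removes prompt and collision, suspends time dilation, and locks the character during a montage.
; After a delay it fires Pushed, unbinds, unlocks the character and restores the time-dilation flag.
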(event `self.Capsule.OnComponentBeginOverlap`
  (params (OverlappedComponent :type "PrimitiveComponent Object Reference") (OtherActor :type "Actor Object Reference") (OtherComp :type "PrimitiveComponent Object Reference") (OtherBodyIndex :type Integer) (bFromSweep :type Boolean) (SweepResult :type "HitResult Structure (by ref)"))
  (if (and (`self.ActorHasTag` OtherActor "player") (not (`self.Used`)))
    (`SceneComponent.SetVisibility` (`self.TextRender`) true true)
    (bind _asplayers_character (cast `/Game/Blueprints/PlayersCharacter` OtherActor))
    (add `/Game/Blueprints/PlayersCharacter.UseDispatcher` _asplayers_character (delegate `EventPushTheButton`))
    (set `self.CharacterOverlapped` _asplayers_character)))

(event `EventPushTheButton`
  (bind _textrender (`self.TextRender`))
  (bind _characteroverlapped (`self.CharacterOverlapped`))
  (bind _characteroverlapped_2 (`self.CharacterOverlapped`))
  (bind _asplayers_character (cast `/Game/Blueprints/PlayersCharacter` (`GameplayStatics.GetPlayerCharacter` 0)))
  (if (`/Game/Blueprints/PlayersCharacter.MasterEnableTimeDilation` _asplayers_character)
    (set `self.TimeVar` true)
    (set `/Game/Blueprints/PlayersCharacter.MasterEnableTimeDilation` false _asplayers_character)
    (`GameplayStatics.SetGamePaused` false)
    (`GameplayStatics.SetGlobalTimeDilation` 1.0)
    (else
      (set `self.TimeVar` false)))
  (set `/Game/Blueprints/PlayersCharacter.Action` true _asplayers_character)
  (set `/Game/Blueprints/PlayersCharacter.BlockMovements` true _characteroverlapped_2)
  (set `/Game/Blueprints/PlayersCharacter.BlockActions` true _characteroverlapped_2)
  (`/Engine/EditorBlueprintResources/StandardMacros.IsValid` _textrender
    (:`Is Valid`
      (`ActorComponent.K2_DestroyComponent` _textrender))
    (:`Is Not Valid`
      _))
  (`PrimitiveComponent.SetCollisionEnabled` (`self.Capsule`) "NoCollision")
  (`Character.PlayAnimMontage` (`self.CharacterOverlapped`) "/Game/Assets/AIBehaviorToolkit/Assets/Mannequin/Animations/AM_ButtonPush.AM_ButtonPush" 1.0 "spine_01")
  (`KismetSystemLibrary.Delay` 1.0)
  (`self.PushedDispatcher`)
  (remove `/Game/Blueprints/PlayersCharacter.UseDispatcher` (`self.CharacterOverlapped`) (delegate `EventPushTheButton`))
  (set `/Game/Blueprints/PlayersCharacter.BlockMovements` false _characteroverlapped)
  (set `/Game/Blueprints/PlayersCharacter.BlockActions` false _characteroverlapped)
  (bind _asplayers_character_2 (cast `/Game/Blueprints/PlayersCharacter` (`GameplayStatics.GetPlayerCharacter` 0)))
  (set `/Game/Blueprints/PlayersCharacter.Action` false _asplayers_character_2)
  (if (`self.TimeVar`)
    (set `/Game/Blueprints/PlayersCharacter.MasterEnableTimeDilation` true _asplayers_character_2)))

(event `self.Capsule.OnComponentEndOverlap`
  (params (OverlappedComponent :type "PrimitiveComponent Object Reference") (OtherActor :type "Actor Object Reference") (OtherComp :type "PrimitiveComponent Object Reference") (OtherBodyIndex :type Integer))
  (bind _textrender (`self.TextRender`))
  (if (and (`self.ActorHasTag` OtherActor "player") (not (`self.Used`)))
    (`/Engine/EditorBlueprintResources/StandardMacros.IsValid` _textrender
      (:`Is Valid`
        (`SceneComponent.SetVisibility` _textrender false true)))))

(fn `UserConstructionScript`
  (`TextRenderComponent.K2_SetText` (`self.TextRender`) (`self.Text`)))