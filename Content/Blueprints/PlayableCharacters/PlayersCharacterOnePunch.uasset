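; Player character variant that gives melee attacks very high damage, as a one-punch character.
; It raises damage on the held melee item and left-hand arms a second after spawn and again, after a short delay, on pickup events.
; The pickup refresh also raises the melee item's self-attack damage.
; On BeginPlay it adds pistol, shotgun, SMG and ricochet pistol to the chosen-weapons game mode's list, if that mode is active.
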(event `SetArmsDamage`
  (`KismetSystemLibrary.Delay` 0.2)
  (bind _asmelee_base (cast `/Game/Blueprints/Weapons/Weapons/Melee/BaseWeaponsMelee/MeleeBase` (`ChildActorComponent.ChildActor` (`self.PickableItem`)))
    (:`then`
      (set `/Game/Blueprints/Weapons/Weapons/Melee/BaseWeaponsMelee/MeleeBase.AttackDamage` 100.0 _asmelee_base)
      (set `/Game/Blueprints/Weapons/Weapons/Melee/BaseWeaponsMelee/MeleeBase.SelfAttackDamage` 100.0 _asmelee_base))
    (:`CastFailed`
      _))
  (bind _asbp_arms (cast `/Game/Blueprints/Weapons/Weapons/Melee/BP_Arms` (`ChildActorComponent.ChildActor` (`self.PickableItemL`))))
  (set `/Game/Blueprints/Weapons/Weapons/Melee/BaseWeaponsMelee/MeleeBase.AttackDamage` 100.0 _asbp_arms))

(event `self.ReceiveBeginPlay`
  (`parent.ReceiveBeginPlay`)
  (add `self.PickEventDispatcher` (delegate `SetArmsDamage`))
  (add `self.PlayerPickUpDispatcher` (delegate `SetArmsDamage`))
  (bind _asonly_chosen_weapns_gm (cast `/Game/Blueprints/OnlyCHosenWeapnsGM` (`GameplayStatics.GetGameMode`))
    (:`then`
      (bind _weapons (`/Game/Blueprints/OnlyCHosenWeapnsGM.Weapons` _asonly_chosen_weapns_gm))
      (`KismetArrayLibrary.Array_Add` _weapons "/Game/Blueprints/Weapons/Weapons/Fire/BP_Pistol.BP_Pistol_C")
      (`KismetArrayLibrary.Array_Add` _weapons "/Game/Blueprints/Weapons/Weapons/Fire/BP_Shotgun.BP_Shotgun_C")
      (`KismetArrayLibrary.Array_Add` _weapons "/Game/Blueprints/Weapons/Weapons/Fire/BP_SM_Ap5.BP_SM_Ap5_C")
      (`KismetArrayLibrary.Array_Add` _weapons "/Game/Blueprints/Weapons/Weapons/Fire/BP_RicohetPistol1.BP_RicohetPistol1_C"))
    (:`CastFailed`
      _))
  (`KismetSystemLibrary.Delay` 1.0)
  (bind _asmelee_base (cast `/Game/Blueprints/Weapons/Weapons/Melee/BaseWeaponsMelee/MeleeBase` (`ChildActorComponent.ChildActor` (`self.PickableItem`)))
    (:`then`
      (set `/Game/Blueprints/Weapons/Weapons/Melee/BaseWeaponsMelee/MeleeBase.AttackDamage` 100.0 _asmelee_base))
    (:`CastFailed`
      _))
  (bind _asbp_arms (cast `/Game/Blueprints/Weapons/Weapons/Melee/BP_Arms` (`ChildActorComponent.ChildActor` (`self.PickableItemL`))))
  (set `/Game/Blueprints/Weapons/Weapons/Melee/BaseWeaponsMelee/MeleeBase.AttackDamage` 100.0 _asbp_arms))

(fn `UserConstructionScript`
  (`parent.UserConstructionScript`))