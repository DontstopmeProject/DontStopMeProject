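; Playable Hacker character Blueprint that adds a hack-tracking toggle on top of its parent character.
; Pressing Dodge while unpaused calls the skip dispatcher, then flips StartTracking on the HackPlayerComponent if it is ReadyToTrack.
; BeginPlay and construction defer to the parent, Tick is disabled, and an unconnected leftover chain would add two weapons to the OnlyChosenWeapnsGM game mode.
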(event `self.ReceiveBeginPlay`
  (`parent.ReceiveBeginPlay`))

(event `InputAction|Dodge`
  (params (Key :type "Key Structure"))
  (bind _hackplayercomponent (`self.HackPlayerComponent`))
  (:`Pressed`
    (if (not (`self.GamePaused`))
      (`self.SkipDispatcher`)
      (if (`/Game/Blueprints/PlayersComponents/HackPlayerComponent.ReadyToTrack` _hackplayercomponent)
        (if (`/Game/Blueprints/PlayersComponents/HackPlayerComponent.StartTracking` _hackplayercomponent)
          (set `/Game/Blueprints/PlayersComponents/HackPlayerComponent.StartTracking` false _hackplayercomponent)
          (else
            (set `/Game/Blueprints/PlayersComponents/HackPlayerComponent.StartTracking` true _hackplayercomponent)))))))

(fn `UserConstructionScript`
  (`parent.UserConstructionScript`))