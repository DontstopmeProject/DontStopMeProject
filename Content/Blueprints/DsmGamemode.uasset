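; Game mode that runs level music, the last-kill death camera and a persistent WorkInProgress widget, and loads the saved weapon.
; Level tracks come from DT_LevelSounds by level name, with audio components kept in the game instance.
; Switching to calm music disables player time dilation and overrides weapon type until level music returns.
; Tick restarts stopped music, triggers the death camera once TargetKills is reached, and adjusts global pitch during slow motion.
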(event `self.ReceiveBeginPlay`
  (bind _asdsm_game_instance (cast `/Game/Blueprints/Dsm_GameInstance` (`GameplayStatics.GetGameInstance`)))
  (set `self.GI` _asdsm_game_instance)
  (bind _returnvalue (`|CreateWidget` "/Game/Blueprints/Widgets/BaseWidgets/WorkInProgress.WorkInProgress_C"))
  (bind _output_get (set `self.WorkInProgress` _returnvalue))
  (`UserWidget.AddToViewport` _output_get 0)
  (add `self.VolumeChangedDispatcher` (delegate `VolumeChangedDispatcher_Event`))
  (`|ExecutionSequence`
    (:`then_0`
      (bind _returnvalue_2 (`GameplayStatics.GetCurrentLevelName` true))
      (if (`KismetStringLibrary.NotEqual_StrStr` _returnvalue_2 "BaseLevel")
        ;[1 1 1] Выбор трека для уровня
        (`self.GetLevelSound`)))
    (:`then_1`
      (set `self.kills` 0)
      (bind _returnvalue_3 (`GameplayStatics.LoadGameFromSlot` (`self.SaveSlotName`)))
      (bind _assave_slot_base (cast `/Game/Blueprints/Saves/SaveSlotBase` _returnvalue_3))
      (bind _weapon_currentweapon (break `/Game/Blueprints/Weapons/Weapons/CurrentWeaponStruct` (`/Game/Blueprints/Saves/SaveSlotBase.Weapon` _assave_slot_base)))
      (if (`KismetSystemLibrary.IsValidClass` _weapon_currentweapon)
        (set `self.CurrentWeapon` (`/Game/Blueprints/Saves/SaveSlotBase.Weapon` _assave_slot_base))))))

(event `EventPlayCalmMusic`
  (bind _curlevelaudiocomponent (`self.CurLevelAudioComponent`))
  (bind _music (`/Game/Blueprints/Dsm_GameInstance.music` (`self.GI`)))
  (`/Engine/EditorBlueprintResources/StandardMacros.IsValid` _music
    (:`Is Valid`
      (if (`AudioComponent.IsPlaying` _music)
        (`AudioComponent.SetVolumeMultiplier` _curlevelaudiocomponent 0.0)
        (bind _output_get (set `self.CurLevelAudioComponent` _music))
        (`AudioComponent.SetVolumeMultiplier` _output_get 0.0)
        (`AudioComponent.SetVolumeMultiplier` _output_get 0.4)
        (else
          (`AudioComponent.SetVolumeMultiplier` _curlevelaudiocomponent 0.0 :!label _label)
          (bind _returnvalue (`GameplayStatics.CreateSound2D` "/Game/Assets/Sounds/Music/LORN_-_A-D_-_02_SPINNING_IN_A_DREAM__WAV_.LORN_-_A-D_-_02_SPINNING_IN_A_DREAM__WAV_" 0.0 1.0 0.0 null false false))
          (bind _output_get_2 (set `/Game/Blueprints/Dsm_GameInstance.music` _returnvalue (`self.GI`)))
          (`AudioComponent.Play` _output_get_2 0.0)
          (bind _output_get_3 (set `self.CurLevelAudioComponent` _output_get_2))
          (`AudioComponent.SetVolumeMultiplier` _output_get_3 0.4))))
    (:`Is Not Valid`
      (goto _label)))
  (bind _asplayers_character (cast `/Game/Blueprints/PlayersCharacter` (`GameplayStatics.GetPlayerCharacter` 0)))
  (set `/Game/Blueprints/PlayersCharacter.MasterEnableTimeDilation` false _asplayers_character)
  (`/Game/Blueprints/PlayersComponents/TimeControlComponent.ToggleTD` (`/Game/Blueprints/PlayersCharacter.TimeControlComponent` _asplayers_character) 0.0 false false)
  (set `/Game/Blueprints/BaseCharacterClass.StopChangingCustomTime` true _asplayers_character)
  (set `Actor.CustomTimeDilation` 1.0 _asplayers_character)
  (add `/Game/Blueprints/BaseCharacterClass.PickEventDispatcher` _asplayers_character (delegate `EventPlayerPickedUpWeapon`))
  (`self.EventPlayerPickedUpWeapon`)
  (`GameplayStatics.PlaySound2D` "/Game/Assets/Sounds/Effects/2Slow_Motion_Sound_Effect__WAV_.2Slow_Motion_Sound_Effect__WAV_"))

(event `VolumeChangedDispatcher_Event`)

(event `EventPlayerPickedUpWeapon`
  (`KismetSystemLibrary.Delay` 0.5)
  (bind _asplayers_character (cast `/Game/Blueprints/PlayersCharacter` (`GameplayStatics.GetPlayerCharacter` 0)))
  (set `self.WeaponsType` (`/Game/Blueprints/BaseCharacterClass.WeaponType` _asplayers_character))
  (set `/Game/Blueprints/BaseCharacterClass.WeaponType` "NewEnumerator0" _asplayers_character))

(event `EventToggleMusic`
  (params (ActiveMusic :type Boolean))
  (bind _curlevelaudiocomponent (`self.CurLevelAudioComponent`))
  (bind _output_get (set `self.ActiveMusic` ActiveMusic))
  (if _output_get
    (`/Engine/EditorBlueprintResources/StandardMacros.IsValid` _curlevelaudiocomponent
      (:`Is Valid`
        (`AudioComponent.SetVolumeMultiplier` _curlevelaudiocomponent 0.0))
      (:`Is Not Valid`
        _))
    (bind _output_get_2 (set `self.CurLevelAudioComponent` (`/Game/Blueprints/Dsm_GameInstance.music_0` (`self.GI`))))
    (if (`AudioComponent.IsPlaying` _output_get_2)
      (`AudioComponent.SetVolumeMultiplier` _output_get_2 0.0)
      (`AudioComponent.SetVolumeMultiplier` (`self.CurLevelAudioComponent`) 0.6))
    (bind _asplayers_character (cast `/Game/Blueprints/PlayersCharacter` (`GameplayStatics.GetPlayerCharacter` 0)))
    (set `/Game/Blueprints/PlayersCharacter.MasterEnableTimeDilation` true _asplayers_character)
    (set `/Game/Blueprints/BaseCharacterClass.StopChangingCustomTime` false _asplayers_character)
    (set `/Game/Blueprints/BaseCharacterClass.WeaponType` (`self.WeaponsType`) _asplayers_character)
    (remove `/Game/Blueprints/BaseCharacterClass.PickEventDispatcher` _asplayers_character (delegate `EventPlayerPickedUpWeapon`))
    (`GameplayStatics.PlaySound2D` "/Game/Assets/Sounds/Effects/1Slow_Motion_Sound_Effect__WAV_.1Slow_Motion_Sound_Effect__WAV_")
    (else
      (`self.EventPlayCalmMusic`))))

(event `self.ReceiveTick`
  (params (DeltaSeconds :type "Float (single-precision)"))
  (bind _returnvalue (`GameplayStatics.GetGlobalTimeDilation`))
  (bind _workinprogress (`self.WorkInProgress`))
  (bind _curlevelaudiocomponent (`self.CurLevelAudioComponent`))
  (bind _killedbotsarray (`self.KilledBotsArray`))
  (bind _output (`|GetArrayItem` _killedbotsarray (`KismetArrayLibrary.Array_LastIndex` _killedbotsarray)))
  (bind _throwedweapon (`/Game/Blueprints/BaseCharacterClass.ThrowedWeapon` _output))
  (`/Engine/EditorBlueprintResources/StandardMacros.IsValid` _workinprogress
    (:`Is Valid`
      _)
    (:`Is Not Valid`
      (bind _returnvalue_2 (`|CreateWidget` "/Game/Blueprints/Widgets/BaseWidgets/WorkInProgress.WorkInProgress_C"))
      (bind _output_get (set `self.WorkInProgress` _returnvalue_2))
      (`UserWidget.AddToViewport` _output_get 0)))
  (if (not (`Widget.IsVisible` _workinprogress))
    (bind _returnvalue_3 (`|CreateWidget` "/Game/Blueprints/Widgets/BaseWidgets/WorkInProgress.WorkInProgress_C"))
    (bind _output_get_2 (set `self.WorkInProgress` _returnvalue_3))
    (`UserWidget.AddToViewport` _output_get_2 0))
  (`/Engine/EditorBlueprintResources/StandardMacros.IsValid` (`self.CurLevelAudioComponent`)
    (:`Is Valid`
      (bind _returnvalue_4 (`GameplayStatics.GetCurrentLevelName` true))
      (if (`KismetStringLibrary.NotEqual_StrStr` _returnvalue_4 "BaseLevel")
        (if (`AudioComponent.IsPlaying` (`self.CurLevelAudioComponent`))
          ;[1 1 1] Динамическая громкость
          (if (!= (`self.TargetKills`) -1)
            (if (>= (`self.kills`) (`self.TargetKills`))
              (if (> (`AudioComponent.VolumeMultiplier` (`/Game/Blueprints/Dsm_GameInstance.music_0` (cast `/Game/Blueprints/Dsm_GameInstance` (`GameplayStatics.GetGameInstance`) :!pure true))) 0.0)
                (`/Engine/EditorBlueprintResources/StandardMacros.DoOnce` true :!label _label_2
                  (:`Completed`
                    (`/Engine/EditorBlueprintResources/StandardMacros.IsValid` _throwedweapon
                      (:`Is Valid`
                        (bind _asweapon_base (cast `/Game/Blueprints/Weapons/Weapons/WeaponBase` _throwedweapon)
                          (:`then`
                            (bind _splinecomponent (`/Game/Blueprints/Weapons/Weapons/WeaponBase.SplineComponent` _asweapon_base))
                            (`/Engine/EditorBlueprintResources/StandardMacros.IsValid` _splinecomponent
                              (:`Is Valid`
                                (`ActorComponent.K2_DestroyComponent` _splinecomponent)
                                (bind _staticmesh (`/Game/Blueprints/Weapons/Weapons/WeaponBase.StaticMesh` _asweapon_base))
                                (`PrimitiveComponent.SetCollisionEnabled` _staticmesh "QueryAndPhysics"))
                              (:`Is Not Valid`
                                _))
                            (`PrimitiveComponent.SetSimulatePhysics` _staticmesh true)
                            (`PrimitiveComponent.SetCollisionResponseToChannel` _staticmesh "ECC_GameTraceChannel2" "ECR_Ignore")
                            (`PrimitiveComponent.SetCollisionResponseToChannel` _staticmesh "ECC_Pawn" "ECR_Ignore")
                            (`PrimitiveComponent.AddImpulse` _staticmesh (* (`self.GetActorForwardVector` _output) 10.0) "None" false))
                          (:`CastFailed`
                            _)))
                      (:`Is Not Valid`
                        _))
                    (`/Game/Blueprints/Ai/Enemies/BaseActionNPC.EventDeathCamera` _output _output)))
                (else
                  (`|ExecutionSequence` :!label _label_3
                    (:`then_0`
                      (goto _label_2 :!via `Reset`))
                    (:`then_1`
                      _))))
              (else
                (goto _label_3)))
            (else
              (goto _label_3)))
          (else
            (`AudioComponent.SetVolumeMultiplier` _curlevelaudiocomponent 0.0)
            (`AudioComponent.SetVolumeMultiplier` _curlevelaudiocomponent 0.6)
            (`AudioComponent.Play` _curlevelaudiocomponent 0.0)))
        ;[1 1 1] Замедление влияет на звук
        (if (<= _returnvalue 0.7) :!label _label_4
          (`/Engine/EditorBlueprintResources/StandardMacros.DoOnce` false :!label _label_5
            (:`Completed`
              (`GameplayStatics.SetGlobalPitchModulation` (* _returnvalue 0.01) 0.1)
              (goto _label_6 :!via `Reset`)))
          (else
            (`/Engine/EditorBlueprintResources/StandardMacros.DoOnce` false :!label _label_6
              (:`Completed`
                (`GameplayStatics.SetGlobalPitchModulation` (`GameplayStatics.GetGlobalTimeDilation`) 0.1)
                (goto _label_5 :!via `Reset`)))))))
    (:`Is Not Valid`
      (goto _label_4))))

(event `ChangeCalmSoundVolume`
  (params (Loud :type Boolean :default false))
  ;[1 1 1] Вызывает затухание или увеличение громкости звука (по входному параметру
  (if Loud
    (bind (_direction _volume) (`Timeline|Timeline_0` :`NewTime` (`AudioComponent.VolumeMultiplier` (`/Game/Blueprints/Dsm_GameInstance.music` (cast `/Game/Blueprints/Dsm_GameInstance` (`GameplayStatics.GetGameInstance`) :!pure true))) :!label _label_7)
      (:`Update`
        (`AudioComponent.SetVolumeMultiplier` (`/Game/Blueprints/Dsm_GameInstance.music` (cast `/Game/Blueprints/Dsm_GameInstance` (`GameplayStatics.GetGameInstance`) :!pure true)) _volume)))
    (else
      (goto _label_7 :!via `Reverse`))))

(event `ChangeLevelSoundVolume`
  (params (Loud :type Boolean :default false))
  (bind _volumemultiplier (`AudioComponent.VolumeMultiplier` (`self.CurLevelAudioComponent`)))
  ;[1 1 1] Вызывает затухание или увеличение громкости звука (по входному параметру
  (bind _returnvalue (`GameplayStatics.GetCurrentLevelName` true))
  (if (`KismetStringLibrary.NotEqual_StrStr` _returnvalue "BaseLevel")
    (if Loud
      (if (not (>= _volumemultiplier 0.4))
        (bind (_direction _volume) (`Timeline|VolumeChanger` :`NewTime` _volumemultiplier :!label _label_8)
          (:`Update`
            (`AudioComponent.SetVolumeMultiplier` (`self.CurLevelAudioComponent`) _volume))
          (:`Finished`
            (`self.VolumeChangedDispatcher`))))
      (else
        (goto _label_8 :!via `Reverse`)))))

(fn `GetLevelSound`
  (bind _music_0 (`/Game/Blueprints/Dsm_GameInstance.music_0` (cast `/Game/Blueprints/Dsm_GameInstance` (`GameplayStatics.GetGameInstance`) :!pure true)))
  (bind _returnvalue (`GameplayStatics.GetCurrentLevelName` true))
  (bind _returnvalue_2 (`|GetDataTableRow` "/Game/Blueprints/DT_LevelSounds.DT_LevelSounds" (`KismetStringLibrary.Conv_StringToName` _returnvalue))
    (:`then`
      (`/Engine/EditorBlueprintResources/StandardMacros.IsValid` _music_0
        (:`Is Valid`
          (if (`KismetStringLibrary.NotEqual_StrStr` (`KismetSystemLibrary.GetObjectName` (`.SoundToPlay_5_08A1C132458E2C00A57C9F9251C61BB1` (break `/Game/Blueprints/S_LevelSound` _returnvalue_2))) (`KismetSystemLibrary.GetObjectName` (`AudioComponent.Sound` _music_0)))
            (bind _returnvalue_3 (`GameplayStatics.GetCurrentLevelName` true :!label _label))
            (bind _returnvalue_4 (`|GetDataTableRow` "/Game/Blueprints/DT_LevelSounds.DT_LevelSounds" (`KismetStringLibrary.Conv_StringToName` _returnvalue_3))
              (:`then`
                (bind (_level _soundtoplay) (break `/Game/Blueprints/S_LevelSound` _returnvalue_4))
                (set `self.LevelSoundWave` _soundtoplay)
                (bind _returnvalue_5 (`GameplayStatics.CreateSound2D` _soundtoplay 1.0 1.0 0.0 null true false))
                (bind _asdsm_game_instance (cast `/Game/Blueprints/Dsm_GameInstance` (`GameplayStatics.GetGameInstance`)))
                (set `/Game/Blueprints/Dsm_GameInstance.music_0` _returnvalue_5 _asdsm_game_instance)
                (set `self.CurLevelAudioComponent` _returnvalue_5)))
            (else
              (`/Engine/EditorBlueprintResources/StandardMacros.IsValid` (`self.CurLevelAudioComponent`)
                (:`Is Not Valid`
                  (bind _asdsm_game_instance_2 (cast `/Game/Blueprints/Dsm_GameInstance` (`GameplayStatics.GetGameInstance`)))
                  (set `self.CurLevelAudioComponent` (`/Game/Blueprints/Dsm_GameInstance.music_0` _asdsm_game_instance_2)))))))
        (:`Is Not Valid`
          (goto _label))))))

(fn `UserConstructionScript`)